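; BP_BoxSpeedUp is a speed-boost trigger volume for the first-person character in the gym prototype.
; When the character enters the Box, it doubles max walk speed and widens the camera field of view for a sense of speed.
; Leaving the box sets walk speed to a hardcoded default and subtracts the same field-of-view offset, so both changes last only while overlapping.
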(event OnComponentBeginOverlap(Box)
  (params (OverlappedComponent :type Primitive%20Component%20Object%20Reference) (OtherActor :type Actor%20Object%20Reference) (OtherComp :type Primitive%20Component%20Object%20Reference) (OtherBodyIndex :type Integer) (bFromSweep :type Boolean) (SweepResult :type Hit%20Result%20Structure%20%28by%20ref%29))
  (bind _asbp_first_person_character (Utilities|Casting|CastToBP_FirstPersonCharacter OtherActor))
  (bind _firstpersoncameracomponent (Variables|/Script/DiamondProject.DiamondProjectCharacter|GetFirstPersonCameraComponent _asbp_first_person_character))
  (Variables|/Script/Engine.CharacterMovementComponent|SetMaxWalkSpeed (Variables|/Script/Engine.Character|GetCharacterMovement _asbp_first_person_character) 1.2e+03)
  (Camera|SetFieldOfView _firstpersoncameracomponent (+ (Variables|/Script/Engine.CameraComponent|GetFieldOfView _firstpersoncameracomponent) 1e+01)))

(event OnComponentEndOverlap(Box)
  (params (OverlappedComponent :type Primitive%20Component%20Object%20Reference) (OtherActor :type Actor%20Object%20Reference) (OtherComp :type Primitive%20Component%20Object%20Reference) (OtherBodyIndex :type Integer))
  (bind _asbp_first_person_character (Utilities|Casting|CastToBP_FirstPersonCharacter OtherActor))
  (bind _firstpersoncameracomponent (Variables|/Script/DiamondProject.DiamondProjectCharacter|GetFirstPersonCameraComponent _asbp_first_person_character))
  (Variables|/Script/Engine.CharacterMovementComponent|SetMaxWalkSpeed (Variables|/Script/Engine.Character|GetCharacterMovement _asbp_first_person_character) 6e+02)
  (Camera|SetFieldOfView _firstpersoncameracomponent (+ (Variables|/Script/Engine.CameraComponent|GetFieldOfView _firstpersoncameracomponent) -1e+01)))

(fn ConstructionScript)