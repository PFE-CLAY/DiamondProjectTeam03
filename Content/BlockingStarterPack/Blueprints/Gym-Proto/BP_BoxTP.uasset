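; BP_BoxTP is a trigger box in the Gym-Proto blockout that teleports the player character sideways along world X.
; On BeginPlay, the Right flag sets Direction to positive or negative.
; When the player character overlaps the Box, it is teleported a fixed distance along X in that direction, keeping its Y and Z.
; NewFunction is an empty stub.
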(event OnComponentBeginOverlap(Box)
  (params (OverlappedComponent :type Primitive%20Component%20Object%20Reference) (OtherActor :type Actor%20Object%20Reference) (OtherComp :type Primitive%20Component%20Object%20Reference) (OtherBodyIndex :type Integer) (bFromSweep :type Boolean) (SweepResult :type Hit%20Result%20Structure%20%28by%20ref%29))
  (bind _returnvalue (Transformation|GetActorLocation OtherActor))
  (bind _returnvalue_2 (Game|GetPlayerCharacter 0))
  (if (== OtherActor _returnvalue_2)
    (Transformation|SetActorLocation _returnvalue_2 (Math|Vector|MakeVector (+ (* (Variables|Default|GetDirection) 1.2e+03) (.x _returnvalue)) (.y _returnvalue) (.z _returnvalue)) false true)))

(event Collision|EventActorBeginOverlap
  (params (OtherActor :type Actor%20Object%20Reference)))

(event EventTick
  (params (DeltaSeconds :type Float%20%28single-precision%29)))

(event EventBeginPlay
  (if (Variables|Default|GetRight?)
    (Variables|Default|SetDirection 1.0)
    (else
      (Variables|Default|SetDirection -1.0))))

(fn ConstructionScript)

(fn NewFunction
  (params (Player%20? :type Object%20Object%20Reference)))