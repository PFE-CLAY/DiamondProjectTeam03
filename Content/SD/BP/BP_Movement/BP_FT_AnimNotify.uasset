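; Anim notify that plays player footstep audio through Wwise when an animation reaches it.
; It line-traces 200 units down from player pawn 0, then calls SetSwitch and posts the Play_MC_FOL_FT_SW event on that pawn, ignoring the notifying mesh.
; Surface switching is unfinished: the traced physical material feeds only disconnected debug and conversion nodes, SetSwitch gets no surface value, and a TODO flags this.
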(fn ReceivedNotify
  (params (MeshComp :type Skeletal%20Mesh%20Component%20Object%20Reference) (Animation :type Anim%20Sequence%20Base%20Object%20Reference) (EventReference :type Anim%20Notify%20Event%20Reference%20Structure%20%28by%20ref%29))
  (bind _returnvalue (Game|Player|GetPlayerPawn 0))
  (bind _returnvalue_2 (Transformation|GetActorLocation _returnvalue))
  ;[0.5649 0.6525 1] Footsteps LineTrace+Switch Surface
  (bind _outhit (Collision|LineTraceByChannel _returnvalue_2 (+ _returnvalue_2 "0.000000,0.000000,-200.000000") "TraceTypeQuery1" false 0 "None"))
  ;;[1 0.15 0.15 0.5] #TODO: Check with SD about SwitchState for physics material
  (Class|AkGameplayStatics|SetSwitch 0 (Game|Player|GetPlayerPawn 0))
  (Class|AkGameplayStatics|PostEvent "/Game/WwiseAudio/Events/MC_WU/Play_MC_FOL_FT_SW.Play_MC_FOL_FT_SW" (Game|Player|GetPlayerPawn 0))
  (return false))