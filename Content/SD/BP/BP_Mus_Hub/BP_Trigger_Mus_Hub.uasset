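; Trigger actor that starts and stops the Blacksands hub music through Wwise.
; Two box components react to player pawn overlaps, each posting its play or stop event via the Wwise manager subsystem without an actor.
; The start box is gated by a DoOnce that is never reset, so the music starts only once, and it also prints a leftover debug "Hello".
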(event OnComponentBeginOverlap(Box_MUS_Stop)
  (params (OverlappedComponent :type Primitive%20Component%20Object%20Reference) (OtherActor :type Actor%20Object%20Reference) (OtherComp :type Primitive%20Component%20Object%20Reference) (OtherBodyIndex :type Integer) (bFromSweep :type Boolean) (SweepResult :type Hit%20Result%20Structure%20%28by%20ref%29))
  (if (== OtherActor (Game|Player|GetPlayerPawn 0))
    (Class|WwiseManagerSubsystem|PostEventWithoutActor (Subsystems|GetWwiseManagerSubsystem) "/Game/WwiseAudio/Events/MUS_WU/Stop_MUS_Blacksands_Hub.Stop_MUS_Blacksands_Hub")))

(event OnComponentBeginOverlap(Box_MUS_Start)
  (params (OverlappedComponent :type Primitive%20Component%20Object%20Reference) (OtherActor :type Actor%20Object%20Reference) (OtherComp :type Primitive%20Component%20Object%20Reference) (OtherBodyIndex :type Integer) (bFromSweep :type Boolean) (SweepResult :type Hit%20Result%20Structure%20%28by%20ref%29))
  (if (== OtherActor (Game|Player|GetPlayerPawn 0))
    (Development|PrintString "Hello")
    (Utilities|FlowControl|DoOnce false
      (:Completed
        (Class|WwiseManagerSubsystem|PostEventWithoutActor (Subsystems|GetWwiseManagerSubsystem) "/Game/WwiseAudio/Events/MUS_WU/Play_MUS_Blacksands_Hub.Play_MUS_Blacksands_Hub")))))

(fn ConstructionScript)