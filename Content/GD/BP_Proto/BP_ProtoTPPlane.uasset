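; BP_ProtoTPPlane is a prototype teleport plane with a scene capture component.
; The construction script assigns the capture's render target.
; On overlap, if the capture's world rotation matches player 0's capsule rotation within a tolerance, it sets the overlapping actor's transform to the player mesh location plus an offset vector.
; Disconnected experiments with distance-based FOV and facing-angle checks remain unused.
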(event Collision|EventActorBeginOverlap
  (params (OtherActor :type Actor%20Object%20Reference))
  (if (Utilities|Operators|EqualEqual (Transformation|GetWorldRotation (Variables|Default|GetSceneCaptureComponent2D)) (Transformation|GetWorldRotation (Variables|/Script/Engine.Character|GetCapsuleComponent (Game|GetPlayerCharacter 0))) (Variables|Default|GetTolerance))
    (Transformation|SetActorTransform OtherActor (Math|Conversions|ToTransform(Vector) (+ (Transformation|GetWorldLocation (Variables|/Script/Engine.Character|GetMesh (Game|GetPlayerCharacter 0))) (Variables|Default|GetNewVector))))))

(fn ConstructionScript
  (Variables|/Script/Engine.SceneCaptureComponent2D|SetTextureTarget (Variables|Default|GetSceneCaptureComponent2D) (Variables|Default|GetTexture%20Target)))