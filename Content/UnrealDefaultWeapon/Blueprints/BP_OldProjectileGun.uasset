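; BP_OldProjectileGun is a weapon pickup that spins and bobs on looping tweens until the player attaches it.
; PlayerProtoWeapon events drive the ammo text, Wwise sounds and animation rifle flag, with material flashes on ammo refills.
; Firing tweens the camera FOV and shows a randomly rotated, scaled muzzle flash.
; On drop, the gun shows a no-ammo material, detaches and destroys itself.
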(event OnDropped(PlayerProtoWeapon)
  (params (PickUpCharacter :type Diamond%20Project%20Character%20Object%20Reference))
  (Class|WwiseManagerSubsystem|PostEvent (Subsystems|GetWwiseManagerSubsystem) "/Game/WwiseAudio/Events/MC_WU/Play_MC_SFX_Weapon_NoAmmo_RC.Play_MC_SFX_Weapon_NoAmmo_RC" self)
  (CallFunction|NoMoreAmmoColor)
  (Utilities|FlowControl|Delay 0.3)
  (Class|PlayerHitscanWeaponComponent|DetachWeapon (Variables|Default|GetPlayerProtoWeapon))
  (bind _asfirst_person_anim_bp (Utilities|Casting|CastToFirstPerson_AnimBP (Components|SkeletalMesh|GetAnimInstance (Variables|/Script/DiamondProject.DiamondProjectCharacter|GetMesh1P PickUpCharacter))))
  (Variables|/Game/FirstPersonArms/Animations/FirstPerson_AnimBP.FirstPerson_AnimBP_C|SetHasRifle _asfirst_person_anim_bp false)
  (Actor|DestroyActor))

(event OnPickUp(TP_PickUp)
  (params (PickUpCharacter :type Diamond%20Project%20Character%20Object%20Reference))
  (bind _returnvalue (Class|WeaponComponent|AttachWeapon (Variables|Default|GetPlayerProtoWeapon) PickUpCharacter))
  (if _returnvalue
    (CallFunction|StopWeaponFloat)
    (bind _asfirst_person_anim_bp (Utilities|Casting|CastToFirstPerson_AnimBP (Components|SkeletalMesh|GetAnimInstance (Variables|/Script/DiamondProject.DiamondProjectCharacter|GetMesh1P PickUpCharacter))))
    (Variables|/Game/FirstPersonArms/Animations/FirstPerson_AnimBP.FirstPerson_AnimBP_C|SetHasRifle _asfirst_person_anim_bp true)
    (Rendering|Components|TextRender|SetText (Variables|Default|GetBulletCountText) (Utilities|Text|ToText(Integer) (Class|PlayerHitscanWeaponComponent|GetAmmoonSpawn (Variables|Default|GetPlayerProtoWeapon))))
    (bind _tp_pickup (Variables|Default|GetTP_PickUp)
      (:then
        (Components|DestroyComponent _tp_pickup)
        (Rendering|SetVisibility (Variables|Default|GetSpotLight) false false))
      (:else))))

(event OnFire(PlayerProtoWeapon)
  (params (CurrentAmmo :type Integer) (HitLocation :type Vector :default "0, 0, 0"))
  (Class|WwiseManagerSubsystem|PostEvent (Subsystems|GetWwiseManagerSubsystem) "/Game/WwiseAudio/Events/MC_WU/Play_MC_SFX_Gun_Shoot_RC.Play_MC_SFX_Gun_Shoot_RC" self)
  (Rendering|Components|TextRender|SetText (Variables|Default|GetBulletCountText) (Utilities|Text|ToText(Integer) CurrentAmmo))
  (Utilities|FlowControl|Sequence
    (:then_0
      (Class|AkGameplayStatics|PostEvent "/Game/WwiseAudio/Events/MC_WU/Play_MC_SFX_Gun_Shoot_RC.Play_MC_SFX_Gun_Shoot_RC" self))
    (:then_1
      (|DisplayVFX_2))))

(event OnUpdateAmmo(PlayerProtoWeapon)
  (params (newAmmoCount :type Integer))
  (bind _returnvalue (Utilities|Text|ToText(Integer) newAmmoCount))
  (Class|WwiseManagerSubsystem|PostEvent (Subsystems|GetWwiseManagerSubsystem) "/Game/WwiseAudio/Events/MC_WU/Play_MC_SFX_UpdateAmmo_RC.Play_MC_SFX_UpdateAmmo_RC" self)
  (Rendering|Components|TextRender|SetText (Variables|Default|GetBulletCountText) _returnvalue)
  (Development|PrintString (Utilities|String|ToString(Text) _returnvalue))
  (if (>= newAmmoCount (Class|PlayerHitscanWeaponComponent|GetMagazineSize (Variables|Default|GetPlayerProtoWeapon)))
    (CallFunction|PickUpAmmoMaxColor)
    (else
      (CallFunction|PickUpAmmoColor))))

(event OnPickedUpWeapon(PlayerProtoWeapon)
  (bind _playerprotoweapon (Variables|Default|GetPlayerProtoWeapon))
  (Utilities|IsValid _playerprotoweapon
    (:Is%20Valid
      (Rendering|Components|TextRender|SetText (Variables|Default|GetBulletCountText) (Utilities|Text|ToText(Integer) (Class|PlayerHitscanWeaponComponent|GetCurrentAmmo _playerprotoweapon)))
      (Class|WwiseManagerSubsystem|PostEvent (Subsystems|GetWwiseManagerSubsystem) "/Game/WwiseAudio/Events/MC_WU/Play_MC_SFX_Weapon_Armed_RC.Play_MC_SFX_Weapon_Armed_RC" self))))

(event Custom|PickUpAmmoColor
  (bind _playerprotoweapon (Variables|Default|GetPlayerProtoWeapon))
  (Rendering|Material|SetMaterial _playerprotoweapon 0 "/Game/Project/Assets/M_GunRifleReload.M_GunRifleReload")
  (Utilities|FlowControl|Delay 0.5)
  (Rendering|Material|SetMaterial _playerprotoweapon 0 "/Game/Project/Assets/M_GunRifle.M_GunRifle"))

(event Custom|NoMoreAmmoColor
  (Rendering|Material|SetMaterial (Variables|Default|GetPlayerProtoWeapon) 0 "/Game/Project/Assets/M_GunRifleNoAmmo.M_GunRifleNoAmmo"))

(event Custom|PickUpAmmoMaxColor
  (bind _playerprotoweapon (Variables|Default|GetPlayerProtoWeapon))
  (Rendering|Material|SetMaterial _playerprotoweapon 0 "/Game/Project/Assets/M_GunRifleReloadMax.M_GunRifleReloadMax")
  (Utilities|FlowControl|Delay 0.5)
  (Rendering|Material|SetMaterial _playerprotoweapon 0 "/Game/Project/Assets/M_GunRifle.M_GunRifle"))

(event EventBeginPlay
  (bind _ashud_game (Utilities|Casting|CastToHUD_GAME (HUD|GetHUD (Game|GetPlayerController 0))))
  (Variables|Default|SetHUD _ashud_game)
  (Utilities|FlowControl|Sequence
    (:then_0
      (|WeaponRotateAndFloatLoop_2))
    (:then_1
      (bind _asbp_first_person_character (Utilities|Casting|CastToBP_FirstPersonCharacter (Game|GetPlayerCharacter 0)))
      (Variables|VFX|SetDefaultFOV (Variables|/Script/Engine.CameraComponent|GetFieldOfView (Variables|/Script/DiamondProject.DiamondProjectCharacter|GetFirstPersonCameraComponent _asbp_first_person_character))))
    (:then_2
      (Development|SetHiddeninGame (Variables|Default|GetMuzzleShotVisual) true false))))

(fn ConstructionScript)

(event Custom|StopWeaponFloat
  (bind _async_float_task (Variables|Default|GetAsync%20float%20task)
    (:then
      (Class|FCTweenBPAction|Stop _async_float_task)
      (bind _async_rotation_task (Variables|Default|GetAsync%20Rotation%20task)
        (:then
          (Class|FCTweenBPAction|Stop _async_rotation_task))
        (:else)))
    (:else)))