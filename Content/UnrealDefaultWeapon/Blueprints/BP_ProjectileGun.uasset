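; BP_ProjectileGun is the player's pickup rifle, handling feedback around its PlayerProtoWeapon component.
; Pickup and drop attach or detach it and toggle the arms AnimBP's HasRifle; dropping shows a no-ammo material, then destroys the actor.
; Weapon events drive Wwise sounds, the bullet-count text and ammo material flashes.
; Firing aims Niagara at the hit and tweens camera FOV with a muzzle flash; impact VFX spawn only on pillars, targets and turrets.
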(event OnDropped(PlayerProtoWeapon)
  (params (PickUpCharacter :type Diamond%20Project%20Character%20Object%20Reference))
  (Class|WwiseManagerSubsystem|PostEvent (Subsystems|GetWwiseManagerSubsystem) "/Game/WwiseAudio/Events/MC_WU/Play_MC_SFX_Weapon_NoAmmo_RC.Play_MC_SFX_Weapon_NoAmmo_RC" self)
  (CallFunction|NoMoreAmmoColor)
  (Utilities|FlowControl|Delay 0.3)
  (Class|WeaponComponent|DetachWeapon (Variables|Default|GetPlayerProtoWeapon))
  (bind _asfirst_person_anim_bp (Utilities|Casting|CastToFirstPerson_AnimBP (Components|SkeletalMesh|GetAnimInstance (Variables|/Script/DiamondProject.DiamondProjectCharacter|GetMesh1P PickUpCharacter))))
  (Variables|/Game/FirstPersonArms/Animations/FirstPerson_AnimBP.FirstPerson_AnimBP_C|SetHasRifle _asfirst_person_anim_bp false)
  (Actor|DestroyActor))

(event OnPickUp(TP_PickUp)
  (params (PickUpCharacter :type Diamond%20Project%20Character%20Object%20Reference))
  (bind _returnvalue (Class|WeaponComponent|AttachWeapon (Variables|Default|GetPlayerProtoWeapon) PickUpCharacter))
  (if _returnvalue
    (bind _asfirst_person_anim_bp (Utilities|Casting|CastToFirstPerson_AnimBP (Components|SkeletalMesh|GetAnimInstance (Variables|/Script/DiamondProject.DiamondProjectCharacter|GetMesh1P PickUpCharacter))))
    (Variables|/Game/FirstPersonArms/Animations/FirstPerson_AnimBP.FirstPerson_AnimBP_C|SetHasRifle _asfirst_person_anim_bp true)))

(event OnFire(PlayerProtoWeapon)
  (params (CurrentAmmo :type Integer) (HitLocation :type Vector :default "0, 0, 0"))
  (Class|WwiseManagerSubsystem|PostEvent (Subsystems|GetWwiseManagerSubsystem) "/Game/WwiseAudio/Events/MC_WU/Play_MC_SFX_Gun_Shoot_RC.Play_MC_SFX_Gun_Shoot_RC" self)
  (Rendering|Components|TextRender|SetText (Variables|Default|GetBulletCountText) (Utilities|Text|ToText(Integer) CurrentAmmo))
  (Utilities|FlowControl|Sequence
    (:then_0
      (bind _returnvalue (AddComponent|AddNiagaraComponent false))
      (Transformation|SetWorldRotation _returnvalue (Math|Rotator|FindLookatRotation (Transformation|GetWorldLocation (Variables|Default|GetNiagaraLocation)) HitLocation) false false)
      (Class|AkGameplayStatics|PostEvent "/Game/WwiseAudio/Events/MC_WU/Play_MC_SFX_Gun_Shoot_RC.Play_MC_SFX_Gun_Shoot_RC" self))
    (:then_1
      (|DisplayVFX_2))))

(event OnUpdateAmmo(PlayerProtoWeapon)
  (params (newAmmoCount :type Integer))
  (bind _returnvalue (Utilities|Text|ToText(Integer) newAmmoCount))
  (Class|WwiseManagerSubsystem|PostEvent (Subsystems|GetWwiseManagerSubsystem) "/Game/WwiseAudio/Events/MC_WU/Play_MC_SFX_UpdateAmmo_RC.Play_MC_SFX_UpdateAmmo_RC" self)
  (Rendering|Components|TextRender|SetText (Variables|Default|GetBulletCountText) _returnvalue)
  (Development|PrintString (Utilities|String|ToString(Text) _returnvalue))
  (if (>= newAmmoCount (Class|WeaponComponent|GetMagazineSize (Variables|Default|GetPlayerProtoWeapon)))
    (CallFunction|PickUpAmmoMaxColor)
    (else
      (CallFunction|PickUpAmmoColor))))

(event OnHit(PlayerProtoWeapon)
  (params (HitInfo :type Hit%20Result%20Structure))
  (Utilities|Casting|CastToBP_FallingPillarBis (.hitactor HitInfo)
    (:then
      _)
    (:CastFailed
      (Utilities|Casting|CastToBP_Target (.hitactor HitInfo)
        (:then
          _)
        (:CastFailed
          (Utilities|Casting|CastToBP_TurretEnemy (.hitactor HitInfo))))))
  (bind _returnvalue (Niagara|SpawnSystematLocation "/Game/Project/VFX/FXS_ImpactBurst.FXS_ImpactBurst" (.impactpoint HitInfo) (Math|Conversions|RotationFromXVector (.normal HitInfo))))
  (Niagara|SetNiagaraVariable(Vector3) _returnvalue "User.Rotation" (.normal HitInfo))
  (Niagara|SpawnSystematLocation "/Game/Project/VFX/VFX_Smoke/Smoke_NS.Smoke_NS" (.impactpoint HitInfo) (Math|Conversions|RotationFromXVector (.normal HitInfo))))

(event OnPickedUpWeapon(PlayerProtoWeapon)
  (bind _playerprotoweapon (Variables|Default|GetPlayerProtoWeapon))
  (Utilities|IsValid _playerprotoweapon
    (:Is%20Valid
      (Rendering|Components|TextRender|SetText (Variables|Default|GetBulletCountText) (Utilities|Text|ToText(Integer) (Class|WeaponComponent|GetCurrentAmmo _playerprotoweapon)))
      (Class|WwiseManagerSubsystem|PostEvent (Subsystems|GetWwiseManagerSubsystem) "/Game/WwiseAudio/Events/MC_WU/Play_MC_SFX_Weapon_Armed_RC.Play_MC_SFX_Weapon_Armed_RC" self))))

(event Custom|NoMoreAmmoColor
  (Rendering|Material|SetMaterial (Variables|Default|GetPlayerProtoWeapon) 0 "/Game/Project/Assets/M_GunRifleNoAmmo.M_GunRifleNoAmmo"))

(event Custom|PickUpAmmoMaxColor
  (bind _playerprotoweapon (Variables|Default|GetPlayerProtoWeapon))
  (Rendering|Material|SetMaterial _playerprotoweapon 0 "/Game/Project/Assets/M_GunRifleReloadMax.M_GunRifleReloadMax")
  (Utilities|FlowControl|Delay 0.5)
  (Rendering|Material|SetMaterial _playerprotoweapon 0 "/Game/Project/Assets/M_GunRifle.M_GunRifle"))

(event Custom|PickUpAmmoColor
  (bind _playerprotoweapon (Variables|Default|GetPlayerProtoWeapon))
  (Rendering|Material|SetMaterial _playerprotoweapon 0 "/Game/Project/Assets/M_GunRifleReload.M_GunRifleReload")
  (Utilities|FlowControl|Delay 0.5)
  (Rendering|Material|SetMaterial _playerprotoweapon 0 "/Game/Project/Assets/M_GunRifle.M_GunRifle"))

(fn ConstructionScript)