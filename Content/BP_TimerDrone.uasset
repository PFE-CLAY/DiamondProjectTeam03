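; BP_TimerDrone is an actor that displays the game timer on two text render components.
; On BeginPlay it finds a BP_Timer actor in the level and caches it.
; Every Tick it formats that timer's Time with TimeSecondsToString and writes it to both texts, without re-checking that the reference is valid.
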(event EventTick
  (params (DeltaSeconds :type Float%20%28single-precision%29))
  (bind _timeractor (Variables|Default|GetTimerActor))
  (bind _time (Variables|/Game/Project/BP/LD/BP_Timer.BP_Timer_C|GetTime _timeractor))
  (bind _returnvalue (Class|KismetStringLibrary|TimeSecondstoString _time))
  (bind _returnvalue_2 (Utilities|Text|ToText(String) _returnvalue))
  (Rendering|Components|TextRender|SetText (Variables|Default|GetTextRender) _returnvalue_2)
  (Rendering|Components|TextRender|SetText (Variables|Default|GetTextRender1) _returnvalue_2))

(event EventBeginPlay
  (bind _returnvalue (Actor|GetActorOfClass "/Game/Project/BP/LD/BP_Timer.BP_Timer_C"))
  (Utilities|IsValid _returnvalue
    (:Is%20Valid
      (Variables|Default|SetTimerActor _returnvalue))))

(fn ConstructionScript)