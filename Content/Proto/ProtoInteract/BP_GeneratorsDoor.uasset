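; Prototype interactable door that stays locked until enough generators are activated.
; GeneratorActivated counts activations and, at the required number, makes the door openable and interactable and destroys its DoorShield component.
; OnInteract disables further interaction and, if the door is openable, tweens the DoorMesh world rotation to a 90-degree roll, keeping pitch and yaw.
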(event Custom|GeneratorActivated
  (bind _result (Math|Integer|IncrementInt (Variables|Default|GetActivatedGenerators))
    (:%20%20
      (if (>= _result (Variables|Default|GetRequiredNumberOfGenerators))
        (bind _output_get (Variables|Default|SetCanBeOpened true))
        (Variables|Default|SetCanBeInteractedWith _output_get)
        (Components|DestroyComponent (Variables|Default|GetDoorShield))
        (else
          (Variables|Default|SetCanBeOpened false))))))

(event EventOnInteract
  (params (InteractingPlayer :type Character%20Object%20Reference))
  (bind _doormesh (Variables|Default|GetDoorMesh))
  (bind _returnvalue (Transformation|GetWorldRotation _doormesh))
  (if (Variables|Default|GetCanBeInteractedWith)
    (Variables|Default|SetCanBeInteractedWith false)
    (if (Variables|Default|GetCanBeOpened)
      (Variables|Default|SetCanBeInteractedWith false)
      (bind _value (|TweenRotator (Math|Rotator|MakeRotator (.roll _returnvalue) (.pitch _returnvalue) (.yaw _returnvalue)) (Math|Rotator|MakeRotator 9e+01 (.pitch _returnvalue) (.yaw _returnvalue)) 1.0 "InOutQuad")
        (:ApplyEasing
          (Transformation|SetWorldRotation (Variables|Default|GetDoorMesh) _value false false))))))

(fn ConstructionScript)