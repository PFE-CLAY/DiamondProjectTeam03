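; Prototype destructible wall that topples over when its health component signals death.
; The death event plays an announcer sound and tweens the wall mesh through a 90-degree roll, flagging it as falling until completion.
; Each tween update also activates the WallFall and CoverTrap preplan steps on the loop subsystem.
; While falling, the mesh deals massive damage to anything it hits that has a health component; the interact event is empty.
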(event OnDeathEvent(AC_Health)
  (bind _wallmesh (Variables|Default|GetWallMesh))
  (bind _returnvalue (Transformation|GetWorldRotation _wallmesh))
  (Audio|SpawnSound2D "/Game/Proto/Sound/Announcer_VoiceLines/SFX_Announcer_WallFall.SFX_Announcer_WallFall" 1.0 1.0 0.0 0)
  (Development|PrintString "wall destroyed")
  (bind _value (|TweenRotator (Math|Rotator|MakeRotator (.roll _returnvalue) (.pitch _returnvalue) (.yaw _returnvalue)) (Math|Rotator|MakeRotator (+ (.roll _returnvalue) -9e+01) (.pitch _returnvalue) (.yaw _returnvalue)) 1.0 "InOutQuad")
    (:then
      (Variables|Default|SetIsFalling true))
    (:ApplyEasing
      (Transformation|SetWorldRotation (Variables|Default|GetWallMesh) _value false false)
      (Class|LoopSubsystem|ActivatePreplanStep (Subsystems|GetLoopSubsystem) "WallFall")
      (Class|LoopSubsystem|ActivatePreplanStep (Subsystems|GetLoopSubsystem) "CoverTrap"))
    (:OnComplete
      (Variables|Default|SetIsFalling false))))

(event OnComponentHit(WallMesh)
  (params (HitComponent :type Primitive%20Component%20Object%20Reference) (OtherActor :type Actor%20Object%20Reference) (OtherComp :type Primitive%20Component%20Object%20Reference) (NormalImpulse :type Vector :default "0, 0, 0") (Hit :type Hit%20Result%20Structure%20%28by%20ref%29))
  (bind _returnvalue (Actor|GetComponentbyClass OtherActor "/Script/DiamondProject.AC_Health"))
  (if (Variables|Default|GetIsFalling)
    (Utilities|IsValid _returnvalue
      (:Is%20Valid
        (Class|ACHealth|DecreaseHealth _returnvalue 1000)))))

(event EventOnInteract
  (params (InteractingPlayer :type Character%20Object%20Reference)))

(fn ConstructionScript)