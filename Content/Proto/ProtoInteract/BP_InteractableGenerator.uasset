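; BP_InteractableGenerator is a one-shot interactable generator switch that reports its activation to a linked generators door.
; BeginPlay applies the switch material; the first permitted interaction disables further use, swaps that material and turns the point light green.
; If the Door reference casts to BP_GeneratorsDoor, it notifies the door, plays an attenuated button sound and activates two LoopSubsystem preplan steps, one configurable and one fixed "NoShield".
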(event EventOnInteract
  (params (InteractingPlayer :type Character%20Object%20Reference))
  (if (Variables|Default|GetCanBeInteractedWith)
    (Variables|Default|SetCanBeInteractedWith false)
    (Rendering|Material|SetMaterial (Variables|Default|GetCube) 0 "/Game/BlockingStarterPack/Blueprints/Others/BlockingTooltip/M_BlockingTooltipBase.M_BlockingTooltipBase")
    (Rendering|Components|Light|SetLightColor (Variables|Default|GetPointLight) "(R=0.000000,G=1.000000,B=0.210394,A=1.000000)" true)
    (bind _asbp_generators_door (Utilities|Casting|CastToBP_GeneratorsDoor (Variables|Default|GetDoor)))
    (Default|GeneratorActivated _asbp_generators_door)
    (Audio|SpawnSoundatLocation "/Game/Proto/PlaceHolderSounds/Folley/Triger_Buton.Triger_Buton" (Transformation|GetActorLocation self) "0, 0, 0" 1.0 1.0 0.0 "/Game/Proto/PlaceHolderSounds/A_GlobalAttenuation.A_GlobalAttenuation" 0)
    (Class|LoopSubsystem|ActivatePreplanStep (Subsystems|GetLoopSubsystem) (Variables|Default|GetPrePlanIdToCall))
    (Class|LoopSubsystem|ActivatePreplanStep (Subsystems|GetLoopSubsystem) "NoShield")))

(event EventBeginPlay
  (Rendering|Material|SetMaterial (Variables|Default|GetCube) 0 (Variables|Default|GetMaterialInterupteur)))

(fn ConstructionScript)