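; BP_ProtoAllied is a prototype allied AI pawn that walks a scripted route and reports milestones to the loop subsystem.
; After a start delay, it moves to Destination, then to Destinatio2, and on arrival activates the "ManDoor" preplan step.
; When its health component fires the death event, it activates the "FallingTrap" preplan step and destroys itself.
; A failed first move only prints a debug string.
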(event OnDeathEvent(AC_Health)
  (Class|LoopSubsystem|ActivatePreplanStep (Subsystems|GetLoopSubsystem) "FallingTrap")
  (Actor|DestroyActor))

(event EventBeginPlay
  (bind _self self)
  (Utilities|FlowControl|Delay 1e+01)
  (AI|AIMoveTo _self "0, 0, 0" (Variables|Default|GetDestination) 5e+01 false
    (:OnSuccess
      (AI|AIMoveTo _self "0, 0, 0" (Variables|Default|GetDestinatio2) 5e+01 false
        (:OnSuccess
          (Class|LoopSubsystem|ActivatePreplanStep (Subsystems|GetLoopSubsystem) "ManDoor"))))
    (:OnFail
      (Development|PrintString "Hello"))))

(fn ConstructionScript)