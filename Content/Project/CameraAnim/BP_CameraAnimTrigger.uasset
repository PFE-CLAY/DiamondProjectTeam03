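; One-shot trigger volume that plays a camera animation with a dust effect and brief slowdown when the first-person character enters it.
; On the first box overlap it spawns a BP_CameraAnimations actor at the character's transform, starts its animation and spawns a tiny falling-dust Niagara system there.
; It halves the character's walk speed for a moment, restores the cached value, then destroys itself after a further delay.
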(event OnComponentBeginOverlap(Box)
  (params (OverlappedComponent :type Primitive%20Component%20Object%20Reference) (OtherActor :type Actor%20Object%20Reference) (OtherComp :type Primitive%20Component%20Object%20Reference) (OtherBodyIndex :type Integer) (bFromSweep :type Boolean) (SweepResult :type Hit%20Result%20Structure%20%28by%20ref%29))
  (bind _asbp_first_person_character (Utilities|Casting|CastToBP_FirstPersonCharacter OtherActor))
  (Utilities|FlowControl|DoOnce false
    (:Completed
      (bind _output_get (Variables|Default|SetFirstPersonRef _asbp_first_person_character))
      (bind _returnvalue (Game|SpawnActorfromClass "/Game/Project/BP/BP_CameraAnimations.BP_CameraAnimations_C" (Math|Transform|MakeTransform (Transformation|GetWorldLocation (Variables|/Script/Engine.Actor|GetRootComponent _asbp_first_person_character)) (Transformation|GetWorldRotation (Variables|/Script/Engine.Actor|GetRootComponent _asbp_first_person_character))) "Undefined" "MultiplyWithRoot" 0 0))
      (Default|PlayCameraAnimaion _returnvalue)
      (Niagara|SpawnSystematLocation "/Game/Project/VFX/FXS_DustHourglassFall.FXS_DustHourglassFall" (Transformation|GetWorldLocation (Variables|/Script/Engine.Actor|GetRootComponent _asbp_first_person_character)) (Transformation|GetWorldRotation (Variables|/Script/Engine.Actor|GetRootComponent _asbp_first_person_character)) "0.010000,0.010000,0.010000")
      (bind _output_get_2 (Variables|Default|SetBaseWalkspeed (Variables|/Script/Engine.CharacterMovementComponent|GetMaxWalkSpeed (Variables|/Script/Engine.Character|GetCharacterMovement _output_get))))
      (Variables|/Script/Engine.CharacterMovementComponent|SetMaxWalkSpeed (Variables|/Script/Engine.Character|GetCharacterMovement _output_get) (/ _output_get_2 2.0))
      (Utilities|FlowControl|Delay 0.5)
      (Variables|/Script/Engine.CharacterMovementComponent|SetMaxWalkSpeed (Variables|/Script/Engine.Character|GetCharacterMovement _output_get) _output_get_2)
      (Utilities|FlowControl|Delay 2.0)
      (Actor|DestroyActor))))

(fn ConstructionScript)