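; BP_TimerDrone is a drone actor that displays the level's BP_Timer time on its text renders.
; On BeginPlay it posts a looping Wwise flying-idle sound on itself and caches the first BP_Timer found in the world.
; Every Tick it formats that timer's Time with TimeSecondsToString and writes it to two text render components, without re-checking that the timer reference is valid.
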(event EventTick
  (params (DeltaSeconds :type Float%20%28single-precision%29))
  (bind _timeractor (Variables|Default|GetTimerActor))
  (bind _time (Variables|/Game/Project/BP/LD/BP_Timer.BP_Timer_C|GetTime _timeractor))
  (bind _returnvalue (Class|KismetStringLibrary|TimeSecondstoString _time))
  (bind _returnvalue_2 (Utilities|Text|ToText(String) _returnvalue))
  (bind _textrender (Variables|Default|GetTextRender)
    (:then
      (Rendering|Components|TextRender|SetText _textrender _returnvalue_2)
      (bind _textrender1 (Variables|Default|GetTextRender1)
        (:then
          (Rendering|Components|TextRender|SetText _textrender1 _returnvalue_2))
        (:else)))
    (:else)))

(event EventBeginPlay
  (Class|WwiseManagerSubsystem|PostEvent (Subsystems|GetWwiseManagerSubsystem) "/Game/WwiseAudio/Events/FOES_Flying_WU/Play_FOES_SFX_Flying_Idle_LP.Play_FOES_SFX_Flying_Idle_LP" self)
  (bind _returnvalue (Actor|GetActorOfClass "/Game/Project/BP/LD/BP_Timer.BP_Timer_C"))
  (Utilities|IsValid _returnvalue
    (:Is%20Valid
      (Variables|Default|SetTimerActor _returnvalue))))

(fn ConstructionScript)