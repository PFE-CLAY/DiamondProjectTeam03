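; Blueprint function library with a PlaySubtitles function meant to show subtitles from supplied SubtitlesData, but its entry node is unconnected, so calling it does nothing.
; The disconnected logic validates the data table, printing an error if invalid, and checks the SubtitlesActivated game setting.
; It then removes existing top-level UW_Subtitles widgets and adds a new one to the viewport, so only one displays.
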(fn PlaySubtitles
  (params (SubtitlesData :type Data%20Table%20Row%20Handle%20Structure)))