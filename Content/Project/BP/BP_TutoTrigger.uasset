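; Tutorial trigger volume that drives the player's TutosWidget prompts according to the current loop number.
; On BeginPlay it sets ShiftActive on loop 0 and destroys itself after loop 1.
; While ShiftActive, player overlap enables the Shift prompt and leaving disables it, using paired DoOnce gates that reset each other.
; Otherwise, both entering and leaving call KillTab on the widget.
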(event OnComponentBeginOverlap(CollisionComponent)
  (params (OverlappedComponent :type Primitive%20Component%20Object%20Reference) (OtherActor :type Actor%20Object%20Reference) (OtherComp :type Primitive%20Component%20Object%20Reference) (OtherBodyIndex :type Integer) (bFromSweep :type Boolean) (SweepResult :type Hit%20Result%20Structure%20%28by%20ref%29))
  (bind _asbp_first_person_character (Utilities|Casting|CastToBP_FirstPersonCharacter OtherActor))
  (if (Variables|Default|GetShiftActive)
    (Utilities|FlowControl|Sequence
      (:then_0
        (Utilities|FlowControl|DoOnce false) ; enters at Reset
      )
      (:then_1
        (Utilities|FlowControl|DoOnce false
          (:Completed
            (Default|EnableShift (stale _tutoswidget))))))
    (else
      (bind _tutoswidget (Variables|/Game/Project/Game/HUD/HUD_GAME.HUD_GAME_C|GetTutosWidget (Variables|/Game/Project/Game/BP_FirstPersonCharacter.BP_FirstPersonCharacter_C|GetInteractHUD _asbp_first_person_character))
        (:then
          (Default|KillTab _tutoswidget))
        (:else)))))

(event OnComponentEndOverlap(CollisionComponent)
  (params (OverlappedComponent :type Primitive%20Component%20Object%20Reference) (OtherActor :type Actor%20Object%20Reference) (OtherComp :type Primitive%20Component%20Object%20Reference) (OtherBodyIndex :type Integer))
  (bind _asbp_first_person_character (Utilities|Casting|CastToBP_FirstPersonCharacter OtherActor))
  (if (Variables|Default|GetShiftActive)
    (Utilities|FlowControl|Sequence
      (:then_0
        (Utilities|FlowControl|DoOnce false) ; enters at Reset
      )
      (:then_1
        (Utilities|FlowControl|DoOnce false
          (:Completed
            (Default|DisableShift (Variables|/Game/Project/Game/HUD/HUD_GAME.HUD_GAME_C|GetTutosWidget (Variables|/Game/Project/Game/BP_FirstPersonCharacter.BP_FirstPersonCharacter_C|GetInteractHUD _asbp_first_person_character)))))))
    (else
      (bind _tutoswidget (Variables|/Game/Project/Game/HUD/HUD_GAME.HUD_GAME_C|GetTutosWidget (Variables|/Game/Project/Game/BP_FirstPersonCharacter.BP_FirstPersonCharacter_C|GetInteractHUD (stale OnComponentBeginOverlap(CollisionComponent) _asbp_first_person_character)))
        (:then
          (Default|KillTab _tutoswidget))
        (:else)))))

(event EventBeginPlay
  (bind _returnvalue (Subsystems|GetLoopSubsystem))
  (bind _loopnb (Variables|/Script/DiamondProject.LoopSubsystem|GetLoopNb _returnvalue))
  (if (<= _loopnb 1)
    (if (== _loopnb 0)
      (Variables|Default|SetShiftActive true))
    (else
      (Actor|DestroyActor))))

(fn ConstructionScript)