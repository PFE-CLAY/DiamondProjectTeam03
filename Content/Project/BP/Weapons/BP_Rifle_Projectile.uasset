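; Player rifle actor that spins and bobs on looping tweens until ActivateWeapon attaches it to the character and triggers the HUD click tutorial.
; PlayerHitWeapon fire events drive the gun AnimBP, Wwise shot sound and randomized muzzle flash with tweened fade.
; Heat changes feed dynamic materials for an overheat indicator and molten gun metal.
; Overheat activates Niagara and steps the AnimBP through recovery before clearing the overheated flag.
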(event OnOverheatStart(PlayerHitWeapon)
  (|MuzzleFlashFadeAway_2
    (:ReturnTween
      (Components|Activation|Activate (Variables|Default|GetOverHeatNiagara) true))
    (:Return
      (CallFunction|RecoverAnimationEnd))))

(event OnPickUp(TP_PickUp)
  (params (PickUpCharacter :type Diamond%20Project%20Character%20Object%20Reference)))

(event OnFireFinished(PlayerHitWeapon)
  (|MuzzleFlashFadeAway)
  (Variables|/Game/Project/BP/Weapons/Final_Weapon/ABP_Gun.ABP_Gun_C|SetIsShooting (Variables|Default|GetABP%20Gun) false))

(event OnFire(PlayerHitWeapon)
  (params (CurrentAmmo :type Integer) (HitLocation :type Vector :default "0, 0, 0"))
  (if (Variables|Default|GetbIsFiring)
    _
    (else
      (Variables|Default|SetbIsFiring true)
      (Variables|/Game/Project/BP/Weapons/Final_Weapon/ABP_Gun.ABP_Gun_C|SetIsShooting (Variables|Default|GetABP%20Gun) true)
      (Rendering|Material|SetScalarParameterValue (Variables|VFX|GetMuzzleFlashMat) "Value" 1.0 :!class /Script/Engine.MaterialInstanceDynamic)))
  (Class|WwiseManagerSubsystem|PostEvent (Subsystems|GetWwiseManagerSubsystem) "/Game/WwiseAudio/Events/MC_WU/Play_MC_SFX_Gun_Shoot_RC.Play_MC_SFX_Gun_Shoot_RC" self)
  (|DisplayVFX_2))

(event OnHeatChanged(PlayerHitWeapon)
  (params (NewHeat :type Float%20%28single-precision%29))
  (bind _playerhitweapon (Variables|Default|GetPlayerHitWeapon))
  (bind _maxheat (Variables|/Script/DiamondProject.PlayerHitWeaponComponent|GetMaxHeat _playerhitweapon))
  (bind _returnvalue (/ NewHeat _maxheat))
  (bind _returnvalue_2 (Math|Float|Clamp(Float) _returnvalue))
  (Rendering|Material|SetScalarParameterValue (Variables|Default|GetOverheatIndicator) "Value" _returnvalue_2 :!class /Script/Engine.MaterialInstanceDynamic)
  (bind _returnvalue_3 (Rendering|Material|GetScalarParameterValue (Variables|Default|GetGunMaterial) "Value" :!class /Script/Engine.MaterialInstanceDynamic))
  (bind _value (|TweenFloat _returnvalue_3 _returnvalue_2 0.5 "Linear")
    (:ApplyEasing
      (Rendering|Material|SetScalarParameterValue (Variables|Default|GetGunMaterial) "Value" _value :!class /Script/Engine.MaterialInstanceDynamic))))

(event Custom|ActivateWeapon
  (bind _returnvalue (Game|GetPlayerCharacter 0))
  (bind _asdiamond_project_character (Utilities|Casting|CastToDiamondProjectCharacter _returnvalue))
  (Variables|/Script/DiamondProject.PlayerHitWeaponComponent|SetProjectileSpawnPoint (Variables|Default|GetPlayerHitWeapon) (Variables|Default|GetWeaponProjectileSpawnPoint))
  (Class|WeaponComponent|AttachWeapon (Variables|Default|GetPlayerHitWeapon) _asdiamond_project_character)
  (bind _asfirst_person_anim_bp (Utilities|Casting|CastToFirstPerson_AnimBP (Components|SkeletalMesh|GetAnimInstance (Variables|/Script/DiamondProject.DiamondProjectCharacter|GetMesh1P _asdiamond_project_character))))
  (Variables|/Game/FirstPersonArms/Animations/FirstPerson_AnimBP.FirstPerson_AnimBP_C|SetHasRifle _asfirst_person_anim_bp true)
  (CallFunction|StopWeaponFloat)
  (Development|SetHiddeninGame (Variables|Default|GetPlayerHitWeapon) true false)
  (Development|SetHiddeninGame (Variables|Default|GetPlayerHitWeapon) false false)
  (Development|SetHiddeninGame (Variables|/Script/DiamondProject.DiamondProjectCharacter|GetMesh1P _asdiamond_project_character) false false)
  (bind _hud (Variables|Default|GetHUD)
    (:then
      (bind _tutoswidget (Variables|/Game/Project/Game/HUD/HUD_GAME.HUD_GAME_C|GetTutosWidget _hud)
        (:then
          (Variables|/Game/Project/UI/UW_TutosOnboarding.UW_TutosOnboarding_C|SetGunActive _tutoswidget true)
          (Utilities|FlowControl|Delay 4.0)
          (Default|ClickTuto _tutoswidget))
        (:else)))
    (:else)))

(event Custom|Overheat%20End
  (bind _abp_gun (Variables|Default|GetABP%20Gun))
  (Variables|/Game/Project/BP/Weapons/Final_Weapon/ABP_Gun.ABP_Gun_C|SetShouldStartRecover _abp_gun false)
  (Variables|/Game/Project/BP/Weapons/Final_Weapon/ABP_Gun.ABP_Gun_C|SetIsRecovering _abp_gun false)
  (Utilities|FlowControl|Delay 0.8)
  (Variables|/Script/DiamondProject.PlayerHitWeaponComponent|SetbIsOverheated (Variables|Default|GetPlayerHitWeapon) false))

(event Custom|RecoverAnimationEnd
  (Variables|/Game/Project/BP/Weapons/Final_Weapon/ABP_Gun.ABP_Gun_C|SetIsRecovering (Variables|Default|GetABP%20Gun) true)
  (Utilities|FlowControl|Delay 0.5)
  (Variables|/Game/Project/BP/Weapons/Final_Weapon/ABP_Gun.ABP_Gun_C|SetShouldStartRecover (Variables|Default|GetABP%20Gun) true))

(event EventBeginPlay
  (bind _asabp_gun (Utilities|Casting|CastToABP_Gun (Components|SkeletalMesh|GetAnimInstance (Variables|Default|GetPlayerHitWeapon))))
  (Variables|Default|SetABP%20Gun _asabp_gun)
  (bind _returnvalue (Rendering|Material|CreateDynamicMaterialInstance (Variables|Default|GetMuzzleFlash) 0 "/Game/Project/Materials/M_MuzzleFlash.M_MuzzleFlash" "" :!class /Script/Engine.PrimitiveComponent))
  (Variables|VFX|SetMuzzleFlashMat _returnvalue)
  ;[0.15 0.15 0.15 0.5] Material instances creation
  (bind _returnvalue_2 (Rendering|Material|CreateDynamicMaterialInstance (Variables|Default|GetNoise) 0 "/Game/Project/UI/UIAssets/Materials/UI_flingue_bruit_Mat.UI_flingue_bruit_Mat" "Value" :!class /Script/Engine.PrimitiveComponent))
  (Variables|Default|SetOverheatIndicator _returnvalue_2)
  (bind _returnvalue_3 (Rendering|Material|CreateDynamicMaterialInstance (Variables|Default|GetPlayerHitWeapon) 1 "/Game/Project/Materials/Gun/M_MoltenMetal.M_MoltenMetal" "None" :!class /Script/Engine.PrimitiveComponent))
  (Variables|Default|SetGunMaterial _returnvalue_3)
  (bind _ashud_game (Utilities|Casting|CastToHUD_GAME (HUD|GetHUD (Game|GetPlayerController 0))))
  (Variables|Default|SetHUD _ashud_game)
  (Utilities|FlowControl|Sequence
    (:then_0
      (|WeaponRotateAndFloatLoop))
    (:then_1
      (bind _asbp_first_person_character (Utilities|Casting|CastToBP_FirstPersonCharacter (Game|GetPlayerCharacter 0)))
      (Variables|VFX|SetDefaultFOV (Variables|/Script/Engine.CameraComponent|GetFieldOfView (Variables|/Script/DiamondProject.DiamondProjectCharacter|GetFirstPersonCameraComponent _asbp_first_person_character)))
      (EventDispatchers|BindEventtoOnOverheatEnd (Variables|Default|GetPlayerHitWeapon) (delegate Custom|Overheat%20End)))))

(fn ConstructionScript
  (|CallParentFunction))

(event Custom|StopWeaponFloat
  (bind _async_float_task (Variables|Default|GetAsync%20float%20task)
    (:then
      (Class|FCTweenBPAction|Stop _async_float_task)
      (bind _async_rotation_task (Variables|Default|GetAsync%20Rotation%20task)
        (:then
          (Class|FCTweenBPAction|Stop _async_rotation_task))
        (:else)))
    (:else)))