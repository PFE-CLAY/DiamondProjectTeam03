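; Hourglass actor that visually tracks the level's BP_Timer by fading its top, tube and bottom shader meshes, with a looping Wwise idle sound.
; BeginPlay creates a dynamic material per mesh, reads the timer's duration and binds ActivateFade to its start event.
; Float tweens drive each "Fade" parameter: top over the first half, tubes over the second, bottom inversely across the whole duration.
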(event Custom|ActivateFade
  (bind (_asynctaskproxy _value) (|TweenFloat 0.0 1.0 (/ (Variables|Default|GetTotalFadeDuration) 2.0) "InOutQuad")
    (:then
      (Variables|Default|SetTopTask _asynctaskproxy)
      (bind (_asynctaskproxy_2 _value_2) (|TweenFloat 1.0 0.0 (Variables|Default|GetTotalFadeDuration) "InOutQuad")
        (:then
          (Variables|Default|SetBottomTask _asynctaskproxy_2))
        (:ApplyEasing
          (Rendering|Material|SetScalarParameterValue (Variables|Default|GetBottomMat) "Fade" _value_2 :!class /Script/Engine.MaterialInstanceDynamic))))
    (:ApplyEasing
      (Rendering|Material|SetScalarParameterValue (Variables|Default|GetTopMat) "Fade" _value :!class /Script/Engine.MaterialInstanceDynamic))
    (:OnComplete
      (bind (_asynctaskproxy_3 _value_3) (|TweenFloat 0.0 1.0 (/ (Variables|Default|GetTotalFadeDuration) 2.0) "InOutQuad")
        (:then
          (Variables|Default|SetTubesTask _asynctaskproxy_3))
        (:ApplyEasing
          (Rendering|Material|SetScalarParameterValue (Variables|Default|GetTubesMat) "Fade" _value_3 :!class /Script/Engine.MaterialInstanceDynamic))))))

(event EventBeginPlay
  (Class|WwiseManagerSubsystem|PostEvent (Subsystems|GetWwiseManagerSubsystem) "/Game/WwiseAudio/Events/SFX_WU/Play_SFX_HourGlass_Idle_LP.Play_SFX_HourGlass_Idle_LP" self)
  (Utilities|FlowControl|Sequence
    (:then_0
      (bind _returnvalue (Rendering|Material|CreateDynamicMaterialInstance "/Game/Project/Materials/Black_Sand/Sh_BS_Inst_Haut.Sh_BS_Inst_Haut" "" "None" :!class /Script/Engine.KismetMaterialLibrary))
      (bind _output_get (Variables|Default|SetTopMat _returnvalue))
      (Rendering|Material|SetMaterial (Variables|Default|GetMeshShader_ShaderHaut) 0 _output_get))
    (:then_1
      (bind _returnvalue_2 (Rendering|Material|CreateDynamicMaterialInstance "/Game/Project/Materials/Black_Sand/Sh_BS_Inst_Tube.Sh_BS_Inst_Tube" "" "None" :!class /Script/Engine.KismetMaterialLibrary))
      (bind _output_get_2 (Variables|Default|SetTubesMat _returnvalue_2))
      (Rendering|Material|SetMaterial (Variables|Default|GetMeshShader_ShaderTube) 0 _output_get_2))
    (:then_2
      (bind _returnvalue_3 (Rendering|Material|CreateDynamicMaterialInstance "/Game/Project/Materials/Black_Sand/Sh_BS_Inst_Bas.Sh_BS_Inst_Bas" "" "None" :!class /Script/Engine.KismetMaterialLibrary))
      (bind _output_get_3 (Variables|Default|SetBottomMat _returnvalue_3))
      (Rendering|Material|SetMaterial (Variables|Default|GetMeshShader_ShaderBas) 0 _output_get_3)
      (Rendering|Material|SetScalarParameterValue (Variables|Default|GetBottomMat) "Fade" 1.0 :!class /Script/Engine.MaterialInstanceDynamic))
    (:then_3
      (bind _returnvalue_4 (Actor|GetActorOfClass "/Game/Project/BP/LD/BP_Timer.BP_Timer_C"))
      (Utilities|IsValid _returnvalue_4
        (:Is%20Valid
          (Variables|Default|SetTotalFadeDuration (Variables|/Game/Project/BP/LD/BP_Timer.BP_Timer_C|GetTime _returnvalue_4))
          (EventDispatchers|BindEventtoOnTimerStarted _returnvalue_4 (delegate Custom|ActivateFade)))))))

(fn ConstructionScript)