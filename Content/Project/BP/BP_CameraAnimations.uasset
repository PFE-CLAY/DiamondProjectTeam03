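; Short-lived actor that plays camera animations and shakes for player moves such as landing and wall dashes.
; The sequence and landing events start an animation through the Engine Cameras subsystem, begin blending the view to this actor, then immediately call EndCameraAnimation.
; That event returns the view to the player character and destroys the actor one second later.
; Wall dash only plays a world camera shake; the explicit animation stop is unconnected.
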(event Custom|PlayWallDash
  (Camera|PlayWorldCameraShake "/Game/Project/BP/CameraShake/BP_DashWallCamShake.BP_DashWallCamShake_C" "0, 0, 0" 3e+13 0.0))

(event Custom|PlayLandingAnim
  (bind _returnvalue (Game|GetPlayerController 0))
  (bind _returnvalue_2 (Class|EngineCamerasSubsystem|PlayCameraAnimation (Subsystems|GetEngineCamerasSubsystem) _returnvalue "/Game/Project/CameraAnim/CAS_LandingAnim.CAS_LandingAnim"))
  (Variables|Default|SetAnim _returnvalue_2)
  (Game|Player|SetViewTargetwithBlend _returnvalue self 0.5 "VTBlend_EaseInOut" 0.0 false)
  (Development|PrintString "PlayCameraAnim")
  (CallFunction|EndCameraAnimation))

(event Custom|EndCameraAnimation
  (Game|Player|SetViewTargetwithBlend (Game|GetPlayerController 0) (Game|GetPlayerCharacter 0) 0.0 "VTBlend_Linear" 0.0 false)
  (Development|PrintString "StopCameraAnim")
  (Utilities|FlowControl|Delay 1.0)
  (Actor|DestroyActor))

(event Custom|PlayAnimationSequence
  (params (Sequence :type Camera%20Animation%20Sequence%20Object%20Reference))
  (bind _returnvalue (Game|GetPlayerController 0))
  (bind _returnvalue_2 (Class|EngineCamerasSubsystem|PlayCameraAnimation (Subsystems|GetEngineCamerasSubsystem) _returnvalue Sequence))
  (Variables|Default|SetAnim _returnvalue_2)
  (Game|Player|SetViewTargetwithBlend _returnvalue self 0.5 "VTBlend_EaseInOut" 0.0 false)
  (Development|PrintString "PlayCameraAnim")
  (CallFunction|EndCameraAnimation))

(fn ConstructionScript)