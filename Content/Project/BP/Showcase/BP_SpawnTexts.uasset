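; Showcase actor that reveals wall-style story texts and tally-count texts according to the current loop number from the loop subsystem.
; On BeginPlay it builds two component-to-index maps and shows entries up to that loop, refreshing the story map inside every tally iteration.
; It calls highlight events for the newest entries, but both are empty.
; Their dynamic-material "Brillance" tween logic is left disconnected and never runs.
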(event Custom|RatureHighlight
  (params (Index :type Primitive%20Component%20Object%20Reference)))

(event Custom|NewTextsHighligh
  (params (Index :type Primitive%20Component%20Object%20Reference)))

(event EventBeginPlay
  (bind _returnvalue (Subsystems|GetLoopSubsystem))
  (bind _loopnb (Variables|/Script/DiamondProject.LoopSubsystem|GetLoopNb _returnvalue))
  (Variables|Default|SetLoopNum _loopnb)
  (|InitStory)
  (|InitialisationComptesLoop)
  ;[0 0.8613 1 0.5] C'EST FIX JVAIS PLEURER
  (CallFunction|RatureHighlight (.Key (Utilities|Map|GetKeyValueByIndex (Variables|Default|GetIndexRature) (Math|Integer|Clamp(Integer) (- _loopnb 1) 0 100))))
  (bind (_keypin _valuepin) (Utilities|Map|ForEachLoop(Map) (Variables|Default|GetIndexRature))
    (:then
      (Rendering|SetVisibility _keypin (< _valuepin (Variables|Default|GetLoopNum)) false)
      (|Masquerethighlightstory))))

(fn ConstructionScript)