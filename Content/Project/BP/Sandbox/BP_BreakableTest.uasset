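; Sandbox test actor for a breakable Geometry Collection that reacts to a break event or to the first-person character hitting it.
; It binds to OnBreakMesh at BeginPlay, then on that event enables gravity and triggers a short-lived FS_MasterField at the hit location.
; A component hit from BP_FirstPersonCharacter triggers a larger, stronger radial field at the impact point, without changing gravity.
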(event OnComponentHit(GeometryCollection)
  (params (HitComponent :type Primitive%20Component%20Object%20Reference) (OtherActor :type Actor%20Object%20Reference) (OtherComp :type Primitive%20Component%20Object%20Reference) (NormalImpulse :type Vector :default "0, 0, 0") (Hit :type Hit%20Result%20Structure%20%28by%20ref%29))
  (Utilities|Casting|CastToBP_FirstPersonCharacter OtherActor)
  (bind _returnvalue (Game|SpawnActorfromClass "/Engine/EditorResources/FieldNodes/FS_MasterField.FS_MasterField_C" (Math|Transform|MakeTransform (.location Hit) "0, 0, 0" "1.500000,1.500000,1.500000") "Undefined" "MultiplyWithRoot" 0 0))
  (Variables|/Engine/EditorResources/FieldNodes/FS_MasterField.FS_MasterField_C|SetActivationType _returnvalue "NewEnumerator4")
  (Variables|/Engine/EditorResources/FieldNodes/FS_MasterField.FS_MasterField_C|SetRadial%20Magnitude _returnvalue 1.5e+02)
  (Variables|/Engine/EditorResources/FieldNodes/FS_MasterField.FS_MasterField_C|SetFieldLifespan _returnvalue 0.1)
  (Default|CETrigger _returnvalue))

(event Custom|OnBreakMesh_Event
  (params (HitLocation :type Vector))
  (Physics|SetEnableGravity (Variables|Default|GetGeometryCollection) true)
  (bind _returnvalue (Game|SpawnActorfromClass "/Engine/EditorResources/FieldNodes/FS_MasterField.FS_MasterField_C" (Math|Transform|MakeTransform HitLocation "0, 0, 0" "1.000000,1.000000,1.000000") "Undefined" "MultiplyWithRoot" 0 0))
  (Variables|/Engine/EditorResources/FieldNodes/FS_MasterField.FS_MasterField_C|SetActivationType _returnvalue "NewEnumerator4")
  (Variables|/Engine/EditorResources/FieldNodes/FS_MasterField.FS_MasterField_C|SetRadial%20Magnitude _returnvalue 5e+01)
  (Variables|/Engine/EditorResources/FieldNodes/FS_MasterField.FS_MasterField_C|SetFieldLifespan _returnvalue 0.1)
  (Default|CETrigger _returnvalue))

(event EventBeginPlay
  (EventDispatchers|AssignOnBreakMesh (delegate Custom|OnBreakMesh_Event)))

(fn ConstructionScript)