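; Test breakable Geometry Collection actor that shatters when hit by a dashing first-person character or an enemy projectile, or on a break-mesh event.
; Breaking enables gravity, spawns a short-lived radial physics field at the hit point and plays a particle effect.
; Dash hits also trigger debounced juice: a temporary vignette, wall-dash camera animation and delayed relaunch at entry velocity.
; The dash path destroys the actor after a cleanup delay.
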(event OnComponentHit(GeometryCollection)
  (params (HitComponent :type Primitive%20Component%20Object%20Reference) (OtherActor :type Actor%20Object%20Reference) (OtherComp :type Primitive%20Component%20Object%20Reference) (NormalImpulse :type Vector :default "0, 0, 0") (Hit :type Hit%20Result%20Structure%20%28by%20ref%29))
  (bind _asbp_first_person_character (Utilities|Casting|CastToBP_FirstPersonCharacter OtherActor)
    (:then
      (if (Variables|/Game/Project/Game/BP_FirstPersonCharacter.BP_FirstPersonCharacter_C|GetisDashing _asbp_first_person_character)
        (Utilities|FlowControl|Sequence
          (:then_0
            (CallFunction|SpawnBreakableField (.location Hit) :!label _label))
          (:then_1
            (|DashWalljuice _asbp_first_person_character))
          (:then_2
            ;[1 0 0 0.8899] Just Cleaning
            (Utilities|FlowControl|Delay 2e+01)
            (Utilities|FlowControl|Delay 0.5)
            (Actor|DestroyActor)))))
    (:CastFailed
      (Utilities|Casting|CastToProjectileEnemy OtherActor)
      (goto _label))))

(event Custom|OnBreakMesh_Event
  (params (HitLocation :type Vector))
  (Physics|SetEnableGravity (Variables|Default|GetGeometryCollection) true)
  (CallFunction|SpawnBreakableField HitLocation))

(event EventBeginPlay
  (EventDispatchers|AssignOnBreakMesh (delegate Custom|OnBreakMesh_Event)))

(fn ConstructionScript)

(fn SpawnBreakableField
  (params (spawn%20location :type Vector))
  (bind _geometrycollection (Variables|Default|GetGeometryCollection))
  (Physics|SetEnableGravity (Variables|Default|GetGeometryCollection) true)
  (bind _returnvalue (Game|SpawnActorfromClass "/Game/Project/BP/Sandbox/BreakableObjects/FS_BlacksandsField.FS_BlacksandsField_C" (Math|Transform|MakeTransform spawn%20location "0, 0, 0" "1.000000,1.000000,1.000000") "Undefined" "MultiplyWithRoot" 0 0))
  (Variables|/Engine/EditorResources/FieldNodes/FS_MasterField.FS_MasterField_C|SetActivationType _returnvalue "NewEnumerator4")
  (Variables|/Engine/EditorResources/FieldNodes/FS_MasterField.FS_MasterField_C|SetRadial%20Magnitude _returnvalue 5e+02)
  (Variables|/Engine/EditorResources/FieldNodes/FS_MasterField.FS_MasterField_C|SetFieldLifespan _returnvalue 0.5)
  (Default|CETrigger _returnvalue)
  (Niagara|SpawnSystematLocation (Variables|Default|GetParticle%20effect) (Transformation|GetWorldLocation _geometrycollection) (Transformation|GetWorldRotation _geometrycollection)))