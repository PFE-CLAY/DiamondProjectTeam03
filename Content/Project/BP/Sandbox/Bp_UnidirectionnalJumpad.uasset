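; Sunlight-powered unidirectional jump pad that only has jump force while its MultiSunlightDetector reports sun activation.
; BeginPlay caches JumpForce, zeroes it so the pad starts inactive, and shows the DirectionVisualizer.
; Sun activation changes restore or zero the force, toggle the pad VFX and the child-actor BP_SunFollower effects, and update the illuminated state.
; The launch itself is not implemented in these graphs.
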(event OnSunActivationChanged(MultiSunlightDetector)
  (params (IsActivated :type Boolean))
  (bind _sunfollower (Variables|Default|GetSunFollower))
  (bind _vfx (Variables|Default|GetVFX))
  (bind _childactor (Variables|/Script/Engine.ChildActorComponent|GetChildActor _sunfollower))
  (bind _asbp_sun_follower (Utilities|Casting|CastToBP_SunFollower _childactor))
  (if IsActivated
    (Variables|Default|SetJumpForce (Variables|Default|GetinitialJumpforce))
    (Components|Activation|Activate _vfx false)
    (Default|ActivateVFX _asbp_sun_follower)
    (else
      (Variables|Default|SetJumpForce 0.0)
      (Components|Activation|Deactivate _vfx)
      (Default|DeactivateVFX _asbp_sun_follower)))
  (Class|JumpPad|SetIsJumpadIlluminated IsActivated))

(event EventBeginPlay
  (Variables|Default|SetinitialJumpforce (Variables|Default|GetJumpForce))
  (Variables|Default|SetJumpForce 0.0)
  (Rendering|SetVisibility (Variables|Default|GetDirectionVisualizer) true false))

(fn ConstructionScript)