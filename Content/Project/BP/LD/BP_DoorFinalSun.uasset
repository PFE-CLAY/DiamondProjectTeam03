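; Final sun door whose two lateral meshes slide apart along X on a timeline when its MultiSunlightDetector activates, and reverse when it deactivates.
; Sun changes also trigger the "door_open" preplan step, toggle the child SunFollower's VFX and switch the PathPoint's wanted path index.
; After a short delay, player overlap with the box either opens the door or, for the pyramid variant, plays an arena dub line and destroys the box.
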(event OnSunActivationChanged(MultiSunlightDetector)
  (params (IsActivated :type Boolean))
  (bind _ssuunn (Variables|Default|GetSSUUNN))
  (bind _pathpoint (Variables|Default|GetPathPoint))
  (bind _childactor (Variables|/Script/Engine.ChildActorComponent|GetChildActor _ssuunn))
  (bind _asbp_sun_follower (Utilities|Casting|CastToBP_SunFollower _childactor))
  (Class|LoopSubsystem|ActivatePreplanStep (Subsystems|GetLoopSubsystem) "door_open")
  (bind _output_get (Variables|Default|SetSun%20is%20Activate%20? IsActivated))
  (if _output_get
    (Default|ActivateVFX _asbp_sun_follower)
    (Utilities|IsValid _pathpoint
      (:Is%20Valid
        (Variables|/Script/DiamondProject.CustomNavigationPoint|SetWantedPathIndex _pathpoint 1))
      (:Is%20Not%20Valid
        _))
    (else
      (Default|DeactivateVFX _asbp_sun_follower)
      (Utilities|IsValid 0
        (:Is%20Valid
          (Variables|/Script/DiamondProject.CustomNavigationPoint|SetWantedPathIndex _pathpoint 0))
        (:Is%20Not%20Valid
          _))))
  (CallFunction|DoorMove))

(event OnComponentBeginOverlap(Box)
  (params (OverlappedComponent :type Primitive%20Component%20Object%20Reference) (OtherActor :type Actor%20Object%20Reference) (OtherComp :type Primitive%20Component%20Object%20Reference) (OtherBodyIndex :type Integer) (bFromSweep :type Boolean) (SweepResult :type Hit%20Result%20Structure%20%28by%20ref%29))
  (bind _sm_lateraldoor (Variables|Default|GetSM_LateralDoor))
  (bind _sm_lateraldoor1 (Variables|Default|GetSM_LateralDoor1))
  (bind _relativelocation (Variables|/Script/Engine.SceneComponent|GetRelativeLocation _sm_lateraldoor))
  (bind _relativelocation_2 (Variables|/Script/Engine.SceneComponent|GetRelativeLocation _sm_lateraldoor1))
  (if true
    (if (== OtherActor (Game|GetPlayerCharacter 0))
      (Utilities|FlowControl|Delay 0.3)
      (if (Variables|Default|GetIsPyramid)
        (Class|WwiseManagerSubsystem|PostEvent (Subsystems|GetWwiseManagerSubsystem) "/Game/WwiseAudio/Events/VOICES_WU/Play_DUB_ARENA_1_3_0.Play_DUB_ARENA_1_3_0" self)
        (bind _box (Variables|Default|GetBox)
          (:then
            (Components|DestroyComponent _box))
          (:else))
        (else
          (bind _door_movement (Timeline|DoorMovement Play)
            (:Update
              (Transformation|SetRelativeLocation _sm_lateraldoor1 (Math|Vector|MakeVector (* _door_movement -1.0) (.y _relativelocation_2) (.z _relativelocation_2)) false false)
              (Transformation|SetRelativeLocation _sm_lateraldoor (Math|Vector|MakeVector _door_movement (.y _relativelocation) (.z _relativelocation)) false false))))))))

(event Custom|DoorMove
  (bind _sm_lateraldoor (Variables|Default|GetSM_LateralDoor))
  (bind _sm_lateraldoor1 (Variables|Default|GetSM_LateralDoor1))
  (bind _relativelocation (Variables|/Script/Engine.SceneComponent|GetRelativeLocation _sm_lateraldoor))
  (bind _relativelocation_2 (Variables|/Script/Engine.SceneComponent|GetRelativeLocation _sm_lateraldoor1))
  (if (Variables|Default|GetSun%20is%20Activate%20?)
    (bind _door_movement (Timeline|DoorMovement Play)
      (:Update
        (Transformation|SetRelativeLocation _sm_lateraldoor1 (Math|Vector|MakeVector (* _door_movement -1.0) (.y _relativelocation_2) (.z _relativelocation_2)) false false)
        (Transformation|SetRelativeLocation _sm_lateraldoor (Math|Vector|MakeVector _door_movement (.y _relativelocation) (.z _relativelocation)) false false)))
    (else
      (Timeline|DoorMovement Reverse))))

(event Custom|DoorClose
  (bind _sm_lateraldoor (Variables|Default|GetSM_LateralDoor))
  (bind _sm_lateraldoor1 (Variables|Default|GetSM_LateralDoor1))
  (bind _relativelocation (Variables|/Script/Engine.SceneComponent|GetRelativeLocation _sm_lateraldoor))
  (bind _relativelocation_2 (Variables|/Script/Engine.SceneComponent|GetRelativeLocation _sm_lateraldoor1))
  (bind _door_movement (Timeline|DoorMovement Reverse)
    (:Update
      (Transformation|SetRelativeLocation _sm_lateraldoor1 (Math|Vector|MakeVector (* _door_movement -1.0) (.y _relativelocation_2) (.z _relativelocation_2)) false false)
      (Transformation|SetRelativeLocation _sm_lateraldoor (Math|Vector|MakeVector _door_movement (.y _relativelocation) (.z _relativelocation)) false false))))

(fn ConstructionScript)