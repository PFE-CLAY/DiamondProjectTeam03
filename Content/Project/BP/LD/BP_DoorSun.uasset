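; BP_DoorSun is a level-design double sliding door that opens and closes according to sunlight activation.
; Its MultiSunlightDetector reports activation changes, which set the SunIsActivate state, trigger DoorsMoving and make the Active component visible.
; DoorsMoving plays or reverses the DoorMovement timeline, sliding the two lateral meshes in opposite directions along relative X.
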(event OnSunActivationChanged(MultiSunlightDetector)
  (params (IsActivated :type Boolean))
  (Variables|Default|SetSun%20is%20Activate%20? IsActivated)
  (CallFunction|DoorsMoving)
  (Rendering|SetVisibility (Variables|Default|GetActive) true false))

(event Custom|DoorsMoving
  (bind _sm_lateraldoor (Variables|Default|GetSM_LateralDoor))
  (bind _sm_lateraldoor1 (Variables|Default|GetSM_LateralDoor1))
  (bind _relativelocation (Variables|/Script/Engine.SceneComponent|GetRelativeLocation _sm_lateraldoor))
  (bind _relativelocation_2 (Variables|/Script/Engine.SceneComponent|GetRelativeLocation _sm_lateraldoor1))
  (if (Variables|Default|GetSun%20is%20Activate%20?)
    (bind _door_movement (Timeline|DoorMovement Play)
      (:Update
        (Transformation|SetRelativeLocation _sm_lateraldoor1 (Math|Vector|MakeVector (* _door_movement -1.0) (.y _relativelocation_2) (.z _relativelocation_2)) false false)
        (Transformation|SetRelativeLocation _sm_lateraldoor (Math|Vector|MakeVector _door_movement (.y _relativelocation) (.z _relativelocation)) false false)))
    (else
      (Timeline|DoorMovement Reverse))))

(fn ConstructionScript)