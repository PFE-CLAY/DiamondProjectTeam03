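; Interactable generator placed in the level that can be activated once to power a linked generator door.
; On interact it disables further use, swaps the cube to a tooltip material and turns its point light green, then notifies its BP_GeneratorsDoor.
; If the door cast succeeds, it also activates a configurable preplan step and the fixed "NoShield" step in the loop subsystem.
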(event EventOnInteract
  (params (InteractingPlayer :type Character%20Object%20Reference))
  (if (Variables|Default|GetCanBeInteractedWith)
    (Variables|Default|SetCanBeInteractedWith false)
    (Rendering|Material|SetMaterial (Variables|Default|GetCube) 0 "/Game/BlockingStarterPack/Blueprints/Others/BlockingTooltip/M_BlockingTooltipBase.M_BlockingTooltipBase")
    (Rendering|Components|Light|SetLightColor (Variables|Default|GetPointLight) "(R=0.000000,G=1.000000,B=0.210394,A=1.000000)" true)
    (bind _asbp_generators_door (Utilities|Casting|CastToBP_GeneratorsDoor (Variables|Default|GetDoor)))
    (Default|GeneratorActivated _asbp_generators_door)
    (Class|LoopSubsystem|ActivatePreplanStep (Subsystems|GetLoopSubsystem) (Variables|Default|GetPrePlanIdToCall))
    (Class|LoopSubsystem|ActivatePreplanStep (Subsystems|GetLoopSubsystem) "NoShield")))

(fn ConstructionScript)