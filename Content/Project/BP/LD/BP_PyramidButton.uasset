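; BP_PyramidButton is an interactable button that opens the pyramid and its door.
; Each interaction plays a Wwise sound and opens the level's BP_DoorPyramid, found by class, if it is not already open.
; A DoOnce then opens the referenced Pyramid, turns the button material red, activates the "open_pyramid" preplan step in LoopSubsystem, and destroys a Target actor after a short delay.
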(event EventOnInteract
  (params (InteractingPlayer :type Character%20Object%20Reference))
  (bind _target (Variables|Default|GetTarget))
  (Class|WwiseManagerSubsystem|PostEvent (Subsystems|GetWwiseManagerSubsystem) "/Game/WwiseAudio/Events/SFX_WU/Play_SFX_Button_Backstage.Play_SFX_Button_Backstage" self)
  (bind _returnvalue (Actor|GetActorOfClass "/Game/Project/BP/LD/BP_DoorPyramid.BP_DoorPyramid_C"))
  (Utilities|IsValid _returnvalue
    (:Is%20Valid
      (if (Variables|/Game/Project/BP/LD/BP_DoorPyramid.BP_DoorPyramid_C|GetIsOpened _returnvalue)
        _
        (else
          (Default|OpenfromButton _returnvalue))))
    (:Is%20Not%20Valid
      _))
  (Utilities|FlowControl|DoOnce false
    (:Completed
      (Default|OPEN! (Variables|Default|GetPyramid))
      (Rendering|Material|SetMaterial (Variables|Default|GetCube) 1 "/Game/Project/Assets/Interactive_Button/M_Interactive_Button_Red.M_Interactive_Button_Red")
      (Class|LoopSubsystem|ActivatePreplanStep (Subsystems|GetLoopSubsystem) "open_pyramid" 1)
      (Utilities|FlowControl|Delay 1.0)
      (Utilities|IsValid _target
        (:Is%20Valid
          (Actor|DestroyActor _target))))))

(fn ConstructionScript
  (|CallParentFunction))