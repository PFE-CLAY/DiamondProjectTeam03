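; BP_EasterEggZone is a zone actor that triggers a hidden material effect when the player stays in its box.
; Shortly after BeginPlay it checks once for player overlap and starts a timer, which tweens the "Scale" parameter on a dynamic M_Preplan material applied to BP_InteractablePreplan's cube.
; Leaving the box only prints a debug string; the timer-cancel and self-destroy logic is disconnected.
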(event OnComponentEndOverlap(Box)
  (params (OverlappedComponent :type Primitive%20Component%20Object%20Reference) (OtherActor :type Actor%20Object%20Reference) (OtherComp :type Primitive%20Component%20Object%20Reference) (OtherBodyIndex :type Integer))
  (Development|PrintString "Hello"))

(event Custom|SpecialEffect
  (bind _value (|TweenFloat 0.0 1.0 1.0 "InOutQuad")
    (:ApplyEasing
      (Rendering|Material|SetScalarParameterValue (Variables|Default|GetMatPreplan) "Scale" _value :!class /Script/Engine.MaterialInstanceDynamic))))

(event Custom|CheckCollision
  (if (Collision|IsOverlappingActor (Variables|Default|GetBox) (Variables|Default|GetPlayer) :!class /Script/Engine.PrimitiveComponent)
    (CallFunction|StartTimer)))

(event Custom|Start%20Timer
  (bind _returnvalue (Utilities|Time|SetTimerbyEvent (delegate Custom|SpecialEffect) (Variables|Default|GetTimeToStayBeforeEffect)))
  (Variables|Default|SetTimer _returnvalue))

(event EventBeginPlay
  (Variables|Default|SetPlayer (Game|Player|GetPlayerPawn 0))
  (bind _returnvalue (Actor|GetActorOfClass "/Game/Project/BP/LD/Preplan/BP_InteractablePreplan.BP_InteractablePreplan_C"))
  (bind _returnvalue_2 (Rendering|Material|CreateDynamicMaterialInstance (Variables|/Game/Project/BP/LD/BP_InteractButton.BP_InteractButton_C|GetCube _returnvalue) 0 "/Game/Project/Assets/Preplan/M_Preplan.M_Preplan" "None" :!class /Script/Engine.PrimitiveComponent))
  (Variables|Default|SetMatPreplan _returnvalue_2)
  (Utilities|FlowControl|Delay 0.2)
  (CallFunction|CheckCollision))

(fn ConstructionScript)