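; Level-design interactable that starts the arena elevator when the player interacts with it.
; On interact it posts the arena dub line through Wwise, then activates the InterpToMovement component on the referenced Elevator.
; If that component exists, it also triggers the "arena" preplan step in the LoopSubsystem, plays the player's helmet animation and destroys itself.
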(event EventOnInteract
  (params (InteractingPlayer :type Character%20Object%20Reference))
  (bind _elevator (Variables|Default|GetElevator))
  (bind _returnvalue (Actor|GetComponentbyClass _elevator "/Script/Engine.InterpToMovementComponent"))
  (Utilities|FlowControl|Delay 0.0)
  (Class|WwiseManagerSubsystem|PostEvent (Subsystems|GetWwiseManagerSubsystem) "/Game/WwiseAudio/Events/VOICES_WU/Play_DUB_ARENA_1_0_0.Play_DUB_ARENA_1_0_0" self)
  (Utilities|IsValid _returnvalue
    (:Is%20Valid
      (Components|Activation|Activate _returnvalue true)
      (Class|LoopSubsystem|ActivatePreplanStep (Subsystems|GetLoopSubsystem) "arena")
      (bind _asbp_first_person_character (Utilities|Casting|CastToBP_FirstPersonCharacter (Game|GetPlayerCharacter 0))
        (:then
          (Default|ActivateAnimationHelmet _asbp_first_person_character))
        (:CastFailed
          _))
      (Actor|DestroyActor))))

(fn ConstructionScript
  (|CallParentFunction))