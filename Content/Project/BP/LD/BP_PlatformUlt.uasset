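; BP_PlatformUlt is a moving platform that crushes the first-person character with a killbox on its return trip.
; Activate or ChangeTargetPosition, ignored while moving, tweens it by a translation offset, holds for a lock delay, then tweens it back.
; The killbox is live only during the return, deals lethal damage through the character's HealthComponent, then switches off.
; The construction script applies the cover box material.
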(event OnComponentBeginOverlap(Killbox)
  (params (OverlappedComponent :type Primitive%20Component%20Object%20Reference) (OtherActor :type Actor%20Object%20Reference) (OtherComp :type Primitive%20Component%20Object%20Reference) (OtherBodyIndex :type Integer) (bFromSweep :type Boolean) (SweepResult :type Hit%20Result%20Structure%20%28by%20ref%29))
  (bind _asbp_first_person_character (Utilities|Casting|CastToBP_FirstPersonCharacter OtherActor))
  (Class|ACHealth|DecreaseHealth (Variables|/Game/Project/Game/BP_FirstPersonCharacter.BP_FirstPersonCharacter_C|GetHealth%20Component _asbp_first_person_character) 10000 self)
  (Collision|SetCollisionEnabled (Variables|Default|GetKillbox) "NoCollision"))

(event Custom|Activate
  (if (not (Variables|Default|GetIsMoving))
    (Variables|Default|SetIsMoving true)
    (bind _value (|TweenVector (Variables|Default|GetBasePos) (Variables|Default|GetTargetPos) (Variables|Default|GetDuration%20to%20move) "InOutQuad")
      (:ApplyEasing
        (Transformation|SetActorLocation _value false false))
      (:OnComplete
        (Utilities|FlowControl|Delay (Variables|Default|GetDuration%20lock))
        (Collision|SetCollisionEnabled (Variables|Default|GetKillbox) "QueryAndPhysics")
        (bind _value_2 (|TweenVector (Variables|Default|GetTargetPos) (Variables|Default|GetBasePos) (Variables|Default|GetDuration%20to%20move) "InOutQuad")
          (:ApplyEasing
            (Transformation|SetActorLocation _value_2 false false))
          (:OnComplete
            (Variables|Default|SetIsMoving false)
            (Collision|SetCollisionEnabled (Variables|Default|GetKillbox) "NoCollision")))))))

(event EventBeginPlay
  (Collision|SetCollisionEnabled (Variables|Default|GetKillbox) "NoCollision")
  (Variables|Default|SetBasePos (Transformation|GetActorLocation))
  (Variables|Default|SetTargetPos (+ (Variables|Default|GetBasePos) (Variables|Default|GetTranslationVector))))

(event EventChangeTargetPosition
  (if (not (Variables|Default|GetIsMoving))
    (Variables|Default|SetIsMoving true)
    (bind _value (|TweenVector (Variables|Default|GetBasePos) (Variables|Default|GetTargetPos) (Variables|Default|GetDuration%20to%20move) "InOutQuad")
      (:ApplyEasing
        (Transformation|SetActorLocation _value false false))
      (:OnComplete
        (Utilities|FlowControl|Delay (Variables|Default|GetDuration%20lock))
        (Collision|SetCollisionEnabled (Variables|Default|GetKillbox) "QueryAndPhysics")
        (bind _value_2 (|TweenVector (Variables|Default|GetTargetPos) (Variables|Default|GetBasePos) (Variables|Default|GetDuration%20to%20move) "InOutQuad")
          (:ApplyEasing
            (Transformation|SetActorLocation _value_2 false false))
          (:OnComplete
            (Variables|Default|SetIsMoving false)
            (Collision|SetCollisionEnabled (Variables|Default|GetKillbox) "NoCollision")))))))

(fn ConstructionScript
  (Rendering|Material|SetMaterial (Variables|Default|GetS_Cover_Box) 0 (Variables|Default|GetMaterial_0)))