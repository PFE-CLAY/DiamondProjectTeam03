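; Level-exit door that unlocks once enough generators are activated and, optionally, an allied character has arrived.
; Generator activations and ally overlaps with the box collider re-run TryUnlockDoor, updating interactability and shield visibility while always disabling shield collision.
; Interacting fires the finish-level dispatcher and tweens the door mesh's roll open.
; On completion it activates NWin, then after a short delay shows the victory widget and disables player input.
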(event OnComponentBeginOverlap(BoxCollider)
  (params (OverlappedComponent :type Primitive%20Component%20Object%20Reference) (OtherActor :type Actor%20Object%20Reference) (OtherComp :type Primitive%20Component%20Object%20Reference) (OtherBodyIndex :type Integer) (bFromSweep :type Boolean) (SweepResult :type Hit%20Result%20Structure%20%28by%20ref%29))
  (bind _asbp_proto_allied (Utilities|Casting|CastToBP_ProtoAllied OtherActor))
  (Default|CompletedTask _asbp_proto_allied)
  (Variables|Default|SetHasAllyArrived true)
  (bind _isunlocked (CallFunction|TryUnlockDoor))
  (bind _output_get (Variables|Default|SetCanBeOpened _isunlocked))
  (bind _output_get_2 (Variables|Default|SetCanBeInteractedWith _output_get))
  (Development|SetHiddeninGame (Variables|Default|GetDoorShield) _output_get_2 false)
  (Collision|SetCollisionEnabled (Variables|Default|GetDoorShield) "NoCollision"))

(event Custom|GeneratorActivated
  (Math|Integer|IncrementInt (Variables|Default|GetActivatedGenerators)
    (:%20%20
      (bind _isunlocked (CallFunction|TryUnlockDoor))
      (bind _output_get (Variables|Default|SetCanBeOpened _isunlocked))
      (bind _output_get_2 (Variables|Default|SetCanBeInteractedWith _output_get))
      (Development|SetHiddeninGame (Variables|Default|GetDoorShield) _output_get_2 false)
      (Collision|SetCollisionEnabled (Variables|Default|GetDoorShield) "NoCollision"))))

(event EventOnInteract
  (params (InteractingPlayer :type Character%20Object%20Reference))
  (bind _doormesh (Variables|Default|GetDoorMesh))
  (bind _returnvalue (Transformation|GetWorldRotation _doormesh))
  (if (Variables|Default|GetCanBeInteractedWith)
    (Variables|Default|SetCanBeInteractedWith false)
    (if (Variables|Default|GetCanBeOpened)
      (Variables|Default|SetCanBeInteractedWith false)
      (Default|CallFinishLevelDispatcher)
      (bind _value (|TweenRotator (Math|Rotator|MakeRotator (.roll _returnvalue) (.pitch _returnvalue) (.yaw _returnvalue)) (Math|Rotator|MakeRotator 9e+01 (.pitch _returnvalue) (.yaw _returnvalue)) 1.0 "InOutQuad")
        (:ApplyEasing
          (Transformation|SetWorldRotation (Variables|Default|GetDoorMesh) _value false false))
        (:OnComplete
          (Components|Activation|Activate (Variables|Default|GetN_Win) false)
          (Utilities|FlowControl|Delay 0.5)
          (bind _returnvalue_2 (UserInterface|CreateWidget "/Game/Project/UI/Menus/UW_Victory.UW_Victory_C" (Game|GetPlayerController 0)))
          (UserInterface|Viewport|AddtoViewport _returnvalue_2 0)
          (Input|DisableInput (Game|GetPlayerCharacter 0) (Game|GetPlayerController 0)))))))

(fn ConstructionScript)

(fn TryUnlockDoor
  (bind _activatedgenerators (Variables|Default|GetActivatedGenerators))
  (bind _requirednumberofgenerators (Variables|Default|GetRequiredNumberOfGenerators))
  (bind _returnvalue (>= _activatedgenerators _requirednumberofgenerators))
  (if (Variables|Default|GetNeedsAnAlly)
    (return (and (Variables|Default|GetHasAllyArrived) _returnvalue))
    (else
      (return _returnvalue))))