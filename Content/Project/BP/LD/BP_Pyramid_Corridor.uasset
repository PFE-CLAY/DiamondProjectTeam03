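; Pyramid corridor level-design Blueprint that animates the roof (Toit) opening and the walls moving, shortly after BeginPlay.
; After a delay, a timeline slides the roof parent along Y, then destroys it and its planes before a second timeline moves the wall parent along Z.
; Timeline values are added to the current relative location each update, so movement accumulates.
; An unconnected draft for moving pieces one by one remains, with debug prints.
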(event EventBeginPlay
  (bind _toit_mother (Variables|Default|GetToit_Mother))
  (bind _wall_mother (Variables|Default|GetWall_Mother))
  (Utilities|FlowControl|Delay 5.0)
  (bind _newtrack_0 (Timeline|Toit_Movement Play)
    (:Update
      (Transformation|SetRelativeLocation _toit_mother (+ (Variables|/Script/Engine.SceneComponent|GetRelativeLocation _toit_mother) (Math|Vector|MakeVector 0.0 _newtrack_0 0.0)) false false))
    (:Finished
      (Components|DestroyComponent (Variables|Default|GetToit_Mother))
      (bind _newtrack_0_2 (Timeline|Wall_Movement Play)
        (:Update
          (Transformation|SetRelativeLocation _wall_mother (+ (Variables|/Script/Engine.SceneComponent|GetRelativeLocation _wall_mother) (Math|Vector|MakeVector 0.0 0.0 _newtrack_0_2)) false false))))))

(fn ConstructionScript)