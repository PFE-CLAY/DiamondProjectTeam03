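; A shielded door Blueprint that opens when its health component reports a change, such as from being shot.
; A timeline slides the door mesh down, holds it for DoorOpenDuration, then reverses to close it.
; A dynamic material on the frame toggles an Active parameter, showing the shield off while open and back on once closed.
; An IsDoorOpen flag ignores further hits until the door finishes closing.
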(event OnHealthChangedEvent(AC_Health)
  (params (CurrentHealth :type Integer) (DamageDealer :type Actor%20Object%20Reference))
  (if (not (Variables|Default|GetIsDoorOpen))
    (Variables|Default|SetIsDoorOpen true)
    (CallFunction|OpenClose true)
    (Rendering|Material|SetScalarParameterValue (Variables|Default|GetMaterialInstance) "Active" 0.0 :!class /Script/Engine.MaterialInstanceDynamic)))

(event Custom|OpenClose
  (params (ShouldOpen :type Boolean))
  (bind _sm_door (Variables|Default|GetSM_Door))
  (bind _relativelocation (Variables|/Script/Engine.SceneComponent|GetRelativeLocation _sm_door))
  (if ShouldOpen
    (bind _door_movement (Timeline|TimelineOpenClose Play)
      (:Update
        (Transformation|SetRelativeLocation _sm_door (Math|Vector|MakeVector (.x _relativelocation) (.y _relativelocation) (* _door_movement -1.0)) false false))
      (:Finished
        (if ShouldOpen
          (Utilities|FlowControl|Delay (Variables|Default|GetDoorOpenDuration))
          (CallFunction|OpenClose false)
          (else
            (Variables|Default|SetIsDoorOpen false)
            (Rendering|Material|SetScalarParameterValue (Variables|Default|GetMaterialInstance) "Active" 1.0 :!class /Script/Engine.MaterialInstanceDynamic)))))
    (else
      (Timeline|TimelineOpenClose Reverse))))

(event EventBeginPlay
  (bind _returnvalue (Rendering|Material|CreateDynamicMaterialInstance "/Game/Project/Materials/M_DoorWithShield.M_DoorWithShield" "None" "None" :!class /Script/Engine.KismetMaterialLibrary))
  (bind _output_get (Variables|Default|SetMaterialInstance _returnvalue))
  (Rendering|Material|SetMaterial (Variables|Default|GetSM_DoorFrame) 0 _output_get)
  (Rendering|Material|SetScalarParameterValue (Variables|Default|GetMaterialInstance) "Active" 1.0 :!class /Script/Engine.MaterialInstanceDynamic))

(fn ConstructionScript)