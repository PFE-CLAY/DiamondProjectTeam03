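; BP_Pyramid is a level design actor for a pyramid that can be opened during play or at start through the StartOpen flag.
; OPEN plays the OpenAnimation1 sequence and sets the OPEN flag.
; Sequencer events add feedback: ShakeBlock plays a world camera shake, while VFX&ShakeEnd activates four smoke effects and plays an ending shake, both centered on the actor.
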(event Custom|OPEN!
  (Class|ActorSequenceComponent|PlaySequence (Variables|Default|GetOpenAnimation1))
  (Variables|Default|SetOPEN? true))

(event EventBeginPlay
  (if (Variables|Default|GetStartOpen?)
    (CallFunction|OPEN!)))

(event Custom|ShakeBlock
  (Camera|PlayWorldCameraShake "/Game/Project/BP/CameraShake/BP_PyramidCamShakeBlock.BP_PyramidCamShakeBlock_C" (Transformation|GetActorLocation) 3e+03 2e+05))

(event Custom|VFX&ShakeEnd
  (Components|Activation|Activate (Variables|Default|GetSmoke1) false)
  (Components|Activation|Activate (Variables|Default|GetSmoke2) false)
  (Components|Activation|Activate (Variables|Default|GetSmoke3) false)
  (Components|Activation|Activate (Variables|Default|GetSmoke4) false)
  (Camera|PlayWorldCameraShake "/Game/Project/BP/CameraShake/BP_PyramidCamShakeEnd.BP_PyramidCamShakeEnd_C" (Transformation|GetActorLocation) 3e+03 2e+05))

(fn ConstructionScript)