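; Sun follower actor whose particle effects point along the sun direction, with active and inactive looks that use jump pad particle materials.
; Tick periodically re-aims both VFX components at the actor's location.
; Activate and Deactivate events restyle the SunDeactive system through Niagara user parameters rather than switching to SunActive.
; Player overlap with a collision box tweens spawn rate up, higher when activated, and exit tweens it to zero, stopping any running tween.
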(event OnComponentBeginOverlap(ActivatingCollisionBox)
  (params (OverlappedComponent :type Primitive%20Component%20Object%20Reference) (OtherActor :type Actor%20Object%20Reference) (OtherComp :type Primitive%20Component%20Object%20Reference) (OtherBodyIndex :type Integer) (bFromSweep :type Boolean) (SweepResult :type Hit%20Result%20Structure%20%28by%20ref%29))
  (Utilities|Casting|CastToDiamondProjectCharacter OtherActor)
  (bind _async_task (Variables|Default|GetAsync%20Task)
    (:then
      (Class|FCTweenBPAction|Stop _async_task))
    (:else
      _))
  (if (Variables|Default|GetisActivated)
    (Variables|Default|SetdesiredSpawnRate 2e+02)
    (else
      (Variables|Default|SetdesiredSpawnRate 35.0)))
  (bind (_asynctaskproxy _value) (|TweenFloat (Variables|Default|GetcurrentSpawnRate) (Variables|Default|GetdesiredSpawnRate) 1.0 "InOutQuad")
    (:then
      (Variables|Default|SetAsync%20Task _asynctaskproxy))
    (:ApplyEasing
      (Niagara|SetNiagaraVariable(Float) (Variables|Default|GetSunDeactive) "User.SpawnRate" _value))
    (:OnComplete
      (Development|PrintString (Utilities|String|Append (Utilities|GetObjectName self) " : Completed")))))

(event OnComponentEndOverlap(ActivatingCollisionBox)
  (params (OverlappedComponent :type Primitive%20Component%20Object%20Reference) (OtherActor :type Actor%20Object%20Reference) (OtherComp :type Primitive%20Component%20Object%20Reference) (OtherBodyIndex :type Integer))
  (Utilities|Casting|CastToDiamondProjectCharacter OtherActor)
  (bind _async_task (Variables|Default|GetAsync%20Task)
    (:then
      (Class|FCTweenBPAction|Stop _async_task))
    (:else
      _))
  (bind (_asynctaskproxy _value) (|TweenFloat (Variables|Default|GetcurrentSpawnRate) 0.0 1.0 "InOutQuad")
    (:then
      (Variables|Default|SetAsync%20Task _asynctaskproxy))
    (:ApplyEasing
      (Niagara|SetNiagaraVariable(Float) (Variables|Default|GetSunDeactive) "User.SpawnRate" _value))))

(event Custom|ActivateVFX
  (bind _sundeactive (Variables|Default|GetSunDeactive))
  (Niagara|SetNiagaraVariable(Float) _sundeactive "User.VelocityScale" 1.0)
  (Niagara|SetNiagaraVariable(Float) _sundeactive "User.WindSpeedScale" 0.0)
  (Niagara|SetNiagaraVariable(Float) _sundeactive "User.AerodynamicDrag" 0.0)
  (Class|NiagaraComponent|SetVariableMaterial _sundeactive "User.Material" "/Game/Project/Materials/M_JumpPadActiveParticle.M_JumpPadActiveParticle")
  (Niagara|SetNiagaraVariable(Float) _sundeactive "User.SystemConeAngle" 5.0)
  (Niagara|SetNiagaraVariable(Float) _sundeactive "User.ConeLength" 8e+02)
  (Niagara|SetNiagaraVariable(Float) _sundeactive "User.LifetimeMin" 1.0)
  (Niagara|SetNiagaraVariable(Float) _sundeactive "User.LifetimeMax" 2.0)
  (Variables|Default|SetisActivated true))

(event Custom|DeactivateVFX
  (bind _sundeactive (Variables|Default|GetSunDeactive))
  (Components|Activation|Deactivate (Variables|Default|GetSunActive))
  (Niagara|SetNiagaraVariable(Float) _sundeactive "User.VelocityScale" 0.0)
  (Niagara|SetNiagaraVariable(Float) _sundeactive "User.WindSpeedScale" 1.0)
  (Niagara|SetNiagaraVariable(Float) _sundeactive "User.AerodynamicDrag" 1.0)
  (Class|NiagaraComponent|SetVariableMaterial _sundeactive "User.Material" "/Game/Project/Materials/M_JumpPadInactiveParticle.M_JumpPadInactiveParticle")
  (Niagara|SetNiagaraVariable(Float) _sundeactive "User.SystemConeAngle" 1e+01)
  (Niagara|SetNiagaraVariable(Float) _sundeactive "User.ConeLength" 8e+02)
  (Niagara|SetNiagaraVariable(Float) _sundeactive "User.LifetimeMin" 1.0)
  (Niagara|SetNiagaraVariable(Float) _sundeactive "User.LifetimeMax" 2.0)
  (Components|Activation|Activate _sundeactive true)
  (Variables|Default|SetisActivated false))

(event EventBeginPlay
  (Variables|Default|GetSunActor
    (:then)
    (:else
      (bind _returnvalue (Actor|GetActorOfClass "/Game/Project/BP/LD/BP_Sun.BP_Sun_C"))
      (Variables|Default|SetSunActor _returnvalue)
      (CallFunction|DeactivateVFX))))

(event EventTick
  (params (DeltaSeconds :type Float%20%28single-precision%29))
  ;[1 1 1] Tick : 0.5sec
  (Utilities|FlowControl|Sequence
    (:then_0
      (Transformation|SetWorldTransform (Variables|Default|GetSunActive) (Math|Transform|MakeTransform (Transformation|GetActorLocation) (Math|Rotator|MakeRotfromZ (Class|SunFollower|GetSunDirection)) "1.000000,1.000000,1.000000") false false))))

(fn ConstructionScript)