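; Conveyor belt actor that pushes Characters standing on it along the direction of its Arrow component while switched on.
; Box overlap events maintain the list of riding Characters and a stepped-on flag, and the Activate event sets the active state.
; Each Tick offsets every listed actor by the arrow's forward vector times Speed, without sweep or delta-time scaling.
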(event OnComponentBeginOverlap(Box)
  (params (OverlappedComponent :type Primitive%20Component%20Object%20Reference) (OtherActor :type Actor%20Object%20Reference) (OtherComp :type Primitive%20Component%20Object%20Reference) (OtherBodyIndex :type Integer) (bFromSweep :type Boolean) (SweepResult :type Hit%20Result%20Structure%20%28by%20ref%29))
  (Utilities|Casting|CastToCharacter OtherActor)
  (if (not (Utilities|Array|ContainsItem (Variables|Default|GetActors) OtherActor))
    (Utilities|Array|Add (Variables|Default|GetActors) OtherActor)
    (Variables|Default|SetIsSteppedOn true)))

(event OnComponentEndOverlap(Box)
  (params (OverlappedComponent :type Primitive%20Component%20Object%20Reference) (OtherActor :type Actor%20Object%20Reference) (OtherComp :type Primitive%20Component%20Object%20Reference) (OtherBodyIndex :type Integer))
  (bind _actors (Variables|Default|GetActors))
  (if (and (Utilities|Array|ContainsItem (Variables|Default|GetActors) OtherActor) (Variables|Default|GetIsSteppedOn))
    (Utilities|Array|RemoveItem _actors OtherActor)
    (if (== (Utilities|Array|Length _actors) 0)
      (Variables|Default|SetIsSteppedOn false))))

(event Custom|Activate
  (params (SwitchOn :type Boolean))
  (Variables|Default|SetisActive SwitchOn))

(event EventTick
  (params (DeltaSeconds :type Float%20%28single-precision%29))
  (if (Variables|Default|GetisActive)
    (if (Variables|Default|GetIsSteppedOn)
      (for _array_element (Variables|Default|GetActors)
        (Transformation|SetActorLocation _array_element (+ (Transformation|GetActorLocation _array_element) (* (Math|Vector|GetForwardVector (Variables|Default|GetArrow)) (Variables|Default|GetSpeed))) false false)))))

(fn ConstructionScript)