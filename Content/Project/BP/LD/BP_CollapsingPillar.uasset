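; Destructible pillar that collapses when its health runs out, activates "pillar" and "sunlight" preplan steps, and damages what it falls on.
; An actor sequence starts the fall, then a sequencer event hands the middle mesh to physics with extra downward force.
; After a delay, overlaps deal damage, with pawns needing sufficient velocity directed at them.
; Slowing below that threshold spawns smoke and ends the collapse; IsPillarMoving actually returns true when slow.
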(event OnComponentBeginOverlap(CollisionFallingPillar)
  (params (OverlappedComponent :type Primitive%20Component%20Object%20Reference) (OtherActor :type Actor%20Object%20Reference) (OtherComp :type Primitive%20Component%20Object%20Reference) (OtherBodyIndex :type Integer) (bFromSweep :type Boolean) (SweepResult :type Hit%20Result%20Structure%20%28by%20ref%29))
  (bind _returnvalue (Actor|GetComponentbyClass OtherActor "/Script/DiamondProject.AC_Health"))
  (if (and (Variables|Default|GetbIsPhysicsActivated) (Variables|Default|GetbCanEndCollapse))
    (bind _aspawn (Utilities|Casting|CastToPawn OtherActor)
      (:then
        (bind _is_under (CallFunction|IsPillarFallingonPawn _aspawn))
        (if (and _is_under (> (Math|Vector|VectorLength (Transformation|GetComponentVelocity (Variables|Default|GetMiddleMesh))) (Variables|Default|GetThresholdVelocityOnCollapse)))
          (Utilities|IsValid _returnvalue :!label _label
            (:Is%20Valid
              (Class|ACHealth|DecreaseHealth _returnvalue (Variables|Default|GetDamage) self)
              (Utilities|Casting|CastToBP_FirstPersonCharacter OtherActor)
              (Collision|SetCollisionEnabled (Variables|Default|GetMiddleMesh) "NoCollision")))))
      (:CastFailed
        (goto _label)))))

(event OnDeathEvent(AC_Health)
  (params (DamageDealer :type Actor%20Object%20Reference) (OwnerActor :type Actor%20Object%20Reference))
  (if (not (Variables|Default|GetbIsCollapsed))
    (CallFunction|Collapse)))

(event Custom|Collapse
  (bind _returnvalue (Subsystems|GetLoopSubsystem))
  (Variables|Default|SetbIsCollapsing true)
  (Class|LoopSubsystem|ActivatePreplanStep _returnvalue "pillar" 1)
  (Class|LoopSubsystem|ActivatePreplanStep _returnvalue "sunlight" 1)
  ;[0.15 0.15 0.15 0.5] Play Sequence
  (bind _actorsequence (Variables|Default|GetActorSequence)
    (:then
      (Class|ActorSequenceComponent|PlaySequence _actorsequence))
    (:else
      _))
  (Class|AkGameplayStatics|PostEvent "/Game/WwiseAudio/Events/GPE_WU/Play_GPE_PillarDestroyed.Play_GPE_PillarDestroyed" self)
  (Utilities|Time|SetTimerbyEvent (delegate Custom|EnableEndCollapse) (Variables|Default|GetDelayTimerCanEndCollapse))
  (if (Variables|Default|GetSound?)
    (CallFunction|PlaySubtitles (Utilities|Struct|MakeDataTableRowHandle "/Game/Project/Subtitles/DataTables/DT_Arena/DT_DUB_ARENA_1_3_1.DT_DUB_ARENA_1_3_1" "None"))
    (Class|WwiseManagerSubsystem|PostEvent (Subsystems|GetWwiseManagerSubsystem) "/Game/WwiseAudio/Events/VOICES_WU/Play_DUB_ARENA_1_3_1.Play_DUB_ARENA_1_3_1" self)))

(event Custom|OnCollapseFinished
  (bind _middlemesh (Variables|Default|GetMiddleMesh))
  (Niagara|SpawnSystematLocation (Variables|Default|GetSmokeVFX) (Transformation|GetWorldLocation _middlemesh) (Transformation|GetWorldRotation _middlemesh))
  (Variables|Default|SetbIsCollapsing false))

(event Custom|EnableEndCollapse
  (Variables|Default|SetbCanEndCollapse true))

(event EventBeginPlay
  (bind _collisionfallingpillar (Variables|Default|GetCollisionFallingPillar)
    (:then
      (Collision|SetCollisionEnabled _collisionfallingpillar "NoCollision"))
    (:else)))

(event EventTick
  (params (DeltaSeconds :type Float%20%28single-precision%29))
  (if (and (Variables|Default|GetbIsCollapsing) (Variables|Default|GetbIsPhysicsActivated))
    (bind _returnvalue (CallFunction|IsPillarMoving))
    (if (and _returnvalue (Variables|Default|GetbCanEndCollapse))
      (Utilities|FlowControl|DoOnce false
        (:Completed
          (CallFunction|OnCollapseFinished)))
      (else
        ;[0.15 0.15 0.15 0.5] Prevent warning
        (if (Class|PrimitiveComponent|IsCollisionEnabled (Variables|Default|GetMiddleMesh))
          (Physics|AddForce (Variables|Default|GetMiddleMesh) "0.000000,0.000000,-9000000.000000" "None" false))))))

(event Custom|Owner_Event
  (params (Owner :type Actor%20Object%20Reference))
  (CallFunction|OnCollapseFinished)
  (Variables|Default|SetbIsCollapsed true))

(event Custom|ActivateCollision
  (params (Owner :type Actor%20Object%20Reference))
  (bind _collisionfallingpillar (Variables|Default|GetCollisionFallingPillar)
    (:then
      (Collision|SetCollisionEnabled _collisionfallingpillar "QueryOnly")
      (bind _actorsequence (Variables|Default|GetActorSequence)
        (:then
          (Class|ActorSequenceComponent|StopSequence _actorsequence)
          (Physics|SetSimulatePhysics (Variables|Default|GetMiddleMesh) true)
          (Variables|Default|SetbIsPhysicsActivated true))
        (:else)))
    (:else)))

(fn ConstructionScript)

(fn IsPillarFallingonPawn
  (params (OtherActor :type Pawn%20Object%20Reference))
  (bind _returnvalue (Transformation|GetActorLocation OtherActor))
  (bind _collisionfallingpillar (Variables|Default|GetCollisionFallingPillar))
  (bind (_outpointonbody _returnvalue_2) (Collision|GetClosestPointonCollision _collisionfallingpillar _returnvalue "None"))
  (bind _returnvalue_3 (Physics|GetPhysicsLinearVelocity (Variables|Default|GetMiddleMesh) "None"))
  (LocalVariables|SetVelocityDirection (Math|Vector|Normalize _returnvalue_3))
  (if (> _returnvalue_2 0.0)
    (Rendering|Debug|DrawDebugSphere _outpointonbody 1e+01 12 "(R=1.000000,G=0.000000,B=0.000000,A=1.000000)" 2.0)
    (LocalVariables|SetVectorDirectionToActor (Math|Vector|Normalize (- (Transformation|GetActorLocation OtherActor) _outpointonbody)))
    (return (> (Math|Vector|DotProduct (LocalVariables|GetVelocityDirection) (LocalVariables|GetVectorDirectionToActor)) 0.5))))

(fn IsPillarMoving
  (return (< (Math|Vector|VectorLength (Transformation|GetComponentVelocity (Variables|Default|GetMiddleMesh))) (Variables|Default|GetThresholdVelocityOnCollapse))))