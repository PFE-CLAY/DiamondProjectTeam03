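; BP_LightPyramid is a level-design light prop made of ten SLight pieces and a LightClassic light, configurable per instance.
; The Construction Script applies a backstage or exterior color to pieces and light; the pyramid color branch is disconnected.
; MoreLight and LessLight flags adjust piece visibility and attenuation radius.
; If SouldMove is set, BeginPlay staggers tweens that offset the pieces along Z by fractions of LightMovementValue, some chained on completion.
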(event Custom|Light_movementS
  (bind _s_light (Variables|Default|GetS_Light))
  (bind _relativelocation (Variables|/Script/Engine.SceneComponent|GetRelativeLocation _s_light))
  (bind (_x _y _z) (Math|Vector|BreakVector _relativelocation))
  (bind _value (|TweenVector _relativelocation (Math|Vector|MakeVector _x _y (+ _z (/ (Variables|Default|GetLight%20movement%20Value) 2.5))) (Variables|Default|GetDuration%20Secs) "InOutQuad" 0.0 0.0 0.0 -1 0.0 true)
    (:ApplyEasing
      (Transformation|SetRelativeLocation (Variables|Default|GetS_Light) _value false false))))

(event Custom|Light_Movement1
  (bind _s_light9 (Variables|Default|GetS_Light9))
  (bind _s_light1 (Variables|Default|GetS_Light1))
  (bind _relativelocation (Variables|/Script/Engine.SceneComponent|GetRelativeLocation _s_light9))
  (bind _relativelocation_2 (Variables|/Script/Engine.SceneComponent|GetRelativeLocation _s_light1))
  (bind (_x _y _z) (Math|Vector|BreakVector _relativelocation_2))
  (bind (_x_2 _y_2 _z_2) (Math|Vector|BreakVector _relativelocation))
  (bind _value (|TweenVector _relativelocation_2 (Math|Vector|MakeVector _x _y (+ _z (/ (Variables|Default|GetLight%20movement%20Value) 2.0))) (Variables|Default|GetDuration%20Secs) "InOutQuad" 0.0 0.0 0.0 -1 0.0 true)
    (:ApplyEasing
      (Transformation|SetRelativeLocation (Variables|Default|GetS_Light1) _value false false))
    (:OnComplete
      (bind _value_2 (|TweenVector _relativelocation (Math|Vector|MakeVector _x_2 _y_2 (+ _z_2 (/ (Variables|Default|GetLight%20movement%20Value) 1.5))) (Variables|Default|GetDuration%20Secs) "InOutQuad" 0.0 0.0 0.0 -1 0.0 true)
        (:ApplyEasing
          (Transformation|SetRelativeLocation (Variables|Default|GetS_Light9) _value_2 false false))))))

(event Custom|Light_Movement2
  (bind _s_light2 (Variables|Default|GetS_Light2))
  (bind _s_light7 (Variables|Default|GetS_Light7))
  (bind _relativelocation (Variables|/Script/Engine.SceneComponent|GetRelativeLocation _s_light2))
  (bind _relativelocation_2 (Variables|/Script/Engine.SceneComponent|GetRelativeLocation _s_light7))
  (bind (_x _y _z) (Math|Vector|BreakVector _relativelocation))
  (bind (_x_2 _y_2 _z_2) (Math|Vector|BreakVector _relativelocation_2))
  (bind _value (|TweenVector _relativelocation (Math|Vector|MakeVector _x _y (+ _z (Variables|Default|GetLight%20movement%20Value))) (Variables|Default|GetDuration%20Secs) "InOutQuad" 0.0 0.0 0.0 -1 0.0 true)
    (:ApplyEasing
      (Transformation|SetRelativeLocation (Variables|Default|GetS_Light2) _value false false))
    (:OnComplete
      (bind _value_2 (|TweenVector _relativelocation_2 (Math|Vector|MakeVector _x_2 _y_2 (+ _z_2 (/ (Variables|Default|GetLight%20movement%20Value) 1.5))) (Variables|Default|GetDuration%20Secs) "InOutQuad" 0.0 0.0 0.0 -1 0.0 true)
        (:ApplyEasing
          (Transformation|SetRelativeLocation (Variables|Default|GetS_Light7) _value_2 false false))))))

(event Custom|Light_Movement3
  (bind _s_light3 (Variables|Default|GetS_Light3))
  (bind _s_light8 (Variables|Default|GetS_Light8))
  (bind _relativelocation (Variables|/Script/Engine.SceneComponent|GetRelativeLocation _s_light8))
  (bind _relativelocation_2 (Variables|/Script/Engine.SceneComponent|GetRelativeLocation _s_light3))
  (bind (_x _y _z) (Math|Vector|BreakVector _relativelocation_2))
  (bind (_x_2 _y_2 _z_2) (Math|Vector|BreakVector _relativelocation))
  (bind _value (|TweenVector _relativelocation_2 (Math|Vector|MakeVector _x _y (+ _z (/ (Variables|Default|GetLight%20movement%20Value) 1.5))) (Variables|Default|GetDuration%20Secs) "InOutQuad" 0.0 0.0 0.0 -1 0.0 true)
    (:ApplyEasing
      (Transformation|SetRelativeLocation (Variables|Default|GetS_Light3) _value false false))
    (:OnComplete
      (bind _value_2 (|TweenVector _relativelocation (Math|Vector|MakeVector _x_2 _y_2 (+ _z_2 (/ (Variables|Default|GetLight%20movement%20Value) 1.5))) (Variables|Default|GetDuration%20Secs) "InOutQuad" 0.0 0.0 0.0 -1 0.0 true)
        (:ApplyEasing
          (Transformation|SetRelativeLocation (Variables|Default|GetS_Light8) _value_2 false false))))))

(event Custom|Light_Movement4
  (bind _s_light4 (Variables|Default|GetS_Light4))
  (bind _relativelocation (Variables|/Script/Engine.SceneComponent|GetRelativeLocation _s_light4))
  (bind (_x _y _z) (Math|Vector|BreakVector _relativelocation))
  (bind _value (|TweenVector _relativelocation (Math|Vector|MakeVector _x _y (+ _z (Variables|Default|GetLight%20movement%20Value))) (Variables|Default|GetDuration%20Secs) "InOutQuad" 0.0 0.0 0.0 -1 0.0 true)
    (:ApplyEasing
      (Transformation|SetRelativeLocation (Variables|Default|GetS_Light4) _value false false))))

(event Custom|Light_movement5
  (bind _s_light5 (Variables|Default|GetS_Light5))
  (bind _s_light6 (Variables|Default|GetS_Light6))
  (bind _relativelocation (Variables|/Script/Engine.SceneComponent|GetRelativeLocation _s_light6))
  (bind _relativelocation_2 (Variables|/Script/Engine.SceneComponent|GetRelativeLocation _s_light5))
  (bind (_x _y _z) (Math|Vector|BreakVector _relativelocation))
  (bind (_x_2 _y_2 _z_2) (Math|Vector|BreakVector _relativelocation_2))
  (bind _value (|TweenVector _relativelocation_2 (Math|Vector|MakeVector _x_2 _y_2 (+ _z_2 (/ (Variables|Default|GetLight%20movement%20Value) 1.5))) (Variables|Default|GetDuration%20Secs) "InOutQuad" 0.0 0.0 0.0 -1 0.0 true)
    (:ApplyEasing
      (Transformation|SetRelativeLocation (Variables|Default|GetS_Light5) _value false false))
    (:OnComplete
      (bind _value_2 (|TweenVector _relativelocation (Math|Vector|MakeVector _x _y (+ _z (/ (Variables|Default|GetLight%20movement%20Value) 1.5))) (Variables|Default|GetDuration%20Secs) "InOutQuad" 0.0 0.0 0.0 -1 0.0 true)
        (:ApplyEasing
          (Transformation|SetRelativeLocation (Variables|Default|GetS_Light6) _value_2 false false))))))

(event EventBeginPlay
  (if (Variables|Default|GetSouldMove)
    (CallFunction|LightMovement1)
    (Utilities|FlowControl|Delay 0.6)
    (CallFunction|LightMovement2)
    (Utilities|FlowControl|Delay 0.4)
    (CallFunction|LightMovement3)
    (Utilities|FlowControl|Delay 0.55)
    (CallFunction|LightMovement4)
    (Utilities|FlowControl|Delay 0.4)
    (CallFunction|LightMovement5)
    (Utilities|FlowControl|Delay 0.5)
    (CallFunction|LightMovementS)))

(fn ConstructionScript
  (bind _s_light (Variables|Default|GetS_Light))
  (if (Variables|Default|GetBackroom?)
    (bind _output_get (LocalVariables|SetColor (Variables|Default|GetColor_Backstage)))
    (Rendering|Material|SetVectorParameterValueonMaterials _s_light "Color" (Math|Conversions|ToVector(LinearColor) _output_get))
    (else
      (bind _output_get_2 (LocalVariables|SetColor (Variables|Default|GetColor%20Exterior)))
      (Rendering|Material|SetVectorParameterValueonMaterials _s_light "Color" (Math|Conversions|ToVector(LinearColor) _output_get_2))))
  (Rendering|Components|Light|SetLightColor (Variables|Default|GetLight%20Classic) (LocalVariables|GetColor) true)
  (if (Variables|Default|GetMoreLight?)
    (Rendering|SetVisibility (Variables|Default|GetS_Light8) true false)
    (Rendering|Lighting|SetAttenuationRadius (Variables|Default|GetLight%20Classic) (Variables|Default|GetRadius%20More))
    (elif (not (Variables|Default|GetLessLight?))
      (Rendering|Lighting|SetAttenuationRadius (Variables|Default|GetLight%20Classic) (Variables|Default|GetRadius%20Classic))
      (else
        (Rendering|SetVisibility (Variables|Default|GetS_Light2) false false)
        (Rendering|Lighting|SetAttenuationRadius (Variables|Default|GetLight%20Classic) (Variables|Default|GetRadius%20Less))))))