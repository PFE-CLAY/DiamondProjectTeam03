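; BP_NewPreplan is an actor that sets up the preplan phase of a level when its Init event is called.
; Init reuses an existing UW_NewPreplan widget or creates one for player 0, then tells the loop subsystem to initialize the preplan.
; It then calls PostInit on every displayed and to-collect collectible actor in the level.
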(event Custom|Event%20Init
  (bind _foundwidgets (Widget|GetAllWidgetsOfClass "/Game/Project/UI/Menus/UW_NewPreplan.UW_NewPreplan_C" false))
  (if (Utilities|Array|IsEmpty _foundwidgets)
    (bind _returnvalue (UserInterface|CreateWidget "/Game/Project/UI/Menus/UW_NewPreplan.UW_NewPreplan_C" (Game|GetPlayerController 0)))
    (Variables|Default|SetUINewPreplan _returnvalue)
    (else
      (Variables|Default|SetUINewPreplan (Utilities|Array|Get(acopy) _foundwidgets))))
  (Class|LoopSubsystem|InitializePreplan (Subsystems|GetLoopSubsystem))
  (bind _outactors (Actor|GetAllActorsOfClass "/Game/Project/BP/Collectible/BP_CollectibleDisplayed.BP_CollectibleDisplayed_C"))
  (for _array_element _outactors
    (Default|PostInit _array_element))
  (bind _outactors_2 (Actor|GetAllActorsOfClass "/Game/Project/BP/Collectible/BP_CollectibleToCollect.BP_CollectibleToCollect_C"))
  (for _array_element_2 _outactors_2
    (Default|PostInit _array_element_2)))

(event Collision|EventActorBeginOverlap
  (params (OtherActor :type Actor%20Object%20Reference)))

(event EventTick
  (params (DeltaSeconds :type Float%20%28single-precision%29)))

(fn ConstructionScript)