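; A destructible level pillar that loses health when its middle mesh is hit and collapses on death.
; Collapse plays an actor sequence with Wwise audio and optional subtitled voice line, and advances LoopSubsystem preplan steps.
; Sequencer events switch on a query-only damage volume during the fall, then disable it and spawn smoke at the end.
; Overlapped actors with health take damage; hitting the first-person character also disables the middle mesh's collision.
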(event OnComponentHit(MiddleMesh)
  (params (HitComponent :type Primitive%20Component%20Object%20Reference) (OtherActor :type Actor%20Object%20Reference) (OtherComp :type Primitive%20Component%20Object%20Reference) (NormalImpulse :type Vector :default "0, 0, 0") (Hit :type Hit%20Result%20Structure%20%28by%20ref%29))
  (bind _ac_health (Variables|Default|GetAC_Health))
  (if (Variables|/Script/DiamondProject.AC_Health|GetbIsDead _ac_health)
    (if (Variables|Default|GetbIsCollapsing)
      _)
    (else
      (Class|ACHealth|DecreaseOneHealth _ac_health)
      (Class|LoopSubsystem|ActivatePreplanStep (Subsystems|GetLoopSubsystem) "PillarDestroy" 1))))

(event OnDeathEvent(AC_Health)
  (params (DamageDealer :type Actor%20Object%20Reference) (OwnerActor :type Actor%20Object%20Reference))
  (if (not (Variables|Default|GetbIsCollapsed))
    (CallFunction|Collapse)))

(event OnComponentBeginOverlap(CollisionFallingPillar)
  (params (OverlappedComponent :type Primitive%20Component%20Object%20Reference) (OtherActor :type Actor%20Object%20Reference) (OtherComp :type Primitive%20Component%20Object%20Reference) (OtherBodyIndex :type Integer) (bFromSweep :type Boolean) (SweepResult :type Hit%20Result%20Structure%20%28by%20ref%29))
  (bind _returnvalue (Actor|GetComponentbyClass OtherActor "/Script/DiamondProject.AC_Health"))
  (Utilities|IsValid _returnvalue
    (:Is%20Valid
      (Class|ACHealth|DecreaseHealth _returnvalue (Variables|Default|GetDamage) self)
      (Utilities|Casting|CastToBP_FirstPersonCharacter OtherActor)
      (Collision|SetCollisionEnabled (Variables|Default|GetMiddleMesh) "NoCollision"))))

(event Custom|Collapse
  (bind _returnvalue (Subsystems|GetLoopSubsystem))
  (Variables|Default|SetbIsCollapsing true)
  (Class|LoopSubsystem|ActivatePreplanStep _returnvalue "pillar" 1)
  (Class|LoopSubsystem|ActivatePreplanStep _returnvalue "sunlight" 1)
  ;[0.15 0.15 0.15 0.5] Play Sequence
  (bind _actorsequence (Variables|Default|GetActorSequence)
    (:then
      (Class|ActorSequenceComponent|PlaySequence _actorsequence)
      (Class|AkGameplayStatics|PostEvent "/Game/WwiseAudio/Events/GPE_WU/Play_GPE_PillarDestroyed.Play_GPE_PillarDestroyed" self)
      (if (Variables|Default|GetSound?)
        (CallFunction|PlaySubtitles (Utilities|Struct|MakeDataTableRowHandle "/Game/Project/Subtitles/DataTables/DT_Arena/DT_DUB_ARENA_1_3_1.DT_DUB_ARENA_1_3_1" "None"))
        (Class|WwiseManagerSubsystem|PostEvent (Subsystems|GetWwiseManagerSubsystem) "/Game/WwiseAudio/Events/VOICES_WU/Play_DUB_ARENA_1_3_1.Play_DUB_ARENA_1_3_1" self)))
    (:else)))

(event Custom|OnCollapseFinished
  (Niagara|SpawnSystematLocation (Variables|Default|GetSmokeVFX) (Transformation|GetWorldLocation (Variables|Default|GetMiddleMesh)))
  (bind _collisionfallingpillar (Variables|Default|GetCollisionFallingPillar)
    (:then
      (Collision|SetCollisionEnabled _collisionfallingpillar "NoCollision")
      (Variables|Default|SetbIsCollapsing false))
    (:else)))

(event EventBeginPlay
  (bind _collisionfallingpillar (Variables|Default|GetCollisionFallingPillar)
    (:then
      (Collision|SetCollisionEnabled _collisionfallingpillar "NoCollision"))
    (:else)))

(event Custom|Owner_Event
  (params (Owner :type Actor%20Object%20Reference))
  (CallFunction|OnCollapseFinished)
  (Variables|Default|SetbIsCollapsed true))

(event Custom|ActivateCollision
  (params (Owner :type Actor%20Object%20Reference))
  (bind _collisionfallingpillar (Variables|Default|GetCollisionFallingPillar)
    (:then
      (Collision|SetCollisionEnabled _collisionfallingpillar "QueryOnly"))
    (:else)))

(fn ConstructionScript)