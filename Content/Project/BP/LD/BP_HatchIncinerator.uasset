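; Incinerator hatch Blueprint with two corpse-trap doors that slide apart on open and back together on close.
; It caches both door origins at BeginPlay, then a timeline offsets them oppositely along X, playing in reverse to close.
; Opening also activates a step of the "robot" preplan through the loop subsystem and calls the parent open logic.
; Wwise events play the opening and closing sounds.
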(event EventBeginPlay
  (Variables|Default|SetDoorROrigin (Variables|/Script/Engine.SceneComponent|GetRelativeLocation (Variables|Default|GetS_Corps_Trap_Right)))
  (Variables|Default|SetDoorLOrigin (Variables|/Script/Engine.SceneComponent|GetRelativeLocation (Variables|Default|GetS_Corps_Trap_Left))))

(event EventOnOpenHatch
  (bind _doorrorigin (Variables|Default|GetDoorROrigin))
  (bind _doorlorigin (Variables|Default|GetDoorLOrigin))
  (Class|LoopSubsystem|ActivatePreplanStep (Subsystems|GetLoopSubsystem) "robot" 1)
  (Class|AkGameplayStatics|PostEvent "/Game/WwiseAudio/Events/GPE_WU/Play_SFX_CorpseTrap_Opening.Play_SFX_CorpseTrap_Opening" self)
  (|CallParentFunction)
  (bind _value (Timeline|OpenDoors Play)
    (:Update
      (Transformation|SetRelativeLocation (Variables|Default|GetS_Corps_Trap_Right) (Math|Vector|MakeVector (+ (.x _doorrorigin) (* _value 2e+01)) (.y _doorrorigin) (.z _doorrorigin)) false false)
      (Transformation|SetRelativeLocation (Variables|Default|GetS_Corps_Trap_Left) (Math|Vector|MakeVector (- (.x _doorlorigin) (* _value 2e+01)) (.y _doorlorigin) (.z _doorlorigin)) false false))))

(event EventOnCloseHatch
  (bind _doorrorigin (Variables|Default|GetDoorROrigin))
  (bind _doorlorigin (Variables|Default|GetDoorLOrigin))
  (Class|AkGameplayStatics|PostEvent "/Game/WwiseAudio/Events/GPE_WU/Play_SFX_CorpseTrap_Closing.Play_SFX_CorpseTrap_Closing" self)
  (bind _value (Timeline|OpenDoors Reverse)
    (:Update
      (Transformation|SetRelativeLocation (Variables|Default|GetS_Corps_Trap_Right) (Math|Vector|MakeVector (+ (.x _doorrorigin) (* _value 2e+01)) (.y _doorrorigin) (.z _doorrorigin)) false false)
      (Transformation|SetRelativeLocation (Variables|Default|GetS_Corps_Trap_Left) (Math|Vector|MakeVector (- (.x _doorlorigin) (* _value 2e+01)) (.y _doorlorigin) (.z _doorlorigin)) false false))))

(fn ConstructionScript)