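; Pyramid target actor that opens the pyramid door when its health changes.
; On the health event it sets its active color and calls OpenDoorFromTarget on the BP_DoorPyramid found in the level.
; If Pyramid.OPEN is true it destroys itself; otherwise it activates the "can_open" preplan step through the loop subsystem, only once.
; Voice-line and FakeOpenPyramid logic remains in the graph but is disconnected.
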(event OnHealthChangedEvent(AC_Health)
  (params (CurrentHealth :type Integer) (DamageDealer :type Actor%20Object%20Reference))
  (CallFunction|SetActiveColor)
  (bind _returnvalue (Actor|GetActorOfClass "/Game/Project/BP/LD/BP_DoorPyramid.BP_DoorPyramid_C"))
  (Default|OpenDoorfromTarget _returnvalue)
  (if (Variables|/Game/Project/BP/LD/BP_Pyramid.BP_Pyramid_C|GetOPEN? (Variables|Default|GetPyramid))
    (Actor|DestroyActor)
    (else
      ;[1 1 1] Pyramid
      (Utilities|FlowControl|DoOnce false
        (:Completed
          (Class|LoopSubsystem|ActivatePreplanStep (Subsystems|GetLoopSubsystem) "can_open" 1))))))

(fn ConstructionScript
  (|CallParentFunction))