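; BP_Target_Platform is a target that moves linked platforms when its health changes.
; On BeginPlay it casts the referenced platforms to the BPI_MovingPlatform interface and caches them, stopping at the first failed cast.
; Each health change event from AC_Health sets the active color and calls ChangeTargetPosition on every cached platform.
; An older directional activation branch for a single prison platform remains in the graph but never runs.
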(event OnHealthChangedEvent(AC_Health)
  (params (CurrentHealth :type Integer) (DamageDealer :type Actor%20Object%20Reference))
  (CallFunction|SetActiveColor)
  (for _array_element (Variables|Default|GetMovingPlatforms)
    (Default|ChangeTargetPosition _array_element)))

(event EventBeginPlay
  (for _array_element (Variables|Default|GetPlatformsRef)
    (bind _asbpi_moving_platform (Utilities|Casting|CastToBPI_MovingPlatform _array_element))
    (Utilities|Array|Add (Variables|Default|GetMovingPlatforms) _asbpi_moving_platform)))

(fn ConstructionScript
  (|CallParentFunction))