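; A test interact button Blueprint for level design that spawns turret enemies when used.
; Its OnInteract event prints a debug message, then spawns three BP_TurretEnemy actors at the transforms of the Spawn1, Spawn2 and Spawn3 reference actors.
; The construction script only calls its parent.
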(event EventOnInteract
  (params (InteractingPlayer :type Character%20Object%20Reference))
  (Development|PrintText "Spawn!")
  (Game|SpawnActorfromClass "/Game/Project/BP/IA/Enemy/BP_TurretEnemy.BP_TurretEnemy_C" (Transformation|GetActorTransform (Variables|Default|GetSpawn1)) "Undefined" "MultiplyWithRoot" 0 0)
  (Game|SpawnActorfromClass "/Game/Project/BP/IA/Enemy/BP_TurretEnemy.BP_TurretEnemy_C" (Transformation|GetActorTransform (Variables|Default|GetSpawn2)) "Undefined" "MultiplyWithRoot" 0 0)
  (Game|SpawnActorfromClass "/Game/Project/BP/IA/Enemy/BP_TurretEnemy.BP_TurretEnemy_C" (Transformation|GetActorTransform (Variables|Default|GetSpawn3)) "Undefined" "MultiplyWithRoot" 0 0))

(fn ConstructionScript
  (|CallParentFunction))