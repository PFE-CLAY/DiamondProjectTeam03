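; Elevator actor that puts up four blocking box walls around itself for the duration of a ride.
; BeginPlay caches the first-person character, gathers the boxes into an array and turns their visibility and collision off.
; Activating the InterpToMovement component turns both on, then off again after a fixed nine-second delay.
; One FlipFlop drives both states, so wall state depends on call order; the Target destroy nodes are unconnected.
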(event OnComponentActivated(InterpToMovement)
  (params (Component :type Actor%20Component%20Object%20Reference) (bReset :type Boolean))
  ;[1 1 1] [Spotlight (Target) + Invisible Walls] destroy over elevator
  (CallFunction|Enable/DisableWalls)
  (Utilities|FlowControl|Delay 9.0)
  (CallFunction|Enable/DisableWalls))

(event Custom|Enable/Disable%20Walls
  (bind _invisarray (Variables|Default|GetInvisArray))
  (Utilities|FlowControl|FlipFlop
    (:A
      (Rendering|SetVisibility _invisarray false false)
      (Collision|SetCollisionEnabled _invisarray "NoCollision"))
    (:B
      (Rendering|SetVisibility _invisarray true false)
      (Collision|SetCollisionEnabled _invisarray "QueryAndPhysics"))))

(event EventBeginPlay
  (bind _asbp_first_person_character (Utilities|Casting|CastToBP_FirstPersonCharacter (Game|GetPlayerCharacter 0)))
  (Variables|Default|SetAs%20BP%20First%20Person%20Character _asbp_first_person_character)
  (Variables|Default|SetInvisArray (Utilities|Array|MakeArray (Variables|Default|GetBoxNorth) (Variables|Default|GetBoxEast) (Variables|Default|GetBoxWest) (Variables|Default|GetBoxSouth)))
  (CallFunction|Enable/DisableWalls))

(fn ConstructionScript)