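; Backstage door actor that opens automatically when the player walks up to it and closes when they leave.
; Begin and end overlap on a Box trigger, filtered to the first player character, each start a half-second float tween in opposite directions.
; The tween value drives the "Open" morph target on the door's skeletal mesh, so the motion comes from blend shapes.
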(event OnComponentBeginOverlap(Box)
  (params (OverlappedComponent :type Primitive%20Component%20Object%20Reference) (OtherActor :type Actor%20Object%20Reference) (OtherComp :type Primitive%20Component%20Object%20Reference) (OtherBodyIndex :type Integer) (bFromSweep :type Boolean) (SweepResult :type Hit%20Result%20Structure%20%28by%20ref%29))
  (if (== OtherActor (Game|GetPlayerCharacter 0))
    (bind _value (|TweenFloat 0.0 1.0 0.5 "InOutQuad")
      (:ApplyEasing
        (Components|SkeletalMesh|SetMorphTarget (Variables|Default|GetSK_DoorBackstage) "Open" _value true)))))

(event OnComponentEndOverlap(Box)
  (params (OverlappedComponent :type Primitive%20Component%20Object%20Reference) (OtherActor :type Actor%20Object%20Reference) (OtherComp :type Primitive%20Component%20Object%20Reference) (OtherBodyIndex :type Integer))
  (if (== OtherActor (Game|GetPlayerCharacter 0))
    (bind _value (|TweenFloat 1.0 0.0 0.5 "InOutQuad")
      (:ApplyEasing
        (Components|SkeletalMesh|SetMorphTarget (Variables|Default|GetSK_DoorBackstage) "Open" _value true)))))

(event EventBeginPlay)

(fn ConstructionScript)