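; BP_Sun is a sun actor that animates its directional light over a timed duration once the arena is entered.
; It binds to BP_NPCActivationZone's enter-arena dispatcher on BeginPlay, which triggers a linear rotator tween of the actor.
; A parallel float tween warms the light's temperature, widens its source angles and raises its intensity.
; The level-finish stop binding and material distortion update are disconnected and never run.
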(event Custom|StartTimerEvent
  (Variables|Default|SetShouldMoveSun true)
  (CallFunction|SunMove))

(event Custom|StopTimerEvent
  (Variables|Default|SetShouldMoveSun false))

(event Custom|SunMove
  (bind _directionallight (Variables|Default|GetDirectionalLight))
  ;[1 1 1] Rotation
  (if (Variables|Default|GetShouldMoveSun)
    (bind (_asynctaskproxy _value) (|TweenRotator (Transformation|GetActorRotation self) "-90.000000,0.000000,0.000000" (Variables|Default|GetSun%20Duration%20Secs) "Linear")
      (:then
        (Variables|Default|SetAsync%20Task%20-%20SUN _asynctaskproxy)
        (bind _value_2 (|TweenFloat 0.0 1.0 (Variables|Default|GetSun%20Duration%20Secs) "InOutQuad")
          (:ApplyEasing
            (Class|LightComponent|SetTemperature _directionallight (Math|Float|Lerp 4e+03 2e+03 _value_2))
            (Class|DirectionalLightComponent|SetLightSourceAngle _directionallight (Math|Float|Lerp 1.5 7.0 _value_2))
            (Class|DirectionalLightComponent|SetLightSourceSoftAngle _directionallight (Math|Float|Lerp 1.5 7.0 _value_2))
            (Rendering|Components|Light|SetIntensity _directionallight (Math|Float|Lerp 3.0 8.0 _value_2)))))
      (:ApplyEasing
        (Transformation|SetActorRotation _value)))))

(event EventBeginPlay
  (bind _returnvalue (Actor|GetActorOfClass "/Game/Project/BP/LD/BP_NPCActivationZone.BP_NPCActivationZone_C"))
  (Utilities|IsValid _returnvalue
    (:Is%20Valid
      (EventDispatchers|BindEventtoEnterArenaDispatcher _returnvalue (delegate Custom|StartTimerEvent)))))

(fn ConstructionScript)