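; Moving elevator platform that starts when the player first overlaps its trigger box, which is then destroyed.
; A recursive yoyo vector tween moves the root 800 units up and back with a pause, optionally playing a one-time arena welcome sound as it starts.
; Optional barrier meshes are hidden when disabled; when enabled, an InterpToMovement stop event removes invisible-wall collision and lowers the barrier.
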(event OnComponentBeginOverlap(TriggerBox)
  (params (OverlappedComponent :type Primitive%20Component%20Object%20Reference) (OtherActor :type Actor%20Object%20Reference) (OtherComp :type Primitive%20Component%20Object%20Reference) (OtherBodyIndex :type Integer) (bFromSweep :type Boolean) (SweepResult :type Hit%20Result%20Structure%20%28by%20ref%29))
  (if (== OtherActor (Variables|Default|GetAs%20BP%20First%20Person%20Character))
    (Components|DestroyComponent (Variables|Default|GetTriggerBox))
    (CallFunction|PlatformMove)))

(event OnInterptoStop(InterpToMovement)
  (params (ImpactResult :type Hit%20Result%20Structure%20%28by%20ref%29) (Time :type Float%20%28single-precision%29))
  (bind _sm_barriermother (Variables|Default|GetSM_BarrierMother))
  (if (Variables|Default|GetBarriers)
    ;[0.4198 0.4198 0.4198] Barrier Down
    (Collision|SetCollisionEnabled (Variables|Default|GetInvisibleWallArray) "NoCollision")
    (Utilities|FlowControl|Delay 0.5)
    (Components|MoveComponentTo _sm_barriermother (+ (Variables|/Script/Engine.SceneComponent|GetRelativeLocation _sm_barriermother) "0.000000,0.000000,-100.000000") (Variables|/Script/Engine.SceneComponent|GetRelativeRotation _sm_barriermother) false false 0.5 false)))

(event Custom|PlatformMove
  (bind _defaultsceneroot (Variables|Default|GetDefaultSceneRoot))
  (bind _relativelocation (Variables|/Script/Engine.SceneComponent|GetRelativeLocation _defaultsceneroot))
  (bind _value (|TweenVector _relativelocation (+ _relativelocation "0.000000,0.000000,800.000000") 3.0 "InOutQuad" 0.0 0.0 0.0 0 0.0 true 1.5)
    (:then
      (if (Variables|Default|GetShouldPlaySound)
        (Variables|Default|SetShouldPlaySound false)
        (Audio|SpawnSoundatLocation "/Game/Project/Sounds/Folleys/Welcome_to_the_Arena.Welcome_to_the_Arena" (Variables|Default|GetSoundLocation) "0, 0, 0" 1.0 1.0 0.0 "/Game/Project/Sounds/A_GlobalAttenuation.A_GlobalAttenuation" 0 false)))
    (:ApplyEasing
      (Transformation|SetRelativeLocation (Variables|Default|GetDefaultSceneRoot) _value false false))
    (:OnComplete
      (CallFunction|PlatformMove))))

(event EventBeginPlay
  (bind _asbp_first_person_character (Utilities|Casting|CastToBP_FirstPersonCharacter (Game|GetPlayerCharacter 0)))
  (Variables|Default|SetAs%20BP%20First%20Person%20Character _asbp_first_person_character)
  (if (not (Variables|Default|GetBarriers))
    (Rendering|SetVisibility (Variables|Default|GetSM_BarrierMother) false false)))

(fn ConstructionScript)