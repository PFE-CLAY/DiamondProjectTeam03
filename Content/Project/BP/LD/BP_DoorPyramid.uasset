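; BP_DoorPyramid is the pyramid door, which opens and closes as its MultiSunlightDetector gains or loses sunlight.
; Activation changes also advance loop preplan steps, play dubbed audio with subtitles, and toggle sun VFX and the entrance path index.
; Vector tweens slide the mesh vertically alongside Wwise sounds and portal toggling.
; Trigger boxes lock out opening behind the player and track allies inside, while path points get notified of openings, including button- or target-triggered ones.
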(event OnSunActivationChanged(MultiSunlightDetector)
  (params (IsActivated :type Boolean))
  (bind _returnvalue (Subsystems|GetLoopSubsystem))
  (bind _suuunn (Variables|Default|GetSUUUNN))
  (bind _pathpointenter (Variables|Default|GetPathPointEnter))
  (bind _childactor (Variables|/Script/Engine.ChildActorComponent|GetChildActor _suuunn))
  (bind _asbp_sun_follower (Utilities|Casting|CastToBP_SunFollower _childactor))
  (Class|LoopSubsystem|ActivatePreplanStep _returnvalue "pyramid_door" 1)
  (Class|LoopSubsystem|ActivatePreplanStep _returnvalue "trials" 1)
  (CallFunction|PlaySubtitles (Utilities|Struct|MakeDataTableRowHandle "/Game/Project/Subtitles/DataTables/DT_Arena/DT_DUB_ARENA_1_7_0.DT_DUB_ARENA_1_7_0" "None"))
  (Class|WwiseManagerSubsystem|PostEvent (Subsystems|GetWwiseManagerSubsystem) "/Game/WwiseAudio/Events/VOICES_WU/Play_DUB_ARENA_1_7_0.Play_DUB_ARENA_1_7_0" self)
  (bind _output_get (Variables|Default|SetSun%20is%20Activate%20? IsActivated))
  (if _output_get
    (Default|ActivateVFX _asbp_sun_follower)
    (Utilities|IsValid _pathpointenter
      (:Is%20Valid
        (Variables|/Script/DiamondProject.CustomNavigationPoint|SetWantedPathIndex _pathpointenter 1))
      (:Is%20Not%20Valid
        _))
    (else
      (Default|DeactivateVFX _asbp_sun_follower)
      (Utilities|IsValid _pathpointenter
        (:Is%20Valid
          (Variables|/Script/DiamondProject.CustomNavigationPoint|SetWantedPathIndex _pathpointenter 0))
        (:Is%20Not%20Valid
          _))))
  (CallFunction|DoorMove))

(event OnComponentBeginOverlap(BoxBefore)
  (params (OverlappedComponent :type Primitive%20Component%20Object%20Reference) (OtherActor :type Actor%20Object%20Reference) (OtherComp :type Primitive%20Component%20Object%20Reference) (OtherBodyIndex :type Integer) (bFromSweep :type Boolean) (SweepResult :type Hit%20Result%20Structure%20%28by%20ref%29))
  (if (== OtherActor (Game|GetPlayerCharacter 0))
    (Variables|Default|SetLockPlayer? false)))

(event OnComponentBeginOverlap(BoxAfter)
  (params (OverlappedComponent :type Primitive%20Component%20Object%20Reference) (OtherActor :type Actor%20Object%20Reference) (OtherComp :type Primitive%20Component%20Object%20Reference) (OtherBodyIndex :type Integer) (bFromSweep :type Boolean) (SweepResult :type Hit%20Result%20Structure%20%28by%20ref%29))
  (if (== OtherActor (Game|GetPlayerCharacter 0))
    (Variables|Default|SetLockPlayer? true)
    (if (Variables|Default|GetLockPlayer?)
      (Utilities|FlowControl|DoOnce false
        (:Completed
          (CallFunction|DoorClose))))))

(event OnComponentBeginOverlap(Box)
  (params (OverlappedComponent :type Primitive%20Component%20Object%20Reference) (OtherActor :type Actor%20Object%20Reference) (OtherComp :type Primitive%20Component%20Object%20Reference) (OtherBodyIndex :type Integer) (bFromSweep :type Boolean) (SweepResult :type Hit%20Result%20Structure%20%28by%20ref%29))
  (Utilities|Casting|CastToBP_AlliedSimple OtherActor)
  (Variables|Default|SetIsAlliedInPyramid (not (Variables|Default|GetIsAlliedInPyramid))))

(event Custom|DoorOpen
  (bind _sm_door_pyramid (Variables|Default|GetSM_Door_Pyramid))
  (bind _sm_door_pyramid_2 (Variables|Default|GetSM_Door_Pyramid))
  (bind _returnvalue (Transformation|GetWorldLocation _sm_door_pyramid))
  (Variables|Default|SetIsOpened true)
  (Class|WwiseManagerSubsystem|PostEvent (Subsystems|GetWwiseManagerSubsystem) "/Game/WwiseAudio/Events/SFX_WU/Play_SFX_Door_Pyramid_Open.Play_SFX_Door_Pyramid_Open" self)
  (Class|AkPortalComponent|EnablePortal (Variables|Default|GetAKP_Pyramid))
  (bind _value (|TweenVector _returnvalue (+ _returnvalue "0.000000,0.000000,-800.000000") (Variables|Default|GetDuration%20Secs) "InOutQuad")
    (:ApplyEasing
      (Transformation|SetWorldLocation (Variables|Default|GetSM_Door_Pyramid) _value false false))
    (:OnComplete
      (Rendering|SetVisibility _sm_door_pyramid_2 false false)
      (Collision|SetCollisionEnabled _sm_door_pyramid_2 "NoCollision")
      (if (not (Variables|Default|GetIsAlliedInPyramid))
        (Default|OnDoorOpened (Variables|Default|GetPathPointEnter))))))

(event Custom|DoorMove
  (if (Variables|Default|GetSun%20is%20Activate%20?)
    (if (not (Variables|Default|GetLockPlayer?))
      (CallFunction|DoorOpen))
    (else
      (CallFunction|DoorClose))))

(event Custom|OpenDoorFromTarget
  (CallFunction|DoorOpen)
  (Utilities|FlowControl|Delay (+ (Variables|Default|GetDuration%20Secs) 1.0))
  (Default|OnDoorOpened (Variables|Default|GetPathPointExit)))

(event Custom|DoorClose
  (bind _sm_door_pyramid (Variables|Default|GetSM_Door_Pyramid))
  (bind _sm_door_pyramid_2 (Variables|Default|GetSM_Door_Pyramid))
  (bind _returnvalue (Transformation|GetWorldLocation _sm_door_pyramid))
  (Class|WwiseManagerSubsystem|PostEvent (Subsystems|GetWwiseManagerSubsystem) "/Game/WwiseAudio/Events/SFX_WU/Play_SFX_Door_Pyramid_Close.Play_SFX_Door_Pyramid_Close" self)
  (Rendering|SetVisibility _sm_door_pyramid_2 true false)
  (Collision|SetCollisionEnabled _sm_door_pyramid_2 "QueryAndPhysics")
  (bind _value (|TweenVector _returnvalue (+ _returnvalue "0.000000,0.000000,800.000000") (Variables|Default|GetDuration%20Secs) "InOutQuad")
    (:ApplyEasing
      (Transformation|SetWorldLocation (Variables|Default|GetSM_Door_Pyramid) _value false false)
      (Utilities|FlowControl|Delay 2.2)
      (Class|AkPortalComponent|DisablePortal (Variables|Default|GetAKP_Pyramid)))
    (:OnComplete
      (Variables|Default|SetIsOpened false))))

(event Custom|OpenFromButton
  (CallFunction|DoorOpen)
  (Utilities|FlowControl|Delay (Variables|Default|GetDuration%20Secs))
  (Default|OnDoorOpened (Variables|Default|GetPathPointExit)))

(fn ConstructionScript)