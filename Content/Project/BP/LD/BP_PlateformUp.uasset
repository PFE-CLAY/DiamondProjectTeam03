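; Moving platform actor for level design that travels to an offset from its starting position, waits, then returns.
; Events pick fixed up, left, right or tall-lift offsets, or a variable offset, relative to the location saved at BeginPlay.
; Async vector tweens drive the actor's location, and each new activation stops the stored tween first.
; The tall lift runs its own fixed-duration tween but shares the delayed return.
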(event Custom|ActivateUp
  (CallFunction|StopCurrentTask)
  (Variables|Default|SetTargetPosition (+ (Variables|Default|GetBasePosition) "0.000000,0.000000,400.000000"))
  (CallFunction|Launch))

(event Custom|ActivateBigUp
  (CallFunction|StopCurrentTask)
  (bind _output_get (Variables|Default|SetTargetPosition (+ (Variables|Default|GetBasePosition) "0.000000,0.000000,2400.000000")))
  (bind (_asynctaskproxy _value) (|TweenVector (Transformation|GetActorLocation) _output_get 5.0 "InOutQuad")
    (:then
      (Variables|Default|SetCurrentTask _asynctaskproxy))
    (:ApplyEasing
      (Transformation|SetActorLocation _value false false))
    (:OnComplete
      (Utilities|FlowControl|Delay (Variables|Default|GetDelayStayAtTargetPosition))
      (bind (_asynctaskproxy_2 _value_2) (|TweenVector (Transformation|GetActorLocation) (Variables|Default|GetBasePosition) (Variables|Default|GetDurationMovementForth) "InOutQuad")
        (:then
          (Variables|Default|SetCurrentTask _asynctaskproxy_2))
        (:ApplyEasing
          (Transformation|SetActorLocation _value_2 false false))))))

(event Custom|ActivateRight
  (CallFunction|StopCurrentTask)
  (Variables|Default|SetTargetPosition (+ (Variables|Default|GetBasePosition) "0.000000,-400.000000,0.000000"))
  (CallFunction|Launch))

(event Custom|Launch
  (bind (_asynctaskproxy _value) (|TweenVector (Transformation|GetActorLocation) (Variables|Default|GetTargetPosition) (Variables|Default|GetDurationMovementBack) "InOutQuad")
    (:then
      (Variables|Default|SetCurrentTask _asynctaskproxy))
    (:ApplyEasing
      (Transformation|SetActorLocation _value false false))
    (:OnComplete
      (Utilities|FlowControl|Delay (Variables|Default|GetDelayStayAtTargetPosition))
      (bind (_asynctaskproxy_2 _value_2) (|TweenVector (Transformation|GetActorLocation) (Variables|Default|GetBasePosition) (Variables|Default|GetDurationMovementForth) "InOutQuad")
        (:then
          (Variables|Default|SetCurrentTask _asynctaskproxy_2))
        (:ApplyEasing
          (Transformation|SetActorLocation _value_2 false false))))))

(event Custom|ActivateLeft
  (CallFunction|StopCurrentTask)
  (Variables|Default|SetTargetPosition (+ (Variables|Default|GetBasePosition) "0.000000,400.000000,0.000000"))
  (CallFunction|Launch))

(event EventBeginPlay
  (Variables|Default|SetBasePosition (Transformation|GetActorLocation)))

(event EventChangeTargetPosition
  (CallFunction|StopCurrentTask)
  (Variables|Default|SetTargetPosition (+ (Variables|Default|GetBasePosition) (Variables|Default|GetOffsetMovement)))
  (CallFunction|Launch))

(fn ConstructionScript)

(fn StopCurrentTask
  (bind _currenttask (Variables|Default|GetCurrentTask)
    (:then
      (Class|FCTweenBPAction|Stop _currenttask))
    (:else)))