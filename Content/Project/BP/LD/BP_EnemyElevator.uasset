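; Elevator tied to a child turret enemy, rising when the player enters its range box and lowering after a delay once they leave.
; Killing the turret activates the "elevator" preplan step and unlocks the child target, which toggles the elevator when shot.
; Moves play a timeline shake and sand FX, then an eased tween with rumble offset, adding camera shakes if the player is aboard.
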(event OnComponentBeginOverlap(BoxTurret)
  (params (OverlappedComponent :type Primitive%20Component%20Object%20Reference) (OtherActor :type Actor%20Object%20Reference) (OtherComp :type Primitive%20Component%20Object%20Reference) (OtherBodyIndex :type Integer) (bFromSweep :type Boolean) (SweepResult :type Hit%20Result%20Structure%20%28by%20ref%29))
  (Utilities|Casting|CastToBP_FirstPersonCharacter OtherActor)
  (if (not (Variables|Entities|GetPlayerInRange))
    (Variables|Entities|SetPlayerInRange true)
    (if (and (Variables|Movement|GetCanGoUp) (not (Variables|Entities|GetIsEnemyDead)))
      (CallFunction|StopOngoingTranslation)
      (if (Utilities|Time|IsValidTimerHandle (Variables|Movement|GetElevatorGoingDownTimerHandle))
        (Utilities|Time|ClearandInvalidateTimerbyHandle (Variables|Movement|GetElevatorGoingDownTimerHandle)))
      (Variables|Movement|SetCanGoUp false)
      (CallFunction|MoveElevator (Variables|Movement|GetTopLocation)))))

(event OnComponentEndOverlap(BoxTurret)
  (params (OverlappedComponent :type Primitive%20Component%20Object%20Reference) (OtherActor :type Actor%20Object%20Reference) (OtherComp :type Primitive%20Component%20Object%20Reference) (OtherBodyIndex :type Integer))
  (Utilities|Casting|CastToBP_FirstPersonCharacter OtherActor)
  (if (Variables|Entities|GetPlayerInRange)
    (Variables|Entities|SetPlayerInRange false)
    (CallFunction|StopShake)
    (bind _returnvalue (Utilities|Time|SetTimerbyEvent (delegate Custom|ElevatorGoesDown) (Variables|Entities|GetNoAlliesInRangeElevatorTimer)))
    (Variables|Movement|SetElevatorGoingDownTimerHandle _returnvalue)))

(event OnComponentBeginOverlap(ElevatorCollision)
  (params (OverlappedComponent :type Primitive%20Component%20Object%20Reference) (OtherActor :type Actor%20Object%20Reference) (OtherComp :type Primitive%20Component%20Object%20Reference) (OtherBodyIndex :type Integer) (bFromSweep :type Boolean) (SweepResult :type Hit%20Result%20Structure%20%28by%20ref%29))
  (Utilities|Casting|CastToBP_FirstPersonCharacter OtherActor)
  (Variables|Shake|SetIsPlayerInElevator true))

(event OnComponentEndOverlap(ElevatorCollision)
  (params (OverlappedComponent :type Primitive%20Component%20Object%20Reference) (OtherActor :type Actor%20Object%20Reference) (OtherComp :type Primitive%20Component%20Object%20Reference) (OtherBodyIndex :type Integer))
  (Utilities|Casting|CastToBP_FirstPersonCharacter OtherActor)
  (Variables|Shake|SetIsPlayerInElevator false))

(event Custom|ElevatorEnemyDeath
  (params (DamageDealer :type Actor%20Object%20Reference) (OwnerActor :type Actor%20Object%20Reference))
  (Class|LoopSubsystem|ActivatePreplanStep (Subsystems|GetLoopSubsystem) "elevator")
  (Variables|ActivationButton|SetIsPressable true)
  (Rendering|Material|SetScalarParameterValueonMaterials (Variables|/Game/Project/BP/LD/BP_Target.BP_Target_C|GetSM_GearAngle (Variables|Entities|GetTarget%20Enemy%20Elevator)) "Statue" 0.0)
  (Variables|Entities|SetIsEnemyDead true))

(event Custom|ElevatorGoesDown
  (if (Math|Boolean|ANDBoolean (not (Variables|Entities|GetPlayerInRange)) (not (Variables|Entities|GetIsEnemyDead)) (not (Variables|Movement|GetCanGoUp)) (not (Variables|ActivationButton|GetIsButtonPressed)))
    (CallFunction|StopOngoingTranslation)
    (Variables|Movement|SetCanGoUp true)
    (CallFunction|MoveElevator (Variables|Movement|GetBottomLocation))))

(event Custom|OnTargetShot
  (params (CurrentHealth :type Integer) (DamageDealer :type Actor%20Object%20Reference))
  (CallFunction|ButtonPress))

(event Custom|ButtonPress
  (Variables|ActivationButton|SetIsButtonPressed true)
  (if (Variables|ActivationButton|GetIsPressable)
    (if (Utilities|Operators|EqualEqual (Transformation|GetWorldLocation (Variables|Default|GetMove)) (Variables|Movement|GetBottomLocation) 0.001)
      (CallFunction|MoveElevator (Variables|Movement|GetTopLocation))
      (else
        (CallFunction|MoveElevator (Variables|Movement|GetBottomLocation))))))

(event Custom|MoveDown
  (CallFunction|MoveElevator (Variables|Movement|GetBottomLocation)))

(event Custom|MoveElevator
  (params (EndLocation :type Vector%20%28by%20ref%29))
  (Variables|Movement|SetEnd%20Location EndLocation)
  (Variables|ActivationButton|SetIsPressable false)
  (Rendering|Material|SetScalarParameterValueonMaterials (Variables|/Game/Project/BP/LD/BP_Target.BP_Target_C|GetSM_GearAngle (Variables|Entities|GetTarget%20Enemy%20Elevator)) "Statue" 1.0)
  (Variables|Shake|SetElevatorRelativeLocation (Variables|/Script/Engine.SceneComponent|GetRelativeLocation (Variables|Default|GetMove)))
  (|ShakeStartTranslation
    (:On%20Complete
      (|ElevatorTranslation
        (:OnComplete
          (Transformation|SetWorldLocation (Variables|Default|GetMove) (Variables|Movement|GetEnd%20Location) false false)
          (Utilities|StartShakeonPlayerCamera "/Game/Project/BP/CameraShake/BP_Idle.BP_Idle_C"
            (:Output
              (Variables|Movement|SetCanGoUp (Utilities|Operators|EqualEqual (Variables|Movement|GetEnd%20Location) (Variables|Movement|GetBottomLocation) 0.0))
              (if (Variables|Entities|GetIsEnemyDead)
                (Variables|ActivationButton|SetIsPressable true)
                (Rendering|Material|SetScalarParameterValueonMaterials (Variables|/Game/Project/BP/LD/BP_Target.BP_Target_C|GetSM_GearAngle (Variables|Entities|GetTarget%20Enemy%20Elevator)) "Statue" 0.0)))))))))

(event Custom|MoveUp
  (CallFunction|MoveElevator (Variables|Movement|GetTopLocation)))

(event EventBeginPlay
  (bind _output_get (Variables|Movement|SetBottomLocation (Transformation|GetActorLocation)))
  (Variables|Movement|SetTopLocation (Math|Vector|MakeVector (.x _output_get) (.y _output_get) (+ (.z _output_get) (Variables|Movement|GetTopLocationZOffset))))
  (bind _asbp_turret_enemy (Utilities|Casting|CastToBP_TurretEnemy (Variables|/Script/Engine.ChildActorComponent|GetChildActor (Variables|Default|GetEnemy))))
  (EventDispatchers|BindEventtoOnDeathEvent (Variables|/Game/Project/BP/IA/Enemy/BP_TurretEnemy.BP_TurretEnemy_C|GetAC_Health _asbp_turret_enemy) (delegate Custom|ElevatorEnemyDeath))
  (bind _asbp_target_enemy_elevator (Utilities|Casting|CastToBP_Target_Enemy_Elevator (Variables|/Script/Engine.ChildActorComponent|GetChildActor (Variables|Default|GetElevatorTarget))))
  (Variables|Entities|SetTarget%20Enemy%20Elevator _asbp_target_enemy_elevator)
  (EventDispatchers|BindEventtoOnHealthChangedEvent (Variables|/Game/Project/BP/LD/BP_Target.BP_Target_C|GetAC_Health _asbp_target_enemy_elevator) (delegate Custom|OnTargetShot))
  (Variables|ActivationButton|SetIsPressable false)
  (Rendering|Material|SetScalarParameterValueonMaterials (Variables|/Game/Project/BP/LD/BP_Target.BP_Target_C|GetSM_GearAngle (Variables|Entities|GetTarget%20Enemy%20Elevator)) "Statue" 1.0)
  (Components|Activation|Deactivate (Variables|Default|GetSandFallingNiagara)))

(fn ConstructionScript)

(fn StopOngoingTranslation
  (bind _currenttranslation (Variables|Movement|GetCurrentTranslation))
  (Utilities|IsValid _currenttranslation
    (:Is%20Valid
      (Class|FCTweenBPAction|Stop _currenttranslation))))

(event Custom|StopShake
  ;[0.15 0.15 0.15 0.5] Shake elevator before translation
  (bind _shakevector (Timeline|TimelineShake Stop)
    (:Update
      (Transformation|SetRelativeLocation (Variables|Default|GetMove) (+ (* _shakevector (Variables|Shake|GetShakeBeforeTranslationIntensity)) (Variables|Shake|GetElevatorRelativeLocation)) false false))
    (:Finished
      (Transformation|SetRelativeLocation (Variables|Default|GetMove) (Variables|Shake|GetElevatorRelativeLocation) false false)
      (return))))