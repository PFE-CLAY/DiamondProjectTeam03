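; BP_AlliedSimple is a simple allied character that turns into a retrievable cadaver when it dies.
; On its health component's death event it sets IsDead, waits briefly, turns on mesh physics simulation and disables character movement.
; It then finds a BP_DroneRetriever in the level and registers itself with it as a new cadaver.
; Health changes only print a debug string, and a mesh collision change is left unconnected.
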(event OnDeathEvent(AC_Health)
  (Variables|Default|SetbIsDead true)
  (Utilities|FlowControl|Delay 0.7)
  (Physics|SetSimulatePhysics (Variables|Character|GetMesh) true)
  (Pawn|Components|CharacterMovement|DisableMovement (Variables|Character|GetCharacterMovement))
  (bind _returnvalue (Actor|GetActorOfClass "/Game/Project/BP/IA/Neutral/BP_DroneRetriever.BP_DroneRetriever_C"))
  (Class|DroneCadaver|GetNewCadaver _returnvalue self))

(event OnHealthChangedEvent(AC_Health)
  (params (CurrentHealth :type Integer))
  (Development|PrintString "Hello"))

(event EventBeginPlay)

(fn ConstructionScript)