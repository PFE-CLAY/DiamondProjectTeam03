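; BP_AlliedDream is an interactable that plays preplanned dream subtitles, one entry per interaction.
; On interact, it plays the first data table in the LoopSubsystem's PreplanDreamSubtitlesArray, then removes it, so the array acts as a queue held outside the actor.
; Once the queue is empty, each interaction plays DT_EndSubtitle instead.
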(event EventOnInteract
  (params (InteractingPlayer :type Character%20Object%20Reference))
  (if (Utilities|Array|IsNotEmpty (Variables|/Script/DiamondProject.LoopSubsystem|GetPreplanDreamSubtitlesArray (Subsystems|GetLoopSubsystem)))
    (CallFunction|PlaySubtitles (Utilities|Struct|MakeDataTableRowHandle (Utilities|Array|Get(acopy) (Variables|/Script/DiamondProject.LoopSubsystem|GetPreplanDreamSubtitlesArray (Subsystems|GetLoopSubsystem))) "None"))
    (Utilities|Array|RemoveIndex (Variables|/Script/DiamondProject.LoopSubsystem|GetPreplanDreamSubtitlesArray (Subsystems|GetLoopSubsystem)))
    (else
      (CallFunction|PlaySubtitles (Utilities|Struct|MakeDataTableRowHandle "/Game/Project/Subtitles/DataTables/DT_EndSubtitle.DT_EndSubtitle" "None")))))

(fn ConstructionScript
  (|CallParentFunction))