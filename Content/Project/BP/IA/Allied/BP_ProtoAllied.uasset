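; Prototype allied NPC that walks a scripted route and reports milestones to the LoopSubsystem, with sound cues along the way.
; StartNavigation waits briefly, flags ABP_NPC as moving, then chains AIMoveTo through two destinations before activating the "ManDoor" preplan step.
; AC_Health death plays ally and announcer sounds, activates "FallingTrap" and ragdolls the mesh.
; CompletedTask sets the animation's completion flag.
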(event OnDeathEvent(AC_Health)
  (Audio|SpawnSoundatLocation "/Game/Project/Sounds/Ally_VoiceLines/SFX_Ally_Death.SFX_Ally_Death" (Transformation|GetActorLocation self) "0, 0, 0" 1.0 1.0 0.0 0 0)
  (Utilities|FlowControl|Delay 0.7)
  (Audio|PlaySound2D "/Game/Project/Sounds/Announcer_VoiceLines/SFX_Announcer_AllyDeath.SFX_Announcer_AllyDeath" 1.0 1.0 0.0 0 0)
  (Class|LoopSubsystem|ActivatePreplanStep (Subsystems|GetLoopSubsystem) "FallingTrap")
  (Physics|SetSimulatePhysics (Variables|Character|GetMesh) true)
  (Collision|SetCollisionEnabled (Variables|Character|GetMesh) "PhysicsOnly"))

(event Custom|StartNavigation
  (bind _self self)
  (Audio|SpawnSoundatLocation "/Game/Project/Sounds/Ally_VoiceLines/SFX_Ally_EndElevator.SFX_Ally_EndElevator" (Transformation|GetActorLocation self) "0, 0, 0" 1.0 1.0 0.0 0 0)
  (Utilities|FlowControl|Delay 3.0)
  (Variables|/Game/Project/Assets/NPC_Assets/Animation/ABP_NPC.ABP_NPC_C|SetisMoving (.AsABP%20NPC (Utilities|Casting|CastToABP_NPC (Components|SkeletalMesh|GetAnimInstance (Variables|Character|GetMesh)))) true)
  (Development|PrintString "npc is moving")
  (AI|AIMoveTo _self "0, 0, 0" (Variables|Default|GetDestination) 5e+01 false
    (:OnSuccess
      (AI|AIMoveTo _self "0, 0, 0" (Variables|Default|GetDestinatio2) 5e+01 false
        (:OnSuccess
          (Class|LoopSubsystem|ActivatePreplanStep (Subsystems|GetLoopSubsystem) "ManDoor")
          (Audio|SpawnSoundatLocation "/Game/Project/Sounds/Ally_VoiceLines/SFX_Ally_Pyramid.SFX_Ally_Pyramid" (Transformation|GetActorLocation self) "0, 0, 0" 1.0 1.0 0.0 0 0))))))

(event Custom|CompletedTask
  (if true
    (Variables|/Game/Project/Assets/NPC_Assets/Animation/ABP_NPC.ABP_NPC_C|SethasCompletedTask (.AsABP%20NPC (Utilities|Casting|CastToABP_NPC (Components|SkeletalMesh|GetAnimInstance (Variables|Character|GetMesh)))) true)))

(event EventBeginPlay
  (Audio|SpawnSoundatLocation "/Game/Project/Sounds/Ally_VoiceLines/SFX_Ally_Elevator.SFX_Ally_Elevator" (Transformation|GetActorLocation self) "0, 0, 0" 1.0 1.0 0.0 0 0))

(fn ConstructionScript)