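; Flying mosquito enemy that pathfinds through a CPathVolume toward the player's location captured when Move is called, while always facing the player.
; The GoTo macro finds paths asynchronously, periodically rechecks them with velocity-alignment and line-trace node skipping, and sets an input vector that Tick applies.
; StopMovement interrupts the path.
; Health component death enables mesh physics and destroys the actor after a delay; an emissive/scale death timeline is left disconnected.
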(event OnHealthChangedEvent(AC_Health)
  (params (CurrentHealth :type Integer))
  (Development|PrintString "Hello"))

(event OnDeathEvent(AC_Health)
  (CallFunction|DestroyMe))

(event Custom|DestroyMe
  ;[1 1 1] Animating death and destroying actor
  (Physics|SetSimulatePhysics (Variables|Default|GetRootMesh) true)
  (Utilities|FlowControl|Delay 1.0)
  (Actor|DestroyActor))

(event Custom|Move
  (bind _overlappingactors (Collision|GetOverlappingActors "/Script/CPathfinding.CPathVolume" :!class /Script/Engine.Actor))
  ;[1 1 1] Movement
  (Variables|Default|SetShouldMove true)
  (if (Utilities|Array|IsNotEmpty _overlappingactors)
    (if (== (Utilities|Array|Get(acopy) _overlappingactors) (Variables|Default|GetVolumeRef))
      (Variables|GotoSettings|SetDestination (Transformation|GetActorLocation (Game|GetPlayerCharacter 0)))
      (Utilities|Goto (Variables|GotoSettings|GetDestination)
        (:Success
          _)
        (:Failed
          _))
      (Variables|Default|SetCurrentInputVector "0, 0, 0"))))

(event Custom|StopMovement
  ;[1 1 1] Movement
  (Variables|Default|SetShouldMove false)
  (Utilities|Goto (Variables|GotoSettings|GetDestination)) ; enters at Interupt
)

(event EventTick
  (params (DeltaSeconds :type Float%20%28single-precision%29))
  ;[1 1 1] Applying the input
  (if (Variables|Default|GetShouldMove)
    (Class|PawnMovementComponent|AddInputVector (Variables|Character|GetCharacterMovement) (Variables|Default|GetCurrentInputVector) false))
  (Transformation|SetActorRotation (Math|Rotator|FindLookatRotation (Transformation|GetActorLocation) (Transformation|GetActorLocation (Variables|Default|GetPlayer)))))

(event EventBeginPlay
  (bind _returnvalue (Actor|GetActorOfClass "/Script/CPathfinding.CPathVolume"))
  (Variables|Default|SetVolumeRef _returnvalue)
  (Variables|Default|SetPlayer (Game|GetPlayerCharacter 0)))

(fn ConstructionScript)

(fn GetNextOptimalNode
  (params (CurrentNodeIndex :type Integer))
  (LocalVariables|SetBestIndex CurrentNodeIndex)
  (LocalVariables|SetBestDot (CallFunction|GetDottoNode (Utilities|Array|Get(acopy) (Variables|Default|GetPathBuffer) CurrentNodeIndex)))
  (while (and (not (LocalVariables|GetWasHit)) (< (LocalVariables|GetBestIndex) (- (Utilities|Array|Length (Variables|Default|GetPathBuffer)) 1)))
    (bind _output_get (LocalVariables|SetCurrDot (CallFunction|GetDottoNode (Utilities|Array|Get(acopy) (Variables|Default|GetPathBuffer) (+ (LocalVariables|GetBestIndex) 1)))))
    (if (> _output_get (LocalVariables|GetBestDot))
      (bind _returnvalue (Collision|LineTraceByChannel (Transformation|GetActorLocation) (.WorldLocation (Utilities|Struct|BreakCPathNode (Utilities|Array|Get(acopy) (Variables|Default|GetPathBuffer) (+ (LocalVariables|GetBestIndex) 1)))) "TraceTypeQuery1" false 0 "None"))
      (bind _output_get_2 (LocalVariables|SetWasHit _returnvalue))
      (if (not _output_get_2)
        (LocalVariables|SetBestDot (LocalVariables|GetCurrDot))
        (Math|Integer|IncrementInt (LocalVariables|GetBestIndex)
          (:%20%20
            (if (>= (LocalVariables|GetBestIndex) (- (Utilities|Array|Length (Variables|Default|GetPathBuffer)) 2))
              (return (LocalVariables|GetBestIndex))))))
      (else
        (return (LocalVariables|GetBestIndex)))))
  (return (LocalVariables|GetBestIndex)))

(fn GetDottoNode
  (params (Node :type C%20Path%20Node%20Structure))
  (return (Math|Vector|DotProduct (Math|Vector|Normalize (Variables|/Script/Engine.MovementComponent|GetVelocity (Variables|Default|GetFlyingMovementComponent))) (Math|Vector|Normalize (- (.WorldLocation (Utilities|Struct|BreakCPathNode Node)) (Transformation|GetActorLocation))))))

(fn DrawPath
  (if (and (Variables|GoToSettings|Additional|GetDrawDebugPath) (Utilities|IsValid (Variables|Default|GetVolumeRef)))
    (Class|CPathVolume|DrawDebugPath (Variables|Default|GetVolumeRef) (Variables|Default|GetPathBuffer) 0.2 true (Variables|GoToSettings|Additional|GetDebugPathColor))))

(fn CheckIsPlayeratRange
  (return (<= (Math|Vector|Distance(Vector) (Transformation|GetActorLocation) (Transformation|GetActorLocation (Game|GetPlayerCharacter 0))) (Variables|MosquitoEnemy|GetRangeDetection))))