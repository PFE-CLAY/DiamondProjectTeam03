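; Melee enemy spawner with an animated door and two child-actor conveyor belts, a main one and an extendable ramp.
; Opening starts the main belt, then chains float tweens to raise the door, slide and lift the ramp, and start its belt.
; Closing reverses the sequence.
; An activation zone starts the behavior of overlapping melee enemies from this spawner and removes them from its tracked array.
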(event OnComponentBeginOverlap(ActivationZone)
  (params (OverlappedComponent :type Primitive%20Component%20Object%20Reference) (OtherActor :type Actor%20Object%20Reference) (OtherComp :type Primitive%20Component%20Object%20Reference) (OtherBodyIndex :type Integer) (bFromSweep :type Boolean) (SweepResult :type Hit%20Result%20Structure%20%28by%20ref%29))
  (bind _asmelee_enemy (Utilities|Casting|CastToMeleeEnemy OtherActor))
  (if (Utilities|Array|ContainsItem (Variables|Default|GetSpawnedEnemiesInSpawner) _asmelee_enemy)
    (Class|ShootingEnemy|StartBehavior _asmelee_enemy)
    (Class|MeleeSpawner|RemoveEnemyfromArray _asmelee_enemy)))

(event Custom|RampOpen
  (bind _conveyorbeltextra (Variables|Default|GetConveyorBeltExtra))
  (bind _conveyorbeltextra_2 (Variables|Default|GetConveyorBeltExtra))
  (bind _relativelocation (Variables|/Script/Engine.SceneComponent|GetRelativeLocation _conveyorbeltextra))
  (bind _relativelocation_2 (Variables|/Script/Engine.SceneComponent|GetRelativeLocation _conveyorbeltextra_2))
  (bind _value (|TweenFloat (.x _relativelocation) (+ (.x _relativelocation) 75.0) 1.0 "InOutQuad")
    (:ApplyEasing
      (Transformation|SetRelativeLocation (Variables|Default|GetConveyorBeltExtra) (Math|Vector|MakeVector _value (.y _relativelocation) (.z _relativelocation)) false false))
    (:OnComplete
      (bind _value_2 (|TweenFloat (.z _relativelocation_2) 0.0 0.3 "InOutQuad")
        (:ApplyEasing
          (Transformation|SetRelativeLocation (Variables|Default|GetConveyorBeltExtra) (Math|Vector|MakeVector (.x _relativelocation_2) (.y _relativelocation_2) _value_2) false false))
        (:OnComplete
          (Default|Activate (Variables|Default|GetSubConveyor) true))))))

(event Custom|RampClose
  (bind _door (Variables|Default|GetDoor))
  (bind _door_2 (Variables|Default|GetDoor))
  (bind _conveyorbeltextra (Variables|Default|GetConveyorBeltExtra))
  (bind _conveyorbeltextra_2 (Variables|Default|GetConveyorBeltExtra))
  (bind _returnvalue (Transformation|GetWorldLocation _door))
  (bind _returnvalue_2 (Transformation|GetWorldLocation _door_2))
  (bind _relativelocation (Variables|/Script/Engine.SceneComponent|GetRelativeLocation _conveyorbeltextra))
  (bind _relativelocation_2 (Variables|/Script/Engine.SceneComponent|GetRelativeLocation _conveyorbeltextra_2))
  (Default|Activate (Variables|Default|GetSubConveyor) false)
  (bind _value (|TweenFloat (.z _relativelocation_2) -3.0 0.3 "InOutQuad")
    (:ApplyEasing
      (Transformation|SetRelativeLocation (Variables|Default|GetConveyorBeltExtra) (Math|Vector|MakeVector (.x _relativelocation_2) (.y _relativelocation_2) _value) false false))
    (:OnComplete
      (bind _value_2 (|TweenFloat (.x _relativelocation) (- (.x _relativelocation) 75.0) 1.0 "InOutQuad")
        (:ApplyEasing
          (Transformation|SetRelativeLocation (Variables|Default|GetConveyorBeltExtra) (Math|Vector|MakeVector _value_2 (.y _relativelocation) (.z _relativelocation)) false false))
        (:OnComplete
          (Default|Activate (Variables|Default|GetMainConveyor) false)
          (Variables|Default|SetbIsDoorOpened false)
          (bind _value_3 (|TweenFloat (.z _returnvalue) (- (.z _returnvalue) 3.5e+02) 1.0 "InOutQuad")
            (:ApplyEasing
              (Transformation|SetWorldLocation _door_2 (Math|Vector|MakeVector (.x _returnvalue_2) (.y _returnvalue_2) _value_3) false false))))))))

(event EventBeginPlay
  (bind _asbp_conveyor_belt (Utilities|Casting|CastToBP_ConveyorBelt (Variables|/Script/Engine.ChildActorComponent|GetChildActor (Variables|Default|GetConveyorBelt))))
  (Variables|Default|SetMainConveyor _asbp_conveyor_belt)
  (bind _asbp_conveyor_belt_2 (Utilities|Casting|CastToBP_ConveyorBelt (Variables|/Script/Engine.ChildActorComponent|GetChildActor (Variables|Default|GetConveyorBeltExtra))))
  (Variables|Default|SetSubConveyor _asbp_conveyor_belt_2)
  (Variables|Default|SetbIsReady true)
  (Variables|/Game/Project/BP/LD/BP_ConveyorBelt.BP_ConveyorBelt_C|SetSpeed (Variables|Default|GetMainConveyor) (Variables|Default|GetSpeed))
  (Variables|/Game/Project/BP/LD/BP_ConveyorBelt.BP_ConveyorBelt_C|SetSpeed (Variables|Default|GetSubConveyor) (Variables|Default|GetSpeed)))

(event EventCloseSpawnDoor
  (CallFunction|RampClose))

(event EventOpenSpawnDoor
  (bind _mainconveyor (Variables|Default|GetMainConveyor))
  (bind _door (Variables|Default|GetDoor))
  (bind _door_2 (Variables|Default|GetDoor))
  (bind _returnvalue (Transformation|GetWorldLocation _door))
  (bind _returnvalue_2 (Transformation|GetWorldLocation _door_2))
  (Utilities|IsValid _mainconveyor
    (:Is%20Valid
      (Default|Activate _mainconveyor true)
      (Variables|Default|SetbIsDoorOpened true)
      (bind _value (|TweenFloat (.z _returnvalue) (+ (.z _returnvalue) 3.5e+02) 1.0 "InOutQuad")
        (:ApplyEasing
          (Transformation|SetWorldLocation _door_2 (Math|Vector|MakeVector (.x _returnvalue_2) (.y _returnvalue_2) _value) false false))
        (:OnComplete
          (CallFunction|RampOpen))))))

(fn ConstructionScript)