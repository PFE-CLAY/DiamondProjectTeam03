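; Turret enemy Blueprint that handles the audio, VFX and animation feedback for shooting and death.
; On BeginPlay it binds the enemy shoot event, caches its AnimBP and creates a dynamic metal material.
; Each shot plays Wwise audio and, given a valid shoot point, spawns VFX and briefly pulses shooting state with the firing side.
; Death from the health component plays sound and disintegration VFX, then tweens a dissolve before calling OnDeath.
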(event OnDeathEvent(AC_Health)
  (params (DamageDealer :type Actor%20Object%20Reference) (OwnerActor :type Actor%20Object%20Reference))
  (Class|WwiseManagerSubsystem|PostEvent (Subsystems|GetWwiseManagerSubsystem) "/Game/WwiseAudio/Events/FOES_Tourelle_WU/Play_FOES_SFX_Tourelle_Death_RC.Play_FOES_SFX_Tourelle_Death_RC" self)
  (Niagara|SpawnSystematLocation "/Game/Project/VFX/FXS_StaticDisintegration.FXS_StaticDisintegration" (Transformation|GetWorldLocation (Variables|Default|GetDeathEffectSpawn)) (Transformation|GetActorRotation))
  (bind _value (|TweenFloat 1.0 0.0 (Variables|Default|GetDissolveEffectDuration) "Linear")
    (:ApplyEasing
      (Rendering|Material|SetScalarParameterValue (Variables|Default|GetEnemyMetalMatInstance) "Dissolve" _value :!class /Script/Engine.MaterialInstanceDynamic))
    (:OnComplete
      (Class|Enemy|OnDeath))))

(event Custom|ChangeShooting
  (params (IsShooting :type Boolean))
  (Variables|/Game/Project/01-Assets/Enemies/Enemy_Turret/Animation/ABP_TurretEnemy.ABP_TurretEnemy_C|SetIsShooting (Variables|Default|GetAnimBP) IsShooting))

(event Custom|OnEnemyShoot_Event
  (bind _returnvalue (Class|ShootingEnemy|GetCurrentShootPoint))
  (Class|WwiseManagerSubsystem|PostEvent (Subsystems|GetWwiseManagerSubsystem) "/Game/WwiseAudio/Events/FOES_Tourelle_WU/Play_FOES_SFX_Tourelle_Shoot_RC.Play_FOES_SFX_Tourelle_Shoot_RC" self)
  (Utilities|IsValid _returnvalue
    (:Is%20Valid
      (CallFunction|ChangeSide (Variables|Default|GetShootSide))
      (CallFunction|ChangeShooting true)
      (Niagara|SpawnSystematLocation "/Game/Project/VFX/FXS_EnemyShoot.FXS_EnemyShoot" (Transformation|GetWorldLocation _returnvalue))
      (Utilities|FlowControl|Delay 0.1)
      (CallFunction|ChangeShooting false))))

(event Custom|ChangeSide
  (params (Side :type EShootSide%20Enum :default "Right"))
  (Variables|/Game/Project/01-Assets/Enemies/Enemy_Turret/Animation/ABP_TurretEnemy.ABP_TurretEnemy_C|SetShootSide (Variables|Default|GetAnimBP) Side))

(event Custom|ChangeActivation
  (params (IsActive :type Boolean))
  (Variables|/Game/Project/01-Assets/Enemies/Enemy_Turret/Animation/ABP_TurretEnemy.ABP_TurretEnemy_C|SetIsActivated (Variables|Default|GetAnimBP) IsActive))

(event EventBeginPlay
  (EventDispatchers|BindEventtoOnEnemyShoot (delegate Custom|OnEnemyShoot_Event))
  (bind _asabp_turret_enemy (Utilities|Casting|CastToABP_TurretEnemy (Components|SkeletalMesh|GetAnimInstance (Variables|Character|GetMesh)))
    (:then
      (Variables|Default|SetAnimBP _asabp_turret_enemy))
    (:CastFailed
      _))
  (bind _returnvalue (Rendering|Material|CreateDynamicMaterialInstance (Variables|Character|GetMesh) 0 "/Game/Project/Assets/Enemy_Turret/M_EnemyMetal_3.M_EnemyMetal_3" "None" :!class /Script/Engine.PrimitiveComponent))
  (Variables|Default|SetEnemyMetalMatInstance _returnvalue))

(fn ConstructionScript)