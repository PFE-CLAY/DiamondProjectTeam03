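; BP_TurretEnemyInactive is a turret enemy variant with a deactivated metal material, handling death and shoot feedback.
; BeginPlay creates dynamic metal and cloth materials and binds the shoot event.
; Health death plays turret and crowd audio, spawns disintegration Niagara, and tweens both materials' Dissolve before calling OnDeath.
; Shooting only posts a Wwise sound, as the muzzle effect spawn is disconnected.
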(event OnDeathEvent(AC_Health)
  (params (DamageDealer :type Actor%20Object%20Reference) (OwnerActor :type Actor%20Object%20Reference))
  (Class|WwiseManagerSubsystem|PostEvent (Subsystems|GetWwiseManagerSubsystem) "/Game/WwiseAudio/Events/FOES_Tourelle_WU/Play_FOES_SFX_Tourelle_Death_RC.Play_FOES_SFX_Tourelle_Death_RC" self)
  (Audio|SpawnSoundatLocation "/Game/Project/Sounds/Folleys/Sound_effect_Arena_Crowd_Cheer.Sound_effect_Arena_Crowd_Cheer" "1930.000000,0.000000,2320.000000" "0, 0, 0" 0.4 1.0 0.0 "/Game/Project/Sounds/A_GlobalAttenuation.A_GlobalAttenuation" 0)
  (Niagara|SpawnSystematLocation "/Game/Project/VFX/FXS_StaticDisintegration.FXS_StaticDisintegration" (Transformation|GetWorldLocation (Variables|Default|GetDeathEffectSpawn)) (Transformation|GetActorRotation))
  (bind _value (|TweenFloat 1.0 0.0 (Variables|Default|GetDissolveEffectDuration) "Linear")
    (:ApplyEasing
      (Rendering|Material|SetScalarParameterValue (Variables|Default|GetEnemyMetalMatInstance) "Dissolve" _value :!class /Script/Engine.MaterialInstanceDynamic)
      (Rendering|Material|SetScalarParameterValue (Variables|Default|GetEnemyClothMatInstance) "Dissolve" _value :!class /Script/Engine.MaterialInstanceDynamic))
    (:OnComplete
      (Class|Enemy|OnDeath))))

(event Custom|OnEnemyShoot_Event
  (Class|WwiseManagerSubsystem|PostEvent (Subsystems|GetWwiseManagerSubsystem) "/Game/WwiseAudio/Events/FOES_Tourelle_WU/Play_FOES_SFX_Tourelle_Shoot_RC.Play_FOES_SFX_Tourelle_Shoot_RC" self)
  (Utilities|IsValid (Class|ShootingEnemy|GetCurrentShootPoint)))

(event EventBeginPlay
  (bind _enemy (Variables|Default|GetEnemy))
  (EventDispatchers|BindEventtoOnEnemyShoot (delegate Custom|OnEnemyShoot_Event))
  (bind _returnvalue (Rendering|Material|CreateDynamicMaterialInstance _enemy 0 "/Game/Project/Assets/Enemy_Turret/M_EnemyMetal_3_Desactive.M_EnemyMetal_3_Desactive" "None" :!class /Script/Engine.PrimitiveComponent))
  (Variables|Default|SetEnemyMetalMatInstance _returnvalue)
  (bind _returnvalue_2 (Rendering|Material|CreateDynamicMaterialInstance _enemy 1 "/Game/Project/Assets/Enemy_Turret/M_EnemyCloth_3.M_EnemyCloth_3" "None" :!class /Script/Engine.PrimitiveComponent))
  (Variables|Default|SetEnemyClothMatInstance _returnvalue_2))

(fn ConstructionScript)