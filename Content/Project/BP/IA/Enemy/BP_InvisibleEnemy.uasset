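; BP_InvisibleEnemy is an invisible enemy that patrols a looping list of waypoints through AI MoveTo.
; While moving, two offset looping timers spawn alternating left and right footprint actors at foot locations, revealing its path.
; When its health component reports death, it plays a crowd cheer and death effect, leaves a death print, then calls OnDeath.
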(event OnDeathEvent(AC_Health)
  (Audio|SpawnSoundatLocation "/Game/Project/Sounds/Folleys/Sound_effect_Arena_Crowd_Cheer.Sound_effect_Arena_Crowd_Cheer" (Transformation|GetActorLocation) "0, 0, 0" 0.4 1.0 0.0 "/Game/Project/Sounds/A_GlobalAttenuation.A_GlobalAttenuation" 0)
  (Niagara|SpawnSystematLocation "/Game/Project/VFX/FXS_EnemyDeath.FXS_EnemyDeath" (Transformation|GetActorLocation))
  (Game|SpawnActorfromClass "/Game/Project/BP/IA/Enemy/BP_DeathPrint.BP_DeathPrint_C" (Math|Transform|MakeTransform (Transformation|GetWorldLocation (Variables|Default|GetFootstepL)) (Transformation|GetActorRotation) "1.000000,1.000000,1.000000") "Undefined" "MultiplyWithRoot" 0 0)
  (Class|Enemy|OnDeath))

(event Custom|SpawnFootstepL
  (if (> (Math|Vector|VectorLength (Variables|/Script/Engine.MovementComponent|GetVelocity (Variables|Character|GetCharacterMovement))) 0.0)
    (Game|SpawnActorfromClass "/Game/Project/BP/IA/Enemy/BP_Footstep_L.BP_Footstep_L_C" (Math|Transform|MakeTransform (Transformation|GetWorldLocation (Variables|Default|GetFootstepL)) (Transformation|GetActorRotation) "0.100000,0.100000,0.100000") "Undefined" "MultiplyWithRoot" 0 0)))

(event Custom|SpawnFootstepR
  (if (> (Math|Vector|VectorLength (Variables|/Script/Engine.MovementComponent|GetVelocity (Variables|Character|GetCharacterMovement))) 0.0)
    (Game|SpawnActorfromClass "/Game/Project/BP/IA/Enemy/BP_Footstep_R.BP_Footstep_R_C" (Math|Transform|MakeTransform (Transformation|GetWorldLocation (Variables|Default|GetFootstepR)) (Transformation|GetActorRotation) "0.100000,0.100000,0.100000") "Undefined" "MultiplyWithRoot" 0 0)))

(event Custom|Move
  (AI|AIMoveTo self "0, 0, 0" (Utilities|Array|Get(acopy) (Variables|Default|GetWaypoints) (Variables|Default|GetWaypointIndex)) 5.0 false
    (:OnSuccess
      (bind _result (Math|Integer|IncrementInt (Variables|Default|GetWaypointIndex))
        (:%20%20
          (Variables|Default|SetWaypointIndex (Math|Integer|%(Integer) _result (Utilities|Array|Length (Variables|Default|GetWaypoints))))
          (CallFunction|Move))))))

(event EventBeginPlay
  (bind _intervalfootsteps (Variables|Default|GetIntervalFootsteps))
  (Utilities|Time|SetTimerbyEvent (delegate Custom|SpawnFootstepL) (Variables|Default|GetIntervalFootsteps) true)
  (Utilities|Time|SetTimerbyEvent (delegate Custom|SpawnFootstepR) _intervalfootsteps true false (/ _intervalfootsteps 2.0))
  (CallFunction|Move))

(fn ConstructionScript)