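; Melee enemy that charges, then damages the player through a hemisphere hitbox, driven by an AI Blackboard seeded with range and timing values.
; Charge and attack events toggle Niagara effects and the hitbox's overlap response, while a tween eases walk speed over the attack before restoring it.
; Helper functions compute a position relative to the player's activation range.
; Death swaps the actor for a Geometry Collection shattered by a radial field, plus VFX.
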(event OnComponentBeginOverlap(SemiSphere)
  (params (OverlappedComponent :type Primitive%20Component%20Object%20Reference) (OtherActor :type Actor%20Object%20Reference) (OtherComp :type Primitive%20Component%20Object%20Reference) (OtherBodyIndex :type Integer) (bFromSweep :type Boolean) (SweepResult :type Hit%20Result%20Structure%20%28by%20ref%29))
  (if (== OtherActor (Game|Player|GetPlayerPawn 0))
    (Class|ACHealth|DecreaseHealth (Variables|/Game/Project/Game/BP_FirstPersonCharacter.BP_FirstPersonCharacter_C|GetHealth%20Component (Variables|Default|GetPlayer)) (Variables|Default|GetAttackDamage) self)))

(event OnDeathEvent(AC_Health)
  (params (DamageDealer :type Actor%20Object%20Reference) (OwnerActor :type Actor%20Object%20Reference))
  (bind _returnvalue (Transformation|GetActorRotation))
  (bind _returnvalue_2 (Game|SpawnActorfromClass "/Script/GeometryCollectionEngine.GeometryCollectionActor" (Math|Transform|MakeTransform (.location (Transformation|GetActorTransform)) (Math|Rotator|MakeRotator (.roll _returnvalue) (.pitch _returnvalue) (+ (.yaw _returnvalue) 9e+01)) "1.000000,1.000000,1.000000") "Undefined" "MultiplyWithRoot" 0 0))
  (Collision|SetCollisionProfileName (Variables|/Script/GeometryCollectionEngine.GeometryCollectionActor|GetGeometryCollectionComponent _returnvalue_2) "Debris" true :!class /Script/Engine.PrimitiveComponent)
  (Class|GeometryCollectionComponent|SetRestCollection (Variables|/Script/GeometryCollectionEngine.GeometryCollectionActor|GetGeometryCollectionComponent _returnvalue_2) (Variables|Default|GetOnDeathGeometryCollection) true)
  (bind _returnvalue_3 (Game|SpawnActorfromClass "/Game/Project/BP/Sandbox/BreakableObjects/FS_BlacksandsField.FS_BlacksandsField_C" (Math|Transform|MakeTransform (+ (Transformation|GetActorLocation) "") "0, 0, 0" "1.000000,1.000000,1.000000") "AlwaysSpawn" "MultiplyWithRoot" 0 0))
  (Variables|/Engine/EditorResources/FieldNodes/FS_MasterField.FS_MasterField_C|SetRadial%20Magnitude _returnvalue_3 7.5e+02)
  (Default|CETrigger _returnvalue_3)
  (Niagara|SpawnSystematLocation "/Game/Project/VFX/FXS_MeleeEnemyDeath.FXS_MeleeEnemyDeath" (Transformation|GetWorldLocation (Variables|Character|GetMesh)) "0, 0, 0" "5.000000,5.000000,5.000000" true true "AutoRelease")
  (Actor|DestroyActor))

(event Custom|DisableAttack
  (Variables|Default|SetbIsAttacking false)
  (Variables|/Script/Engine.CharacterMovementComponent|SetMaxWalkSpeed (Variables|Character|GetCharacterMovement) (Variables|Default|GetSpeed))
  (Collision|SetCollisionResponsetoChannel (Variables|Default|GetSemiSphere) "ECC_GameTraceChannel4" "ECR_Ignore")
  (Components|Activation|Deactivate (Variables|Default|GetNiagara)))

(event Custom|ChargeEffect
  (Components|Activation|Activate (Variables|Default|GetChargeVFX) true))

(event Custom|EnableAttack
  (params (AttackTarget :type Actor%20Object%20Reference))
  (bind _charactermovement (Variables|Character|GetCharacterMovement))
  (Variables|Default|SetbIsAttacking true)
  (Collision|SetCollisionResponsetoChannel (Variables|Default|GetSemiSphere) "ECC_GameTraceChannel4" "ECR_Overlap")
  (Components|Activation|Activate (Variables|Default|GetNiagara) false)
  (bind _value (|TweenFloat (Variables|/Script/Engine.CharacterMovementComponent|GetMaxWalkSpeed _charactermovement) 1e+02 (Variables|Default|GetAttackDuration) "OutQuad")
    (:ApplyEasing
      (Variables|/Script/Engine.CharacterMovementComponent|SetMaxWalkSpeed _charactermovement _value))
    (:OnComplete
      (CallFunction|DisableAttack))))

(event EventOnAttackEvent
  (params (Target :type Actor%20Object%20Reference))
  (CallFunction|EnableAttack Target)
  (Components|Activation|Deactivate (Variables|Default|GetChargeVFX)))

(event EventBeginPlay
  (bind _asbp_first_person_character (Utilities|Casting|CastToBP_FirstPersonCharacter (Game|GetPlayerCharacter 0)))
  (Variables|Default|SetPlayer _asbp_first_person_character)
  (EventDispatchers|AssignOnChargeEvent (delegate Custom|ChargeEffect)))

(event EventStartBehavior
  (|CallParentFunction)
  (|SetupAIvalues))

(fn ConstructionScript)

(fn GetXYVector
  (params (Origin :type Vector) (Destination :type Vector))
  (bind (_x _y) (Math|Vector|BreakVector Origin))
  (bind (_x_2 _y_2) (Math|Vector|BreakVector Destination))
  (return (Math|Vector|MakeVector (- _x_2 _x) (- _y_2 _y) 0.0)))

(fn GetClosestPos
  (params (CurrentPawnPos :type Vector) (PlayerPos :type Vector) (RangeFromPlayer :type Float%20%28double-precision%29))
  (bind _vector (CallFunction|GetXYVector CurrentPawnPos PlayerPos))
  (bind (_x _y) (Math|Vector|BreakVector PlayerPos))
  (bind _returnvalue (Math|Vector|VectorLength _vector))
  (if (> _returnvalue RangeFromPlayer)
    (return (+ (Math|Vector|MakeVector _x _y (.z PlayerPos)) (+ (CallFunction|GetXYVector PlayerPos CurrentPawnPos) (* (Math|Vector|Normalize _vector) (- _returnvalue RangeFromPlayer)))))
    (else
      (return CurrentPawnPos))))

(fn GetPlayerCustomPos
  (return (CallFunction|GetClosestPos (Transformation|GetActorLocation) (Transformation|GetActorLocation (Game|Player|GetPlayerPawn 0)) (Variables|AttackMelee|GetActivationRange))))

(event Custom|OnMeleeAttackEvent
  (Utilities|FlowControl|Delay 0.3)
  (AI|Components|Blackboard|SetValueasBool (AI|GetBlackboard (Variables|Default|GetAIController)) (Utilities|Name|MakeLiteralName "IsCharging") false))