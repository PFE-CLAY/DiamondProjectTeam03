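; Flying drone that retrieves cadavers, carrying each back to the incinerator hatch and throwing it in.
; A GoTo macro requests an async 3D path from the overlapped CPathVolume, then steers node to node by setting an input vector that Tick feeds to the flying movement component.
; Trips through the hatch bypass pathfinding, using delayed float tweens to lerp the drone between its spawn origin and the hatch.
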(event Custom|GoBackToOrigin
  (bind _hatchincinerator (Variables|Default|GetHatchIncinerator))
  (Utilities|Goto (Variables|/Script/DiamondProject.HatchIncinerator|GetDroneStartLocation _hatchincinerator)
    (:Success
      (Variables|Default|SetCurrentInputVector "0, 0, 0")
      (Utilities|FlowControl|Delay 1.5)
      (Class|HatchIncinerator|OnOpenHatch _hatchincinerator)
      (Utilities|FlowControl|Delay 2.5)
      (Class|DroneCadaver|ThrowBody)
      (Components|Activation|Deactivate (Variables|Default|GetCatch%20Drone%20VFX)))))

(event EventBeginPlay
  (Variables|Default|SetOrigin (Transformation|GetActorLocation))
  (Components|Activation|Deactivate (Variables|Default|GetCatch%20Drone%20VFX)))

(event EventOnMovingtoNewCadaver
  (params (Target :type Allied%20Object%20Reference))
  (Utilities|IsValid Target
    (:Is%20Valid
      (Utilities|Goto (+ (Transformation|GetWorldLocation (Variables|/Script/DiamondProject.Allied|GetGrabPoint Target)) (Math|Vector|MakeVector 0.0 0.0 2e+02))
        (:Success
          (Variables|Default|SetCurrentInputVector "0, 0, 0")
          (Components|Activation|Activate (Variables|Default|GetCatch%20Drone%20VFX) false)
          (Class|DroneCadaver|CarryBody)
          (Utilities|FlowControl|Delay 1.0)
          (CallFunction|GoBacktoOrigin))
        (:Failed
          (Variables|Default|SetCurrentInputVector "0, 0, 0"))))))

(event EventTick
  (params (DeltaSeconds :type Float%20%28single-precision%29))
  ;[1 1 1] Applying the input
  (Class|PawnMovementComponent|AddInputVector (Variables|Default|GetFlyingMovementComponent) (Variables|Default|GetCurrentInputVector) false))

(event EventGoOutHatch
  (Class|HatchIncinerator|OnOpenHatch (Variables|Default|GetHatchIncinerator))
  (bind _value (|TweenFloat 0.0 1.0 2.0 "InOutQuad" 0.0 0.0 2.0)
    (:ApplyEasing
      (Transformation|SetActorLocation (Math|Vector|Lerp(Vector) (Variables|Default|GetOrigin) (Variables|/Script/DiamondProject.HatchIncinerator|GetDroneStartLocation (Variables|Default|GetHatchIncinerator)) _value) false false))
    (:OnComplete
      (Class|DroneCadaver|GotoNewTarget))))

(event EventGoinHatch
  (Class|HatchIncinerator|OnOpenHatch (Variables|Default|GetHatchIncinerator))
  (bind _value (|TweenFloat 0.0 1.0 5.0 "InOutQuad" 0.0 0.0 2.0)
    (:ApplyEasing
      (Transformation|SetActorLocation (Math|Vector|Lerp(Vector) (Transformation|GetActorLocation) (Variables|Default|GetOrigin) _value) false false))))

(fn ConstructionScript)

(fn GetNextOptimalNode
  (params (CurrentNodeIndex :type Integer))
  (LocalVariables|SetBestIndex CurrentNodeIndex)
  (LocalVariables|SetBestDot (CallFunction|GetDottoNode (Utilities|Array|Get(acopy) (Variables|Default|GetPathBuffer) CurrentNodeIndex)))
  (while (and (not (LocalVariables|GetWasHit)) (< (LocalVariables|GetBestIndex) (- (Utilities|Array|Length (Variables|Default|GetPathBuffer)) 1)))
    (bind _output_get (LocalVariables|SetCurrDot (CallFunction|GetDottoNode (Utilities|Array|Get(acopy) (Variables|Default|GetPathBuffer) (+ (LocalVariables|GetBestIndex) 1)))))
    (if (> _output_get (LocalVariables|GetBestDot))
      (bind _returnvalue (Collision|LineTraceByChannel (Transformation|GetActorLocation) (.WorldLocation (Utilities|Struct|BreakCPathNode (Utilities|Array|Get(acopy) (Variables|Default|GetPathBuffer) (+ (LocalVariables|GetBestIndex) 1)))) "TraceTypeQuery1" false 0 "None"))
      (bind _output_get_2 (LocalVariables|SetWasHit _returnvalue))
      (if (not _output_get_2)
        (LocalVariables|SetBestDot (LocalVariables|GetCurrDot))
        (Math|Integer|IncrementInt (LocalVariables|GetBestIndex)
          (:%20%20
            (if (>= (LocalVariables|GetBestIndex) (- (Utilities|Array|Length (Variables|Default|GetPathBuffer)) 2))
              (return (LocalVariables|GetBestIndex))))))
      (else
        (return (LocalVariables|GetBestIndex)))))
  (return (LocalVariables|GetBestIndex)))

(fn GetDottoNode
  (params (Node :type C%20Path%20Node%20Structure))
  (return (Math|Vector|DotProduct (Math|Vector|Normalize (Variables|/Script/Engine.MovementComponent|GetVelocity (Variables|Default|GetFlyingMovementComponent))) (Math|Vector|Normalize (- (.WorldLocation (Utilities|Struct|BreakCPathNode Node)) (Transformation|GetActorLocation))))))

(fn DrawPath
  (if (and (Variables|GoToSettings|Additional|GetDrawDebugPath) (Utilities|IsValid (Variables|Default|GetVolumeRef)))
    (Class|CPathVolume|DrawDebugPath (Variables|Default|GetVolumeRef) (Variables|Default|GetPathBuffer) 0.2 true (Variables|GoToSettings|Additional|GetDebugPathColor))))