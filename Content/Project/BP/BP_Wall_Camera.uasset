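; BP_Wall_Camera is an actor that continually turns with the player's position.
; Each Tick starts a short TweenRotator toward the look-at rotation from player character to actor, so its forward axis eases to point away from the player.
; The eased value sets the actor's rotation.
; BeginPlay caches the BP_FirstPersonCharacter reference, which the rotation logic does not use.
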(event EventBeginPlay
  (bind _asbp_first_person_character (Utilities|Casting|CastToBP_FirstPersonCharacter (Game|GetPlayerCharacter 0)))
  (Variables|Default|SetAs%20BP%20First%20Person%20Character _asbp_first_person_character))

(event EventTick
  (params (DeltaSeconds :type Float%20%28single-precision%29))
  (bind _self self)
  (bind _value (|TweenRotator (Transformation|GetActorRotation _self) (Math|Rotator|FindLookatRotation (Transformation|GetActorLocation (Game|GetPlayerCharacter 0)) (Transformation|GetActorLocation _self)) 0.2 "InOutQuad")
    (:ApplyEasing
      (Transformation|SetActorRotation _self _value))))

(fn ConstructionScript)