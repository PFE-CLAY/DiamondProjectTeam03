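; Prototype teleport plane actor with a scene capture component whose render target is assigned in the construction script.
; On actor overlap, it compares the capture's rotation to the player capsule's within a tolerance.
; On a match, it moves the player to their mesh location offset by the capture's forward vector, a step marked as a failed attempt.
; Distance-driven FOV and facing-angle debug experiments remain disconnected.
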(event Collision|EventActorBeginOverlap
  (params (OtherActor :type Actor%20Object%20Reference))
  (bind _returnvalue (Game|GetPlayerCharacter 0))
  (if (Utilities|Operators|EqualEqual (Transformation|GetWorldRotation (Variables|Default|GetSceneCaptureComponent2D)) (Transformation|GetWorldRotation (Variables|/Script/Engine.Character|GetCapsuleComponent (Game|GetPlayerCharacter 0))) (Variables|Default|GetTolerance))
    (Transformation|SetActorLocation _returnvalue (+ (Transformation|GetWorldLocation (Variables|/Script/Engine.Character|GetMesh _returnvalue)) (Math|Vector|GetForwardVector (Variables|Default|GetSceneCaptureComponent2D))) false false)))

(fn ConstructionScript
  (Variables|/Script/Engine.SceneCaptureComponent2D|SetTextureTarget (Variables|Default|GetSceneCaptureComponent2D) (Variables|Default|GetTexture%20Target)))