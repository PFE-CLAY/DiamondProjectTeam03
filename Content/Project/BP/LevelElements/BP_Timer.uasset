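; Level countdown timer that kills the player when time runs out.
; On BeginPlay it binds to the NPC activation zone's enter-arena dispatcher to start and the generators door's finish-level dispatcher to stop, then caches the interact HUD.
; While running, Tick decrements the time to a floor of zero and pushes it to the HUD.
; At zero, a DoOnce calls OnDeath on the first-person character.
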(event Custom|StartTimerEvent
  (Variables|Default|SetShouldTickTimer true))

(event Custom|StopTimerEvent
  (Variables|Default|SetShouldTickTimer false))

(event EventTick
  (params (DeltaSeconds :type Float%20%28single-precision%29))
  (if (Variables|Default|GetShouldTickTimer)
    (bind _output_get (Variables|Default|SetTime (Math|Float|Max(Float) (- (Variables|Default|GetTime) (Utilities|Time|GetWorldDeltaSeconds)) 0.0)))
    (bind _hud_interact (Variables|Default|GetHUD_INTERACT)
      (:then
        (Default|UpdateTimer _hud_interact _output_get)
        (if (== (Variables|Default|GetTime) 0.0)
          (Utilities|FlowControl|DoOnce false
            (:Completed
              (bind _asbp_first_person_character (Utilities|Casting|CastToBP_FirstPersonCharacter (Game|GetPlayerCharacter 0)))
              (Default|OnDeath _asbp_first_person_character)))))
      (:else))))

(event EventBeginPlay
  (bind _returnvalue (Actor|GetActorOfClass "/Game/Proto/BP_NPCActivationZone.BP_NPCActivationZone_C"))
  (EventDispatchers|BindEventtoEnterArenaDispatcher _returnvalue (delegate Custom|StartTimerEvent))
  (bind _returnvalue_2 (Actor|GetActorOfClass "/Game/Proto/ProtoInteract/BP_GeneratorsDoor.BP_GeneratorsDoor_C"))
  (EventDispatchers|BindEventtoFinishLevelDispatcher _returnvalue_2 (delegate Custom|StopTimerEvent))
  (bind _ashud_interact (Utilities|Casting|CastToHUD_INTERACT (HUD|GetHUD (Game|GetPlayerController 0))))
  (Variables|Default|SetHUD_INTERACT _ashud_interact))

(fn ConstructionScript)