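; BP_Sun is a level actor that animates the sun during the arena fight by slowly pitching itself over time.
; On BeginPlay it finds the NPC activation zone and generators door, binding to their enter-arena and finish-level dispatchers.
; Those events toggle a flag that starts and stops the rotation.
; While the flag is set, Tick adds a local pitch rotation scaled by delta time and a Speed variable.
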(event Custom|StartTimerEvent
  (Variables|Default|SetShouldMoveSun true))

(event Custom|StopTimerEvent
  (Variables|Default|SetShouldMoveSun false))

(event EventTick
  (params (DeltaSeconds :type Float%20%28single-precision%29))
  (if (Variables|Default|GetShouldMoveSun)
    ;[1 1 1] Rotate SUN
    (Transformation|AddActorLocalRotation (Math|Rotator|MakeRotator 0.0 (* DeltaSeconds (Variables|Default|GetSpeed)) 0.0) false false)))

(event EventBeginPlay
  (bind _returnvalue (Actor|GetActorOfClass "/Game/Proto/BP_NPCActivationZone.BP_NPCActivationZone_C"))
  (EventDispatchers|BindEventtoEnterArenaDispatcher _returnvalue (delegate Custom|StartTimerEvent))
  (bind _returnvalue_2 (Actor|GetActorOfClass "/Game/Proto/ProtoInteract/BP_GeneratorsDoor.BP_GeneratorsDoor_C"))
  (EventDispatchers|BindEventtoFinishLevelDispatcher _returnvalue_2 (delegate Custom|StopTimerEvent)))

(fn ConstructionScript)