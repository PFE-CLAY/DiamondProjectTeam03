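; BP_LoopExplosion is the explosion actor that kills the first-person character at the end of a loop.
; When its sphere overlaps BP_FirstPersonCharacter, it clears the ScreenShake flag and calls DeathByEndLoop on the character.
; Tick polls that flag to play BP_LoopCamShake once over a huge radius, then resets it; nothing in this graph sets it true.
; Both paths print debug text.
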(event OnComponentBeginOverlap(Sphere)
  (params (OverlappedComponent :type Primitive%20Component%20Object%20Reference) (OtherActor :type Actor%20Object%20Reference) (OtherComp :type Primitive%20Component%20Object%20Reference) (OtherBodyIndex :type Integer) (bFromSweep :type Boolean) (SweepResult :type Hit%20Result%20Structure%20%28by%20ref%29))
  (bind (_asbp_first_person_character _bsuccess) (Utilities|Casting|CastToBP_FirstPersonCharacter OtherActor))
  (if _bsuccess
    (Development|PrintString "Enorme etron")
    (Variables|Default|SetScreenShake false)
    (Default|DeathbyEndLoop _asbp_first_person_character)))

(event EventTick
  (params (DeltaSeconds :type Float%20%28single-precision%29))
  ;[1 1 1] Ne regardez pas ça les progs
  (if (Variables|Default|GetScreenShake)
    (Camera|PlayWorldCameraShake "/Game/Project/BP/CameraShake/BP_LoopCamShake.BP_LoopCamShake_C" "0, 0, 0" 0.0 3e+09)
    (Variables|Default|SetScreenShake false)
    (Development|PrintText "shake")))

(fn ConstructionScript)