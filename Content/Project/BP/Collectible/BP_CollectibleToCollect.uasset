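; BP_CollectibleToCollect is a world pickup that the first-person player collects by overlapping its sphere or box.
; On overlap it activates its CollectibleID in the loop subsystem, then shows preplan HUD feedback with the ID and step.
; It destroys itself only if that feedback widget is valid, or at PostInit if already collected.
; The construction script applies the configured collectible material to the mesh.
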(event OnComponentBeginOverlap(Box)
  (params (OverlappedComponent :type Primitive%20Component%20Object%20Reference) (OtherActor :type Actor%20Object%20Reference) (OtherComp :type Primitive%20Component%20Object%20Reference) (OtherBodyIndex :type Integer) (bFromSweep :type Boolean) (SweepResult :type Hit%20Result%20Structure%20%28by%20ref%29))
  (bind _collectibleid (Variables|Default|GetCollectibleID))
  (bind _asbp_first_person_character (Utilities|Casting|CastToBP_FirstPersonCharacter OtherActor))
  (Class|LoopSubsystem|ActivateCollectible (Subsystems|GetLoopSubsystem) _collectibleid)
  (bind _preplanfeeedbackwidget (Variables|/Game/Project/Game/HUD/HUD_GAME.HUD_GAME_C|GetPreplanFeeedbackWidget (Variables|/Game/Project/Game/BP_FirstPersonCharacter.BP_FirstPersonCharacter_C|GetInteractHUD _asbp_first_person_character))
    (:then
      (Default|AppearFeedback _preplanfeeedbackwidget _collectibleid (Variables|Default|GetStep))
      (Actor|DestroyActor))
    (:else)))

(event OnComponentBeginOverlap(Sphere)
  (params (OverlappedComponent :type Primitive%20Component%20Object%20Reference) (OtherActor :type Actor%20Object%20Reference) (OtherComp :type Primitive%20Component%20Object%20Reference) (OtherBodyIndex :type Integer) (bFromSweep :type Boolean) (SweepResult :type Hit%20Result%20Structure%20%28by%20ref%29))
  (bind _collectibleid (Variables|Default|GetCollectibleID))
  (bind _asbp_first_person_character (Utilities|Casting|CastToBP_FirstPersonCharacter (stale OnComponentBeginOverlap(Box) OtherActor)))
  (Class|LoopSubsystem|ActivateCollectible (Subsystems|GetLoopSubsystem) _collectibleid)
  (bind _preplanfeeedbackwidget (Variables|/Game/Project/Game/HUD/HUD_GAME.HUD_GAME_C|GetPreplanFeeedbackWidget (Variables|/Game/Project/Game/BP_FirstPersonCharacter.BP_FirstPersonCharacter_C|GetInteractHUD _asbp_first_person_character))
    (:then
      (Default|AppearFeedback _preplanfeeedbackwidget _collectibleid (Variables|Default|GetStep))
      (Actor|DestroyActor))
    (:else)))

(event Custom|PostInit
  (if (Variables|Default|GetbHasBeenCollected)
    (Actor|DestroyActor)))

(event Collision|EventActorBeginOverlap
  (params (OtherActor :type Actor%20Object%20Reference)))

(event EventTick
  (params (DeltaSeconds :type Float%20%28single-precision%29)))

(fn ConstructionScript
  (Rendering|Material|SetMaterial (Variables|Default|Getre) 0 (Variables|Default|GetCollectible_Material)))