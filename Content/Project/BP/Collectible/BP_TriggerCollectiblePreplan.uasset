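; BP_TriggerCollectiblePreplan is a trigger volume that activates a collectible, a preplan step or both when the first-person character overlaps its box.
; TriggerValue selects which of these fire, passing the configured collectible ID or preplan step ID and part to the LoopSubsystem.
; On PostInit, the actor destroys itself if HasBeenCollected is set, to prevent repeated collection across loops.
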(event OnComponentBeginOverlap(Box)
  (params (OverlappedComponent :type Primitive%20Component%20Object%20Reference) (OtherActor :type Actor%20Object%20Reference) (OtherComp :type Primitive%20Component%20Object%20Reference) (OtherBodyIndex :type Integer) (bFromSweep :type Boolean) (SweepResult :type Hit%20Result%20Structure%20%28by%20ref%29))
  (bind _returnvalue (Subsystems|GetLoopSubsystem))
  (Utilities|Casting|CastToBP_FirstPersonCharacter OtherActor)
  (switch int (Variables|Default|GetTriggerValue)
    (:0
      (Utilities|FlowControl|Sequence
        (:then_0
          (Class|LoopSubsystem|ActivateCollectible _returnvalue (Variables|Default|GetCollectibleID) :!label _label))
        (:then_1
          (Class|LoopSubsystem|ActivatePreplanStep _returnvalue (Variables|Default|GetPreplanStepID) (Variables|Default|GetPreplanStepPart) :!label _label_2))))
    (:1
      (goto _label))
    (:2
      (goto _label_2))))

(event Custom|PostInit
  ;[0.1355 0.000216 0.15 0.5] Nécessaire pour ne pas pouvoir collecter les collectibles en boucle.
  (if (Variables|Default|GetbHasBeenCollected)
    (Actor|DestroyActor)))

(fn ConstructionScript)