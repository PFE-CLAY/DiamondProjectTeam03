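; Trigger actor that starts the end-of-demo cutscene when the player character overlaps it.
; On overlap it looks up BP_Timer and proceeds only while its Time is above zero.
; It then disables input on the player character, creates a level sequence player for LS_EndDemo and plays it.
; Nothing here re-enables input or guards against repeated triggering.
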(event Collision|EventActorBeginOverlap
  (params (OtherActor :type Actor%20Object%20Reference))
  (bind _returnvalue (Game|GetPlayerCharacter 0))
  (if (== OtherActor _returnvalue)
    (bind _returnvalue_2 (Actor|GetActorOfClass "/Game/Project/BP/LD/BP_Timer.BP_Timer_C"))
    (if (> (Variables|/Game/Project/BP/LD/BP_Timer.BP_Timer_C|GetTime _returnvalue_2) 0.0)
      (Input|DisableInput _returnvalue 0)
      (bind _outactor (Sequencer|Player|CreateLevelSequencePlayer "/Game/Project/CameraAnim/LS_EndDemo.LS_EndDemo"))
      (Sequencer|Player|Play (Variables|/Script/LevelSequence.LevelSequenceActor|GetSequencePlayer _outactor) :!class /Script/MovieScene.MovieSceneSequencePlayer))))

(fn ConstructionScript)