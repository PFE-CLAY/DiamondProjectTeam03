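; Bear trap that freezes the player on overlap and spawns a group of BP_BearTrapEnemy actors.
; Spawn points fan out by rotating a vector derived from the player-to-trap direction, using Range, AngleRange and EnemiesNumber, with persistent debug lines and spheres drawn.
; Each enemy gets the trap as Parent and an index-based spawn event.
; RemoveSpawnActorToArray drops enemies from the tracked array and restores input and walking once it empties.
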(event Custom|On%20Empty%20Array%20Event
  (CallFunction|EnableMovement))

(event EventBeginPlay)

(event Collision|EventActorBeginOverlap
  (params (OtherActor :type Actor%20Object%20Reference))
  (bind _returnvalue (Transformation|GetActorLocation))
  (bind _returnvalue_2 (Game|GetPlayerController 0))
  (bind _returnvalue_3 (Game|GetPlayerController 0))
  (bind _returnvalue_4 (Pawn|GetControlledPawn _returnvalue_3))
  (bind _returnvalue_5 (Pawn|GetControlledPawn _returnvalue_2))
  (bind _returnvalue_6 (Transformation|GetActorLocation _returnvalue_4))
  (bind _returnvalue_7 (Transformation|GetActorLocation _returnvalue_5))
  (Utilities|Casting|CastToBP_FirstPersonCharacter OtherActor)
  (CallFunction|DisableMovement)
  (Variables|Default|SetPlayerPosition (Math|Vector|MakeVector (.x _returnvalue_6) (.y _returnvalue_6) 0.0))
  (Variables|Default|SetOwnPosition (Math|Vector|MakeVector (.x _returnvalue) (.y _returnvalue) 0.0))
  (Rendering|Debug|DrawDebugSphere _returnvalue_7 1e+01 12 "(R=0.676580,G=0.000000,B=1.000000,A=1.000000)" 9999.0 1.0)
  (bind _output_get (Variables|Default|SetDirection (* (- (Variables|Default|GetPlayerPosition) (Variables|Default|GetOwnPosition)) -1.0)))
  (Rendering|Debug|DrawDebugLine _returnvalue_7 (+ _returnvalue_7 _output_get) "(R=1.000000,G=0.000000,B=0.027083,A=1.000000)" 9999.0 5.0)
  (Rendering|Debug|DrawDebugLine (+ _returnvalue_7 (Variables|Default|GetDirection)) (+ (+ _returnvalue_7 (Variables|Default|GetDirection)) (Variables|Default|GetDirection)) "(R=0.109128,G=1.000000,B=0.000000,A=1.000000)" 9999.0 5.0)
  (bind _output_get_2 (Variables|Default|SetDirection (* (Math|Vector|Normalize (Variables|Default|GetDirection)) (Variables|Default|GetRange))))
  (Rendering|Debug|DrawDebugLine (+ (Math|Vector|MakeVector 0.0 0.0 (+ (.z (Transformation|GetActorLocation (Pawn|GetControlledPawn (Game|GetPlayerController 0)))) 3e+01)) (Variables|Default|GetOwnPosition)) (+ (+ (+ (Math|Vector|MakeVector 0.0 0.0 (+ (.z (Transformation|GetActorLocation (Pawn|GetControlledPawn (Game|GetPlayerController 0)))) 3e+01)) (Variables|Default|GetOwnPosition)) _output_get_2) "0.000000,0.000000,30.000000") "(R=1.000000,G=0.871250,B=0.000000,A=1.000000)" 9999.0 5.0)
  (Variables|Default|SetDirection (+ (+ (Math|Vector|MakeVector 0.0 0.0 (.z (Transformation|GetActorLocation (Pawn|GetControlledPawn (Game|GetPlayerController 0))))) (Variables|Default|GetOwnPosition)) (Math|Vector|RotateVector (Variables|Default|GetDirection) (Math|Rotator|MakeRotator 0.0 0.0 (* (/ (Variables|Default|GetAngleRange) 2.0) -1.0)))))
  (for _index (range 0 (- (Variables|Default|GetEnemiesNumber) 1))
    (Rendering|Debug|DrawDebugSphere (+ (+ (Math|Vector|MakeVector 0.0 0.0 (.z (Transformation|GetActorLocation (Pawn|GetControlledPawn (Game|GetPlayerController 0))))) (Variables|Default|GetOwnPosition)) (Math|Vector|RotateVector (Variables|Default|GetDirection) (Math|Rotator|MakeRotator 0.0 0.0 (* (/ (Variables|Default|GetAngleRange) (Variables|Default|GetEnemiesNumber)) _index)))) 2e+01 12 "(R=1.000000,G=1.000000,B=1.000000,A=1.000000)" 9999.0 2.5)
    (bind _returnvalue_8 (Game|SpawnActorfromClass "/Game/Proto/BP_BearTrapEnemy.BP_BearTrapEnemy_C" (Math|Transform|MakeTransform (+ (+ (Math|Vector|MakeVector 0.0 0.0 (.z (Transformation|GetActorLocation (Pawn|GetControlledPawn (Game|GetPlayerController 0))))) (Variables|Default|GetOwnPosition)) (Math|Vector|RotateVector (Variables|Default|GetDirection) (Math|Rotator|MakeRotator 0.0 0.0 (* (/ (Variables|Default|GetAngleRange) (Variables|Default|GetEnemiesNumber)) _index)))) "0, 0, 0" "1.000000,1.000000,1.000000") "Undefined" "MultiplyWithRoot" 0 0))
    (Utilities|Array|Add (Variables|Default|GetSpawnedActor) _returnvalue_8)
    (Variables|/Game/Proto/BP_BearTrapEnemy.BP_BearTrapEnemy_C|SetParent _returnvalue_8 self)
    (Default|OnSpawnEvent _returnvalue_8 (+ (Math|Conversions|ToFloat(Integer) _index) 1.0))))

(event EventTick
  (params (DeltaSeconds :type Float%20%28single-precision%29)))

(fn ConstructionScript)

(fn RemoveSpawnActortoArray
  (params (Target :type Actor%20Object%20Reference))
  (Utilities|Array|RemoveItem (Variables|Default|GetSpawnedActor) Target)
  (if (== (Utilities|Array|Length (Variables|Default|GetSpawnedActor)) 0)
    (CallFunction|OnEmptyArrayEvent)))

(fn DisableMovement
  (bind _returnvalue (Game|GetPlayerController 0))
  (bind _returnvalue_2 (Pawn|GetControlledPawn _returnvalue))
  (Input|DisableInput _returnvalue_2 _returnvalue)
  (bind _asbp_player_first_person_character (Utilities|Casting|CastToBP_PlayerFirstPersonCharacter _returnvalue_2))
  (Variables|/Script/Engine.MovementComponent|SetVelocity (Variables|/Script/Engine.Character|GetCharacterMovement _asbp_player_first_person_character) "0, 0, 0")
  (Pawn|Components|CharacterMovement|DisableMovement (Variables|/Script/Engine.Character|GetCharacterMovement _asbp_player_first_person_character)))

(fn EnableMovement
  (bind _returnvalue (Game|GetPlayerController 0))
  (bind _returnvalue_2 (Pawn|GetControlledPawn _returnvalue))
  (Input|EnableInput _returnvalue_2 _returnvalue)
  (bind _asbp_player_first_person_character (Utilities|Casting|CastToBP_PlayerFirstPersonCharacter _returnvalue_2))
  (Pawn|Components|CharacterMovement|SetMovementMode (Variables|/Script/Engine.Character|GetCharacterMovement _asbp_player_first_person_character) "MOVE_Walking" 0))